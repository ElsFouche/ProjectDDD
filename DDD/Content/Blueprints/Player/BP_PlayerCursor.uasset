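; Player grid cursor that carries an orbiting orthographic camera, with a looping bob on the cursor component.
; Digital moves step one grid cell relative to camera yaw, while stick moves ramp up speed and snap to the grid on release.
; Camera input either pivots in quarter turns and pitch steps, using edge-detected stick flicks, or turns freely and snaps on release.
; Tick eases ortho width toward the zoom target within a short timer.
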(event Custom|TickZoom
  (params (Delta%20Seconds :type Float%20%28double-precision%29))
  (bind _maincamera (Variables|Default|GetMainCamera))
  ;[0.3698 1 0.7391 0.5] Camera
  (if (and (> (Variables|Camera|GetZoomTimer) 0.0) (> (Math|Float|Absolute(Float) (- (Variables|/Script/Engine.CameraComponent|GetOrthoWidth (Variables|Default|GetMainCamera)) (Variables|Camera|GetCamZoomTarget))) 1.0))
    (bind _output_get (Variables|Camera|SetZoomTimer (- (Variables|Camera|GetZoomTimer) Delta%20Seconds)))
    (Class|CameraComponent|SetOrthoWidth _maincamera (select (<= _output_get 0.0) (Variables|Camera|GetCamZoomTarget) (Math|Float|Lerp (Variables|/Script/Engine.CameraComponent|GetOrthoWidth _maincamera) (Variables|Camera|GetCamZoomTarget) (* Delta%20Seconds (Variables|Camera|GetZoomLerpSpeed)))))))

(event Custom|CursorBobbing
  (bind _cursorbobspeed (Variables|Visuals|GetCursorBobSpeed))
  (bind _tempcursor (Variables|Default|GetTempCursor))
  (bind _cursorbobheight (Variables|Visuals|GetCursorBobHeight))
  (bind _returnvalue (Transformation|GetRelativeTransform _tempcursor))
  ;[0.9375 0.8484 0.502 0.5] Cursor Bob Loop
  (Components|MoveComponentTo _tempcursor (Math|Vector|MakeVector (.x (.location _returnvalue)) (.y (.location _returnvalue)) (+ (.z (.location _returnvalue)) _cursorbobheight)) (.rotation _returnvalue) true true _cursorbobspeed false)
  (Components|MoveComponentTo _tempcursor (Math|Vector|MakeVector (.x (.location _returnvalue)) (.y (.location _returnvalue)) (+ (.z (.location _returnvalue)) (* _cursorbobheight -1.0))) (.rotation _returnvalue) true true _cursorbobspeed false)
  (CallFunction|CursorBobbing))

(event Input|EnhancedActionEvents|EnhancedInputActionIA_CamPivotLeft
  (params (ActionValue :type Boolean) (ElapsedSeconds :type Float%20%28double-precision%29) (TriggeredSeconds :type Float%20%28double-precision%29) (InputAction :type Input%20Action%20Object%20Reference :default "/Game/Blueprints/Player/InputActions/IA_CamPivotLeft.IA_CamPivotLeft"))
  (bind _cameraboom (Variables|Default|GetCameraBoom))
  (bind _camyawindex (Variables|Camera|GetCamYawIndex))
  ;[0.3698 1 0.7391 0.5] Camera
  (:Started
    (if (not (Variables|Camera|GetCamIsTurning))
      (if (Variables|Camera|GetFlipPivotYawDirection)
        (Math|Integer|DecrementInt _camyawindex
          (:%20%20
            _))
        (else
          (Math|Integer|IncrementInt _camyawindex
            (:%20%20
              _))))
      (Transformation|SetRelativeRotation _cameraboom (Math|Rotator|MakeRotator 0.0 (.Pitch (Math|Rotator|BreakRotator (Variables|/Script/Engine.SceneComponent|GetRelativeRotation _cameraboom))) (Utilities|RotIndextoAngle _camyawindex)) false false))))

(event Input|EnhancedActionEvents|EnhancedInputActionIA_CamPivotRight
  (params (ActionValue :type Boolean) (ElapsedSeconds :type Float%20%28double-precision%29) (TriggeredSeconds :type Float%20%28double-precision%29) (InputAction :type Input%20Action%20Object%20Reference :default "/Game/Blueprints/Player/InputActions/IA_CamPivotRight.IA_CamPivotRight"))
  (bind _cameraboom (Variables|Default|GetCameraBoom))
  (bind _camyawindex (Variables|Camera|GetCamYawIndex))
  ;[0.3698 1 0.7391 0.5] Camera
  (:Started
    (if (not (Variables|Camera|GetCamIsTurning))
      (if (Variables|Camera|GetFlipPivotYawDirection)
        (Math|Integer|IncrementInt _camyawindex
          (:%20%20
            _))
        (else
          (Math|Integer|DecrementInt _camyawindex
            (:%20%20
              _))))
      (Transformation|SetRelativeRotation _cameraboom (Math|Rotator|MakeRotator 0.0 (.Pitch (Math|Rotator|BreakRotator (Variables|/Script/Engine.SceneComponent|GetRelativeRotation _cameraboom))) (Utilities|RotIndextoAngle _camyawindex)) false false))))

(event Input|EnhancedActionEvents|EnhancedInputActionIA_CamTurn
  (params (ActionValue :type Vector%202D%20Structure) (ElapsedSeconds :type Float%20%28double-precision%29) (TriggeredSeconds :type Float%20%28double-precision%29) (InputAction :type Input%20Action%20Object%20Reference :default "/Game/Blueprints/Player/InputActions/IA_CamTurn.IA_CamTurn"))
  (bind _cameraboom (Variables|Default|GetCameraBoom))
  (bind _camturnsensitivity (Variables|Camera|GetCamTurnSensitivity))
  (bind _cameraboom_2 (Variables|Default|GetCameraBoom))
  (bind _cameraboom_3 (Variables|Default|GetCameraBoom))
  (bind _cameraboom_4 (Variables|Default|GetCameraBoom))
  (bind _camminmaxpitch (Variables|Camera|GetCamMinMaxPitch))
  (bind _cameraboom_5 (Variables|Default|GetCameraBoom))
  (bind _flippivotyawdirection (Variables|Camera|GetFlipPivotYawDirection))
  (bind (_x _y) (Math|Vector2D|BreakVector2D _camminmaxpitch))
  (bind _returnvalue (* _camturnsensitivity ActionValue))
  (bind _relativerotation (Variables|/Script/Engine.SceneComponent|GetRelativeRotation _cameraboom_4))
  (bind _relativerotation_2 (Variables|/Script/Engine.SceneComponent|GetRelativeRotation _cameraboom_5))
  (bind _relativerotation_3 (Variables|/Script/Engine.SceneComponent|GetRelativeRotation _cameraboom))
  (bind (_roll _pitch _yaw) (Math|Rotator|BreakRotator _relativerotation_3))
  (bind _pitch_2 (Math|Rotator|BreakRotator _relativerotation))
  (bind (_roll_2 _pitch_3 _yaw_2) (Math|Rotator|BreakRotator _relativerotation_2))
  (bind (_x_2 _y_2) (Math|Vector2D|BreakVector2D _returnvalue))
  ;[0.3698 1 0.7391 0.5] Camera
  (:Triggered
    (if (Variables|Camera|GetPivotMode)
      (|DetectStickPulse ActionValue
        (:Exec
          (|PivotFromAnalogInput (Utilities|BoundVector2D ActionValue)
            (:Up
              (if (not (Variables|Camera|GetCamIsTurning))
                (Transformation|SetRelativeRotation _cameraboom_3 (Math|Rotator|MakeRotator 0.0 (Utilities|SnapPitchtoRestPoint (+ (Utilities|GetPitchStepAngle false) _pitch_2)) (Utilities|RotIndextoAngle (Variables|Camera|GetCamYawIndex))) false false)))
            (:Right
              (if (not (Variables|Camera|GetCamIsTurning))
                (if _flippivotyawdirection
                  (Math|Integer|IncrementInt (Variables|Camera|GetCamYawIndex) :!label _label
                    (:%20%20
                      _))
                  (else
                    (Math|Integer|DecrementInt (Variables|Camera|GetCamYawIndex) :!label _label_2
                      (:%20%20
                        _))))
                (Transformation|SetRelativeRotation _cameraboom_2 (Math|Rotator|MakeRotator 0.0 (.Pitch (Math|Rotator|BreakRotator (Variables|/Script/Engine.SceneComponent|GetRelativeRotation _cameraboom_2))) (Utilities|RotIndextoAngle (Variables|Camera|GetCamYawIndex))) false false)))
            (:Down
              (if (not (Variables|Camera|GetCamIsTurning))
                (Transformation|SetRelativeRotation _cameraboom_3 (Math|Rotator|MakeRotator 0.0 (Utilities|SnapPitchtoRestPoint (+ (Utilities|GetPitchStepAngle true) _pitch_2)) (Utilities|RotIndextoAngle (Variables|Camera|GetCamYawIndex))) false false)))
            (:Left
              (if (not (Variables|Camera|GetCamIsTurning))
                (if _flippivotyawdirection
                  (goto _label_2)
                  (else
                    (goto _label))))))))
      (else
        (Transformation|SetRelativeRotation (Variables|Default|GetCameraBoom) (Math|Rotator|MakeRotator 0.0 (* (Math|Float|Clamp(Float) (* (+ _pitch_3 _y_2) -1.0) _x _y) -1.0) (+ _yaw_2 _x_2)) false false))))
  (:Started
    (Variables|Camera|SetCamIsTurning (not (Variables|Camera|GetPivotMode))))
  (:Completed
    (Variables|Camera|SetCamIsTurning false)
    ;;[0.15 0.15 0.15 0.5] Snap to Nearest Angle when Input Completes
    (if (not (Variables|Camera|GetPivotMode))
      (bind _output_get (Variables|Camera|SetCamYawIndex (Utilities|AngletoRotIndex _yaw)))
      (Transformation|SetRelativeRotation _cameraboom (Math|Rotator|MakeRotator 0.0 (Utilities|SnapPitchtoRestPoint _pitch) (Utilities|RotIndextoAngle _output_get)) false false))))

(event Input|EnhancedActionEvents|EnhancedInputActionIA_CamPivotUp
  (params (ActionValue :type Boolean) (ElapsedSeconds :type Float%20%28double-precision%29) (TriggeredSeconds :type Float%20%28double-precision%29) (InputAction :type Input%20Action%20Object%20Reference :default "/Game/Blueprints/Player/InputActions/IA_CamPivotUp.IA_CamPivotUp"))
  ;[0.3698 1 0.7391 0.5] Camera
  (:Started
    (if (not (Variables|Camera|GetCamIsTurning))
      (Transformation|SetRelativeRotation (Variables|Default|GetCameraBoom) (Math|Rotator|MakeRotator 0.0 (Utilities|SnapPitchtoRestPoint (+ (Utilities|GetPitchStepAngle false) (.Pitch (Math|Rotator|BreakRotator (Variables|/Script/Engine.SceneComponent|GetRelativeRotation (Variables|Default|GetCameraBoom)))))) (Utilities|RotIndextoAngle (Variables|Camera|GetCamYawIndex))) false false))))

(event Input|EnhancedActionEvents|EnhancedInputActionIA_CamPivotDown
  (params (ActionValue :type Boolean) (ElapsedSeconds :type Float%20%28double-precision%29) (TriggeredSeconds :type Float%20%28double-precision%29) (InputAction :type Input%20Action%20Object%20Reference :default "/Game/Blueprints/Player/InputActions/IA_CamPivotDown.IA_CamPivotDown"))
  ;[0.3698 1 0.7391 0.5] Camera
  (:Started
    (if (not (Variables|Camera|GetCamIsTurning))
      (Transformation|SetRelativeRotation (Variables|Default|GetCameraBoom) (Math|Rotator|MakeRotator 0.0 (Utilities|SnapPitchtoRestPoint (+ (Utilities|GetPitchStepAngle true) (.Pitch (Math|Rotator|BreakRotator (Variables|/Script/Engine.SceneComponent|GetRelativeRotation (Variables|Default|GetCameraBoom)))))) (Utilities|RotIndextoAngle (Variables|Camera|GetCamYawIndex))) false false))))

(event Input|EnhancedActionEvents|EnhancedInputActionIA_ToggleCamPivot
  (params (ActionValue :type Boolean) (ElapsedSeconds :type Float%20%28double-precision%29) (TriggeredSeconds :type Float%20%28double-precision%29) (InputAction :type Input%20Action%20Object%20Reference :default "/Game/Blueprints/Player/InputActions/IA_ToggleCamPivot.IA_ToggleCamPivot"))
  ;[0.3698 1 0.7391 0.5] Camera
  (:Started
    (bind _output_get (Variables|Camera|SetPivotMode (not (Variables|Camera|GetPivotMode))))
    (Development|PrintString (select _output_get "Right Stick Mode: Pivot" "Right Stick Mode: Turn"))))

(event Input|EnhancedActionEvents|EnhancedInputActionIA_Zoom
  (params (ActionValue :type Float%20%28double-precision%29) (ElapsedSeconds :type Float%20%28double-precision%29) (TriggeredSeconds :type Float%20%28double-precision%29) (InputAction :type Input%20Action%20Object%20Reference :default "/Game/Blueprints/Player/InputActions/IA_Zoom.IA_Zoom"))
  (bind _camminmaxdistance (Variables|Camera|GetCamMinMaxDistance))
  (bind (_x _y) (Math|Vector2D|BreakVector2D _camminmaxdistance))
  ;[0.3698 1 0.7391 0.5] Camera
  (Variables|Camera|SetCamZoomTarget (Math|Float|Clamp(Float) (+ (* (Variables|Camera|GetCamZoomSpeed) ActionValue) (Variables|Camera|GetCamZoomTarget)) _x _y))
  (Variables|Camera|SetZoomTimer 1.0))

(event Input|EnhancedActionEvents|EnhancedInputActionIA_Move
  (params (ActionValue :type Vector%202D%20Structure) (ElapsedSeconds :type Float%20%28double-precision%29) (TriggeredSeconds :type Float%20%28double-precision%29) (InputAction :type Input%20Action%20Object%20Reference :default "/Game/Blueprints/Player/InputActions/IA_Move.IA_Move"))
  (bind _ac_gridnavigation (Variables|Default|GetAC_GridNavigation))
  (bind _gridsize (Variables|/Game/Blueprints/ActorComponents/AC_GridNavigation.AC_GridNavigation_C|GetGridSize _ac_gridnavigation))
  ;[0.9375 0.8484 0.502 0.5] Movement - WASD / Dpad
  (Utilities|FlowControl|DoOnce false :!label _label
    (:Completed
      (bind _snappedpoint (Default|PointSnaptoGrid (Variables|Default|GetAC_GridNavigation) (+ (Math|Vector|RotateVector (Math|Vector|MakeVector (* (.x ActionValue) (.x _gridsize)) (* (.y ActionValue) (.y _gridsize)) 0.0) (Math|Rotator|MakeRotator 0.0 0.0 (+ (.yaw (Variables|/Script/Engine.SceneComponent|GetRelativeRotation (Variables|Default|GetCameraBoom))) (Variables|Movement|GetMoveAngleOffset)))) (Transformation|GetWorldLocation (Variables|Default|GetDefaultSceneRoot)))))
      (Components|MoveComponentTo (Variables|Default|GetDefaultSceneRoot) (Math|Conversions|ToVector(Float) _snappedpoint) "0, 0, 0" true true (Math|Float|SafeDivide 1.0 (Variables|Movement|GetCursorTravelSpeed)) false)
      (goto _label Reset))))

(event Input|EnhancedActionEvents|EnhancedInputActionIA_StickMove
  (params (ActionValue :type Vector%202D%20Structure) (ElapsedSeconds :type Float%20%28double-precision%29) (TriggeredSeconds :type Float%20%28double-precision%29) (InputAction :type Input%20Action%20Object%20Reference :default "/Game/Blueprints/Player/InputActions/IA_StickMove.IA_StickMove"))
  (bind _returnvalue (/ ElapsedSeconds 1.5))
  (bind _ac_gridnavigation (Variables|Default|GetAC_GridNavigation))
  (bind _defaultsceneroot (Variables|Default|GetDefaultSceneRoot))
  (bind _returnvalue_2 (Math|Float|Clamp(Float) _returnvalue))
  (bind _gridsize (Variables|/Game/Blueprints/ActorComponents/AC_GridNavigation.AC_GridNavigation_C|GetGridSize _ac_gridnavigation))
  ;[0.9375 0.8484 0.502 0.5] Movement - Joystick
  (:Triggered
    (Components|MoveComponentTo (Variables|Default|GetDefaultSceneRoot) (+ (Transformation|GetWorldLocation (Variables|Default|GetDefaultSceneRoot)) (Math|Vector|RotateVector (Math|Vector|MakeVector (* (* (.x ActionValue) _returnvalue_2) (.x _gridsize)) (* (* _returnvalue_2 (.y ActionValue)) (.y _gridsize)) 0.0) (Math|Rotator|MakeRotator 0.0 0.0 (+ (.yaw (Variables|/Script/Engine.SceneComponent|GetRelativeRotation (Variables|Default|GetCameraBoom))) -9e+01)))) "0, 0, 0" true true (Math|Float|SafeDivide 0.25 (Variables|Movement|GetCursorTravelSpeed)) false :!label _label))
  (:Completed
    (Utilities|FlowControl|Sequence
      (:then_0
        (goto _label Stop))
      (:then_1
        ;;[0.04844 0.0493 0.15 0.5] Input Released
        (Utilities|FlowControl|DoOnce false :!label _label_2
          (:Completed
            (bind _snappedpoint (Default|PointSnaptoGrid (Variables|Default|GetAC_GridNavigation) (Transformation|GetWorldLocation _defaultsceneroot)))
            (Components|MoveComponentTo _defaultsceneroot (Math|Conversions|ToVector(Float) _snappedpoint) "0, 0, 0" true true (Math|Float|SafeDivide 1.0 (Variables|Movement|GetCursorTravelSpeed)) false)
            (goto _label_2 Reset)))))))

(event EventTick
  (params (DeltaSeconds :type Float%20%28single-precision%29))
  (CallFunction|TickZoom DeltaSeconds))

(event EventBeginPlay
  (CallFunction|CursorBobbing))

(fn ConstructionScript)