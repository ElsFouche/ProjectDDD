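; Player controller Blueprint that sets up Enhanced Input when play begins.
; It adds IMC_Main to player 0's Enhanced Input local player subsystem, printing an error if that subsystem is invalid.
; It then registers every mapping context from GetAllIMC with the input user settings, skipping those already registered.
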(event EventBeginPlay
  (bind _returnvalue (Game|GetPlayerController 0))
  (bind _settings (CallFunction|GetUserSettings))
  (bind _returnvalue_2 (PlayerController|LocalPlayerSubsystems|GetEnhancedInputLocalPlayerSubsystem _returnvalue))
  (Utilities|IsValid _returnvalue_2
    (:Is%20Valid
      (Input|AddMappingContext _returnvalue_2 "/Game/Blueprints/Player/IMC_Main.IMC_Main" 0 "(bIgnoreAllPressedKeysUntilRelease=True,bForceImmediately=False,bNotifyUserSettings=False)")
      (for _array_element (CallFunction|GetAllIMC)
        (if (not (Class|EnhancedInputUserSettings|IsMappingContextRegistered _settings _array_element))
          (Class|EnhancedInputUserSettings|RegisterInputMappingContext _settings _array_element))))
    (:Is%20Not%20Valid
      (Development|PrintString "Enhanced input local player susbsystem is invalid. "))))

(fn ConstructionScript)