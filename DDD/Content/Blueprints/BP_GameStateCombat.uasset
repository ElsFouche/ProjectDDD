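; Combat game state for a turn-based tactics game, holding units, initiative, turn order and random team names, still largely test scaffolding.
; BeginPlay has a construction actor generate a room, then spawns a hardcoded test unit once progress completes.
; DIV initiative derives from unit stats and turns taken, and UpdateTurnOrder swap-sorts units by ascending DIV.
; CombatStart and AddtoTacticalCortex are empty, with their turn-start and cortex-broadcast logic left disconnected.
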(event Custom|CombatStart)

(event EventBeginPlay
  ;[0 0 0 0.5] Test Functionality
  (Class|AutomationBlueprintFunctionLibrary|AutomationWaitforLoading)
  (DEBUG|CreateBattlefield))

(event EventAddSpawnPoints
  (params (NewSpawnPoints :type Array%20of%20F%20Unit%20Spawn%20Point%20Structures))
  (Utilities|Array|AppendArray (Variables|Default|GetSpawnPoints) NewSpawnPoints))

(event EventAddtoTacticalCortex
  (params (NewTacticalCortexPiece :type BP%20Tactical%20Cortex%20Object%20Reference%20%28by%20ref%29)))

(event EventGenerateRoomProgress
  (params (Success :type Boolean) (Progress :type Float%20%28double-precision%29))
  ;[0 0 0 0.5] Test Functionality
  (if (and Success (Math|Float|NearlyEqual(Float) Progress 1e+02 0.001))
    (DEBUG|CreateUnits (Utilities|Array|MakeArray (Utilities|Struct|MakeF_UnitSpawnPoint (Utilities|Struct|MakeIntVector 100 100 100) "NewEnumerator0" 0))) ; Only spawns Actors for Units based on Spawn Points
  ))

(fn ConstructionScript)

(fn DIVCalculator
  (params (Unit :type BP%20Base%20Unit%20Object%20Reference%20%28by%20ref%29))
  (bind _unitsincombat (Variables|DerivedInitiativeValue|GetUnitsInCombat))
  (bind _currstats (Variables|/Game/Units/BP_BaseUnit.BP_BaseUnit_C|GetCurrStats Unit))
  (bind (_ap _move _speed) (Utilities|Struct|BreakF_UnitStats _currstats))
  (bind (_value _returnvalue) (Utilities|Map|Find _unitsincombat Unit))
  (if _returnvalue
    (Utilities|Struct|SetmembersinF_UnitInitiativeData _value (* (+ _move _ap (LocalVariables|GetSpeedWeight)) (Math|Integer|Max(Integer) (- _speed (* (LocalVariables|GetTurnWeight) (.TurnsTaken (Utilities|Struct|BreakF_UnitInitiativeData _value)))))))
    (return true)
    (else
      (return false))))

(fn ModifyUnitDIV
  (params (Unit :type BP%20Base%20Unit%20Object%20Reference%20%28by%20ref%29) (DIV :type Integer))
  (bind _unitsincombat (Variables|DerivedInitiativeValue|GetUnitsInCombat))
  (bind (_value _returnvalue) (Utilities|Map|Find _unitsincombat Unit))
  (if _returnvalue
    (Utilities|Struct|SetmembersinF_UnitInitiativeData _value (Math|Integer|Max(Integer) (+ (Utilities|Struct|BreakF_UnitInitiativeData _value) DIV)))
    (DerivedInitiativeValue|UpdateTurnOrder)
    (return true)
    (else
      (return false))))

(fn UpdateTurnOrder
  (bind _unitsincombat (Variables|DerivedInitiativeValue|GetUnitsInCombat))
  (bind _keys (Utilities|Map|Keys (Variables|DerivedInitiativeValue|GetUnitsInCombat)))
  (bind _output_get (Variables|DerivedInitiativeValue|SetTurnOrder _keys))
  (for _index (range 0 (Utilities|Array|LastIndex _output_get))
    (for _index_2 (range (+ _index 1) (Utilities|Array|LastIndex _output_get))
      (if (< (Utilities|Struct|BreakF_UnitInitiativeData (.Value (Utilities|Map|Find _unitsincombat (Utilities|Array|Get(acopy) _output_get _index_2)))) (Utilities|Struct|BreakF_UnitInitiativeData (.Value (Utilities|Map|Find _unitsincombat (Utilities|Array|Get(acopy) _output_get _index)))))
        (Utilities|Array|Swap _output_get _index_2 _index))))
  (return))

(fn CreateBattlefield
  (bind _gridsize (CallFunction|GetDefaultGridSize))
  (bind (_x _y _z) (Utilities|Struct|BreakIntVector _gridsize))
  ;[0 0 0 0.5] DEBUG
  (bind _returnvalue (Game|SpawnActorfromClass "/Game/Procedural/BP_ConstructionActor.BP_ConstructionActor_C" (Math|Transform|MakeTransform (Math|Vector|MakeVector (Math|Conversions|ToFloat(Integer) _x) (Math|Conversions|ToFloat(Integer) _y) (Math|Conversions|ToFloat(Integer) _z)) "0, 0, 0" "1.000000,1.000000,1.000000") "AlwaysSpawn" "MultiplyWithRoot" 0 0))
  (bind _output_get (Variables|Procedural|SetCurrConstructionActor _returnvalue))
  (Class|BPIRoomConstruction|GenerateRoomStart(Message) _output_get self "NewEnumerator1" (Utilities|Struct|MakeIntVector 7 7 7)))

(fn CreateUnits
  (params (SpawnPoints :type Array%20of%20F%20Unit%20Spawn%20Point%20Structures))
  ;[0 0 0 0.5] DEBUG
  (bind _teamnames (DEBUG|CreateTeamNames SpawnPoints))
  (for _array_element SpawnPoints
    (bind _returnvalue (Game|SpawnActorfromClass "/Game/Units/BP_BaseUnit.BP_BaseUnit_C" (Math|Transform|MakeTransform (Math|Conversions|ToVector(Float) (.Location (Utilities|Struct|BreakF_UnitSpawnPoint _array_element))) "0, 0, 0" "1.000000,1.000000,1.000000") "DontSpawnIfColliding" "MultiplyWithRoot" 0 0))
    (Default|NewUnitOfType _returnvalue "NewEnumerator2")
    (Variables|/Game/Units/BP_BaseUnit.BP_BaseUnit_C|SetCurrentAnimationState _returnvalue "NewEnumerator0")
    (Variables|/Game/Units/BP_BaseUnit.BP_BaseUnit_C|SetUnitFacing _returnvalue (.Facing (Utilities|Struct|BreakF_UnitSpawnPoint _array_element)))
    (Variables|/Game/Units/BP_BaseUnit.BP_BaseUnit_C|SetTeamName _returnvalue (.Value (Utilities|Map|Find _teamnames (.TeamID (Utilities|Struct|BreakF_UnitSpawnPoint _array_element)))))
    (Utilities|Array|AddUnique (Variables|DEBUG|GetAllUnits) _returnvalue)))

(fn CreateTeamNames
  (params (SpawnPoints :type Array%20of%20F%20Unit%20Spawn%20Point%20Structures))
  (bind _localteamnames (LocalVariables|GetLocalTeamNames))
  (for _array_element SpawnPoints
    (Utilities|Map|Add (LocalVariables|GetLocalTeamNames) (Utilities|Struct|BreakF_UnitSpawnPoint _array_element) ""))
  (bind _keys (Utilities|Map|Keys _localteamnames))
  (for _array_element_2 _keys
    (bind _outrownames (DataTable|GetDataTableRowNames "/Game/Data/Procedural/DT_NamePartsArticles.DT_NamePartsArticles"))
    (bind _returnvalue (Utilities|GetDataTableRow "/Game/Data/Procedural/DT_NamePartsArticles.DT_NamePartsArticles" (.OutItem (Utilities|Array|Random _outrownames)))
      (:then
        (LocalVariables|SetCurrArticle (.prefix _returnvalue)))
      (:RowNotFound
        (LocalVariables|SetCurrArticle "")))
    (switch int (Math|Random|RandomInteger 3)
      (:0
        (bind _outrownames_2 (DataTable|GetDataTableRowNames "/Game/Data/Procedural/DT_NamePartsNegative.DT_NamePartsNegative"))
        (bind _returnvalue_2 (Utilities|GetDataTableRow "/Game/Data/Procedural/DT_NamePartsNegative.DT_NamePartsNegative" (.OutItem (Utilities|Array|Random _outrownames_2)))
          (:then
            (LocalVariables|SetCurrAdjective (.Adjective (Utilities|Struct|BreakF_TeamNameParts _returnvalue_2))))
          (:RowNotFound
            (LocalVariables|SetCurrAdjective ""))))
      (:1
        (bind _outrownames_3 (DataTable|GetDataTableRowNames "/Game/Data/Procedural/DT_NamePartsNeutral.DT_NamePartsNeutral"))
        (bind _returnvalue_3 (Utilities|GetDataTableRow "/Game/Data/Procedural/DT_NamePartsNeutral.DT_NamePartsNeutral" (.OutItem (Utilities|Array|Random _outrownames_3)))
          (:then
            (LocalVariables|SetCurrAdjective (.Adjective (Utilities|Struct|BreakF_TeamNameParts _returnvalue_3))))
          (:RowNotFound
            (LocalVariables|SetCurrAdjective ""))))
      (:2
        (bind _outrownames_4 (DataTable|GetDataTableRowNames "/Game/Data/Procedural/DT_NamePartsPositive.DT_NamePartsPositive"))
        (bind _returnvalue_4 (Utilities|GetDataTableRow "/Game/Data/Procedural/DT_NamePartsPositive.DT_NamePartsPositive" (.OutItem (Utilities|Array|Random _outrownames_4)))
          (:then
            (LocalVariables|SetCurrAdjective (.Adjective (Utilities|Struct|BreakF_TeamNameParts _returnvalue_4))))
          (:RowNotFound
            (LocalVariables|SetCurrAdjective "")))))
    (switch int (Math|Random|RandomInteger 3)
      (:0
        (bind _outrownames_5 (DataTable|GetDataTableRowNames "/Game/Data/Procedural/DT_NamePartsNegative.DT_NamePartsNegative"))
        (bind _returnvalue_5 (Utilities|GetDataTableRow "/Game/Data/Procedural/DT_NamePartsNegative.DT_NamePartsNegative" (.OutItem (Utilities|Array|Random _outrownames_5)))
          (:then
            (LocalVariables|SetCurrNoun (.Noun (Utilities|Struct|BreakF_TeamNameParts _returnvalue_5))))
          (:RowNotFound
            (LocalVariables|SetCurrNoun ""))))
      (:1
        (bind _outrownames_6 (DataTable|GetDataTableRowNames "/Game/Data/Procedural/DT_NamePartsNeutral.DT_NamePartsNeutral"))
        (bind _returnvalue_6 (Utilities|GetDataTableRow "/Game/Data/Procedural/DT_NamePartsNeutral.DT_NamePartsNeutral" (.OutItem (Utilities|Array|Random _outrownames_6)))
          (:then
            (LocalVariables|SetCurrNoun (.Noun (Utilities|Struct|BreakF_TeamNameParts _returnvalue_6))))
          (:RowNotFound
            (LocalVariables|SetCurrNoun ""))))
      (:2
        (bind _outrownames_7 (DataTable|GetDataTableRowNames "/Game/Data/Procedural/DT_NamePartsPositive.DT_NamePartsPositive"))
        (bind _returnvalue_7 (Utilities|GetDataTableRow "/Game/Data/Procedural/DT_NamePartsPositive.DT_NamePartsPositive" (.OutItem (Utilities|Array|Random _outrownames_7)))
          (:then
            (LocalVariables|SetCurrNoun (.Noun (Utilities|Struct|BreakF_TeamNameParts _returnvalue_7))))
          (:RowNotFound
            (LocalVariables|SetCurrNoun "")))))
    (Utilities|Map|Add _localteamnames _array_element_2 (Utilities|String|StringToName (Utilities|String|Append (LocalVariables|GetCurrArticle) " " (LocalVariables|GetCurrAdjective) " " (LocalVariables|GetCurrNoun)))))
  (return _localteamnames))

(fn GetAllUnits
  (return 0))

(fn GetTacticalCortex
  (return (Variables|Navigation|GetTacticalCortex)))