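; BP_TacticalNode is a data object for one tile of the tactical map, holding position, terrain type, character height, four edge heights and pickups.
; NewTacticalNode constructs a node and fills its heights from the DT_TileShapeInfo row named after the tile shape, always returning IsStandable as false.
; Helpers add and remove pickups, and a debug function prints position and heights, with the contents option left empty.
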(fn NewTacticalNode
  (params (TileShape :type E_TileShapes%20Enum :default "NewEnumerator29") (TerrainType :type E_TerrainTypes%20Enum :default "NewEnumerator0") (Position :type Int%20Vector%20Structure))
  (bind _returnvalue (Game|ConstructObjectfromClass "BP_TacticalNode_C"))
  (Variables|BP_TacticalNode_C|SetPosition _returnvalue Position)
  (Variables|BP_TacticalNode_C|SetTerrainType _returnvalue TerrainType)
  (bind _returnvalue_2 (Utilities|GetDataTableRow "/Game/Blueprints/DT_TileShapeInfo.DT_TileShapeInfo" (Utilities|Name|EnumtoName TileShape))
    (:then
      (Variables|BP_TacticalNode_C|SetPlayerHeight _returnvalue (.characterheight _returnvalue_2))
      (Variables|BP_TacticalNode_C|SetNorthEdgeHeight _returnvalue (.edgeheightnorth _returnvalue_2))
      (Variables|BP_TacticalNode_C|SetEastEdgeHeight _returnvalue (.edgeheighteast _returnvalue_2))
      (Variables|BP_TacticalNode_C|SetSouthEdgeHeight _returnvalue (.edgeheightsouth _returnvalue_2))
      (Variables|BP_TacticalNode_C|SetWestEdgeHeight _returnvalue (.edgeheightwest _returnvalue_2))
      (return _returnvalue false))
    (:RowNotFound
      (Development|PrintString 0 "tile shape info not found"))))

(fn AddPickup
  (params (TacticalNode :type BP%20Tactical%20Node%20Object%20Reference) (Pickup :type Pawn%20Object%20Reference))
  (bind _returnvalue (Utilities|Array|Add (Variables|BP_TacticalNode_C|GetPickups TacticalNode) Pickup))
  (return _returnvalue))

(fn RemovePickup
  (params (TacticalNode :type BP%20Tactical%20Node%20Object%20Reference) (Pickup :type Pawn%20Object%20Reference))
  (bind _pickups (Variables|BP_TacticalNode_C|GetPickups TacticalNode))
  (Utilities|Array|RemoveIndex _pickups (Utilities|Array|FindItem _pickups Pickup)))

(fn PrintTacticalNodeData
  (params (Position :type Boolean) (Heights :type Boolean) (Contents :type Boolean))
  (if Position
    (bind _output_get (LocalVariables|SetprintString (Utilities|String|Append (LocalVariables|GetprintString) "X: " (Utilities|String|ToString(Integer) (.x (Variables|TacticalContents|GetPosition))) " Y: " (Utilities|String|ToString(Integer) (.y (Variables|TacticalContents|GetPosition))) " Z: " (Utilities|String|ToString(Integer) (.z (Variables|TacticalContents|GetPosition)))))))
  (if Heights
    (bind _output_get_2 (LocalVariables|SetprintString (Utilities|String|Append _output_get "\\nHeights:\\nP: " (Utilities|String|ToString(Integer) (Variables|TacticalElevationOffsets|GetPlayerHeight)) " N: " (Utilities|String|ToString(Integer) (Variables|TacticalElevationOffsets|GetNorthEdgeHeight)) " E: " (Utilities|String|ToString(Integer) (Variables|TacticalElevationOffsets|GetEastEdgeHeight)) " S: " (Utilities|String|ToString(Integer) (Variables|TacticalElevationOffsets|GetSouthEdgeHeight)) " W: " (Utilities|String|ToString(Integer) (Variables|TacticalElevationOffsets|GetWestEdgeHeight))))))
  (if Contents
    _
    (else
      _))
  (Development|PrintString 0 _output_get_2 true true "(R=0.000000,G=0.660000,B=1.000000,A=1.000000)" 6e+01)
  (return))