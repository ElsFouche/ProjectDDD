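; BP_TacticalCortex is a registry of navigable tactical nodes, indexed by grid position.
; NavigablePoints maps each XY coordinate to an FTacticalArray struct, whose inner map keys nodes by Z so several can share a column.
; AddNode files a valid node under its position, creating the XY entry when missing.
; PrintNodes walks both map levels to print every node's position, heights and contents for debugging.
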(fn AddNode
  (params (NewNode :type BP%20Tactical%20Node%20Object%20Reference))
  (bind _position (Variables|/Game/Blueprints/TacticalCortex/BP_TacticalNode.BP_TacticalNode_C|GetPosition NewNode))
  (bind _navigablepoints (Variables|Default|GetNavigablePoints))
  (bind (_value _returnvalue) (Utilities|Map|Find _navigablepoints (Utilities|Struct|MakeF_IntVector2d (.x _position) (.y _position))))
  (Utilities|IsValid NewNode
    (:Is%20Valid
      (if _returnvalue
        (Utilities|Map|Add (Utilities|Struct|BreakF_TacticalArray _value) (.z _position) NewNode)
        (else
          (Utilities|Map|Add _navigablepoints (Utilities|Struct|MakeF_IntVector2d (.x _position) (.y _position)) (Utilities|Struct|MakeF_TacticalArray (Utilities|Map|MakeMap (.z _position) NewNode))))))))

(fn PrintNodes
  (bind _navigablepoints (Variables|Default|GetNavigablePoints))
  (bind _keys (Utilities|Map|Keys _navigablepoints))
  (for _array_element _keys
    (bind _keys_2 (Utilities|Map|Keys (Utilities|Struct|BreakF_TacticalArray (.Value (Utilities|Map|Find _navigablepoints _array_element)))))
    (for _array_element_2 _keys_2
      (Default|PrintTacticalNodeData (.Value (Utilities|Map|Find (Utilities|Struct|BreakF_TacticalArray (.Value (Utilities|Map|Find _navigablepoints _array_element))) _array_element_2)) true true true))))