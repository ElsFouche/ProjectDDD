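; Blueprint function library for the tactical system, providing a factory that creates BP_TacticalNode objects to represent tiles.
; NewTacticalNode constructs the node on the given owner and stores its position and terrain type.
; It uses the tile shape enum's name as the row key into DT_TileShapeInfo to fill in character height and the four compass edge heights.
; A missing row only prints an error.
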(fn NewTacticalNode
  (params (Owner :type Object%20Object%20Reference) (TileShape :type E_TileShapes%20Enum :default "NewEnumerator29") (TerrainType :type E_TerrainTypes%20Enum :default "NewEnumerator0") (Position :type Int%20Vector%20Structure))
  (bind _returnvalue (Game|ConstructObjectfromClass Owner "/Game/Blueprints/TacticalCortex/BP_TacticalNode.BP_TacticalNode_C"))
  (Utilities|IsValid _returnvalue
    (:Is%20Valid
      (Variables|/Game/Blueprints/TacticalCortex/BP_TacticalNode.BP_TacticalNode_C|SetPosition _returnvalue Position)
      (Variables|/Game/Blueprints/TacticalCortex/BP_TacticalNode.BP_TacticalNode_C|SetTerrainType _returnvalue TerrainType)
      (bind _returnvalue_2 (Utilities|GetDataTableRow "/Game/Blueprints/DT_TileShapeInfo.DT_TileShapeInfo" (Utilities|String|StringToName (Utilities|String|EnumtoString TileShape)))
        (:then
          (Variables|/Game/Blueprints/TacticalCortex/BP_TacticalNode.BP_TacticalNode_C|SetPlayerHeight _returnvalue (.characterheight _returnvalue_2))
          (Variables|/Game/Blueprints/TacticalCortex/BP_TacticalNode.BP_TacticalNode_C|SetNorthEdgeHeight _returnvalue (.edgeheightnorth _returnvalue_2))
          (Variables|/Game/Blueprints/TacticalCortex/BP_TacticalNode.BP_TacticalNode_C|SetEastEdgeHeight _returnvalue (.edgeheighteast _returnvalue_2))
          (Variables|/Game/Blueprints/TacticalCortex/BP_TacticalNode.BP_TacticalNode_C|SetSouthEdgeHeight _returnvalue (.edgeheightsouth _returnvalue_2))
          (Variables|/Game/Blueprints/TacticalCortex/BP_TacticalNode.BP_TacticalNode_C|SetWestEdgeHeight _returnvalue (.edgeheightwest _returnvalue_2))
          (return _returnvalue))
        (:RowNotFound
          (Development|PrintString 0 "tile shape info not found"))))))