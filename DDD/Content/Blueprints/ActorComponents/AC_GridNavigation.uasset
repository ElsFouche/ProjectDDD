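; Grid navigation component that finds unit paths and movement ranges for tactical, tile-based movement.
; FindPath runs an A*-style search with Manhattan distances plus tile hazard, random tie-breaking and an iteration cap, then rebuilds the path from parent links.
; GetTilesInMoveRange recursively flood-fills reachable tiles, tracking remaining movement per tile.
; Both get neighboring moves, filtered by jump score, from the GameState's Tactical Cortex.
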(fn FindPath
  (params (StartLocation :type Int%20Vector%20Structure) (DesiredLocation :type Int%20Vector%20Structure) (VerticalTolerance :type Integer))
  (bind _gridsize (CallFunction|GetDefaultGridSize))
  (bind _possiblenexttiles (LocalVariables|GetPossibleNextTiles))
  (bind _numchecks (LocalVariables|GetNumChecks))
  (bind _alllocations (LocalVariables|GetAllLocations))
  (bind _possiblenexttiles_2 (LocalVariables|GetPossibleNextTiles))
  (bind _alllocations_2 (LocalVariables|GetAllLocations))
  (bind _alllocations_3 (LocalVariables|GetAllLocations))
  (bind _checklimit (LocalVariables|GetCheckLimit))
  (bind _pathpoints (LocalVariables|GetPathPoints))
  (bind _returnvalue (/ (.z _gridsize) 2))
  (bind _returnvalue_2 (< _numchecks _checklimit))
  ;[0.4924 0.5312 0.4748 0.5] Normalize Start and End Locations
  (bind _snappedpoint (GridNavigation|PointSnaptoGrid (Math|Conversions|ToVector(Float) StartLocation)))
  (LocalVariables|SetNormalizedStartLocation _snappedpoint)
  (bind _snappedpoint_2 (GridNavigation|PointSnaptoGrid (Math|Conversions|ToVector(Float) DesiredLocation)))
  (LocalVariables|SetNormalizedDesiredLocation _snappedpoint_2)
  ;[0.4924 0.5312 0.4748 0.5 12] Unit jump value is converted to half the grid size height value
  (bind _output_get (LocalVariables|SetJumpDistance (* VerticalTolerance _returnvalue)))
  ;[0.4924 0.5312 0.4748 0.5 12] Units may fall 25% further than they can jump. Round by half the grid height to account for half tiles.
  (bind _roundedvalue (CallFunction|RoundAround (+ _output_get (* _output_get 0.25)) _returnvalue))
  (LocalVariables|SetDropDistance _roundedvalue)
  ;[0.4924 0.5312 0.4748 0.5] Retrieve Tactical Cortex.
  (bind _tacticalcortex (Class|BPITacticalCortex|GetTacticalCortex(Message) (Game|GetGameState)))
  (Utilities|IsValid _tacticalcortex
    (:Is%20Valid
      (LocalVariables|SetTacticalCortex _tacticalcortex)
      ;[0.1303 0.1406 0.1257 0.5] Core Loop - while not at goal
      (LocalVariables|SetCurrentLocation (LocalVariables|GetNormalizedStartLocation))
      (while (and (not (Utilities|Equals(IntVector2d) (Utilities|ToIntVector2d (LocalVariables|GetCurrentLocation)) (Utilities|ToIntVector2d (LocalVariables|GetNormalizedDesiredLocation)))) _returnvalue_2)
        (Math|Integer|IncrementInt (LocalVariables|GetNumChecks)
          (:%20%20
            ;;[0.07734 0.15 0.09409 0.5] For each adjacent location
            (bind _validmoves (Default|FindMoves (LocalVariables|GetTacticalCortex) (LocalVariables|GetCurrentLocation) VerticalTolerance))
            (for _array_element _validmoves
              (bind _fvalue (GridNavigation|CalculateAStarFValue (LocalVariables|GetNormalizedStartLocation) (LocalVariables|GetNormalizedDesiredLocation) (.MoveDestination (Utilities|Struct|BreakF_MoveData _array_element)) (Utilities|Array|MakeArray (.HazardRating (Utilities|Struct|BreakF_MoveData _array_element)))))
              (if (or (< _fvalue (.fvalue (.Value (Utilities|Map|Find (LocalVariables|GetAllLocations) (.MoveDestination (Utilities|Struct|BreakF_MoveData _array_element)))))) (not (.ReturnValue (Utilities|Map|Find (LocalVariables|GetAllLocations) (.MoveDestination (Utilities|Struct|BreakF_MoveData _array_element))))))
                (Utilities|Map|Add (LocalVariables|GetAllLocations) (.MoveDestination (Utilities|Struct|BreakF_MoveData _array_element)) (Utilities|Struct|MakeF_AStarNavigation _fvalue (LocalVariables|GetCurrentLocation) false _array_element))))
            ;;[0.08493 0.0937 0.1615 0.5] Close our current tile and select the next tile to check from the list of all non-closed tiles.
            (Utilities|Map|Add _alllocations_3 (LocalVariables|GetCurrentLocation) (Utilities|Struct|MakeF_AStarNavigation (.fvalue (.Value (Utilities|Map|Find _alllocations_3 (LocalVariables|GetCurrentLocation)))) (.parentlocation (.Value (Utilities|Map|Find _alllocations_3 (LocalVariables|GetCurrentLocation)))) true (.unitmovedata (.Value (Utilities|Map|Find _alllocations_3 (LocalVariables|GetCurrentLocation))))))
            (LocalVariables|SetLowestF 100000)
            (bind _keys (Utilities|Map|Keys _alllocations_2))
            (for _array_element_2 _keys
              (if (not (.IsClosedLocation? (Utilities|Struct|BreakF_AStarNavigation (.Value (Utilities|Map|Find _alllocations_2 _array_element_2)))))
                (Math|Integer|CompareInt (.FValue (Utilities|Struct|BreakF_AStarNavigation (.Value (Utilities|Map|Find _alllocations_2 _array_element_2)))) (LocalVariables|GetLowestF)
                  (:==
                    (Utilities|Array|Add _possiblenexttiles _array_element_2))
                  (:<
                    (Utilities|Array|Clear _possiblenexttiles)
                    (Utilities|Array|Add _possiblenexttiles _array_element_2)
                    (LocalVariables|SetLowestF (.FValue (Utilities|Struct|BreakF_AStarNavigation (.Value (Utilities|Map|Find _alllocations_2 _array_element_2)))))))))
            (LocalVariables|SetCurrentLocation (.OutItem (Utilities|Array|Random _possiblenexttiles_2)))
            (Utilities|Array|Clear _possiblenexttiles_2))))
      ;[0.142 0.0911 0.15 0.5] Once a path has been found, populate the output array with data and return. Only proceed if the number of checks was not exceeded to prevent sending out junk data.
      (if _returnvalue_2
        ;;[0.2612 0.1676 0.276 0.5] Data population loop. Works backwards through the generated path by using the parent location as the index for the next piece of path data.
        ;;;[0.4042 0.2594 0.4271 0.5] Initialize our output array with the current location's data.
        (Utilities|Array|Add (LocalVariables|GetPathPoints) (.unitmovedata (.Value (Utilities|Map|Find (LocalVariables|GetAllLocations) (LocalVariables|GetCurrentLocation)))))
        (while (not (Utilities|Equals(IntVector2d) (Utilities|ToIntVector2d (LocalVariables|GetCurrentLocation)) (Utilities|ToIntVector2d (LocalVariables|GetNormalizedStartLocation))))
          ;;;[0.4042 0.2594 0.4271 0.5] Retrieve the parent of our current location and populate our output array with the parent's data.
          (Utilities|Array|Add (LocalVariables|GetPathPoints) (.unitmovedata (.Value (Utilities|Map|Find _alllocations (.parentlocation (.Value (Utilities|Map|Find _alllocations (LocalVariables|GetCurrentLocation))))))))
          (LocalVariables|SetCurrentLocation (.parentlocation (.Value (Utilities|Map|Find _alllocations (LocalVariables|GetCurrentLocation))))))
        ;;[0.2612 0.1676 0.276 0.5] Return path, ordered start to finish
        (Utilities|Array|Reverse _pathpoints)
        (return _pathpoints true)
        (else
          (Development|PrintString (Utilities|String|Append "Path generation failed: " "CheckLimit exceeded. " "CheckLimit: " (Utilities|String|ToString(Integer) (LocalVariables|GetCheckLimit))) false true "(R=0.000000,G=0.660000,B=1.000000,A=1.000000)" 0.0)
          (return 0 false))))
    (:Is%20Not%20Valid
      (return 0 false))))

(fn PointSnaptoGrid
  (params (InPoint :type Vector))
  (bind _gridsize (CallFunction|GetDefaultGridSize))
  (bind _returnvalue (Math|Float|Truncate (.z InPoint)))
  (bind _returnvalue_2 (Math|Float|Truncate (.x InPoint)))
  (bind _returnvalue_3 (Math|Float|Truncate (.y InPoint)))
  (bind _gridsize_2 (CallFunction|GetDefaultGridSize))
  (return (Utilities|Struct|MakeIntVector (+ (- _returnvalue_2 (Utilities|Int% _returnvalue_2 (Math|Integer|Absolute(Integer) (.x _gridsize_2)))) (/ (.x _gridsize) 2)) (+ (/ (.y _gridsize) 2) (- _returnvalue_3 (Utilities|Int% _returnvalue_3 (Math|Integer|Absolute(Integer) (.y _gridsize_2))))) (- _returnvalue (Utilities|Int% _returnvalue (Math|Integer|Absolute(Integer) (.z _gridsize_2)))))))

(fn CalculateAStarFValue
  (params (StartPos :type Int%20Vector%20Structure) (EndPos :type Int%20Vector%20Structure) (CurrPos :type Int%20Vector%20Structure) (AddHeuristics :type Array%20of%20Integers))
  (bind _gridsize (CallFunction|GetDefaultGridSize))
  (bind ____ (Utilities|Divide(IntVector) CurrPos _gridsize))
  (bind ___ (Utilities|ToIntVector2d ____))
  ;[0.15 0.15 0.15 0.5] Accumulate additional heuristics
  (LocalVariables|SetTempFValue (+ (Utilities|ManhattenDistance(2d) (Utilities|ToIntVector2d (Utilities|Divide(IntVector) StartPos _gridsize)) ___) (Utilities|ManhattenDistance(2d) ___ (Utilities|ToIntVector2d (Utilities|Divide(IntVector) EndPos _gridsize)))))
  (for _array_element AddHeuristics
    (LocalVariables|SetTempFValue (+ _array_element (LocalVariables|GetTempFValue))))
  (return (LocalVariables|GetTempFValue)))

(fn GetTilesinMoveRange
  (params (StartPosition :type Int%20Vector%20Structure) (UnitMove :type Integer) (UnitJump :type Integer))
  (bind _tacticalcortex (Class|BPITacticalCortex|GetTacticalCortex(Message) (Game|GetGameState)))
  (Utilities|IsValid _tacticalcortex
    (:Is%20Valid
      (bind _output_get (LocalVariables|SetTacticalCortex _tacticalcortex))
      ;[0.01731 0.06886 0.151 0.5] MoveCheckRecursive is called continuously, checking each point before finding that point's neightbors and calling itself to check those.
      ; Exit conditions:
      ; - Movement depleted
      ; - Node found but has the same or worse movement cost
      ; - Final node found and checked
      (Helpers|MoveCheckRecursive (Utilities|Struct|MakeF_MoveData StartPosition) UnitMove UnitJump (LocalVariables|GetPossibleMoves) _output_get)
      (bind _keys (Utilities|Map|Keys (LocalVariables|GetPossibleMoves)))
      (return _keys))))

(fn MoveCheckRecursive
  (params (MoveToCheck :type F%20Move%20Data%20Structure%20%28by%20ref%29) (RemainingMovement :type Integer) (JumpScore :type Integer) (PossibleMoves :type Map%20of%20Int%20Vector%20Structures%20to%20Integers) (TacticalCortex :type BP%20Tactical%20Cortex%20Object%20Reference%20%28by%20ref%29))
  (bind (_movedestination _movecost) (Utilities|Struct|BreakF_MoveData MoveToCheck))
  (bind (_value _returnvalue) (Utilities|Map|Find PossibleMoves _movedestination))
  (bind _returnvalue_2 (- RemainingMovement _movecost))
  (if (<= _movecost RemainingMovement)
    (if _returnvalue
      (if (< _returnvalue_2 _value)
        (return)
        (else
          _)))
    (Utilities|Map|Add PossibleMoves _movedestination _returnvalue_2)
    ;[0.15 0.15 0.15 0.5] Recursion
    (bind _validmoves (Default|FindMoves TacticalCortex _movedestination JumpScore))
    (bind _arrayelement (Utilities|ForEachLoopReal _validmoves :!label _label)
      (:LoopBody
        (Helpers|MoveCheckRecursive _arrayelement (.Value (Utilities|Map|Find PossibleMoves _movedestination)) JumpScore PossibleMoves TacticalCortex)
        (goto _label Continue))
      (:Completed
        (return)))
    (else
      (return))))