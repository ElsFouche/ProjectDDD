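; Blueprint function library for weighted random decisions over maps of named choices to float weights.
; Pick shuffles the keys, then subtracts weights from a random fraction of the total until it reaches zero, failing on an empty map.
; Helpers build maps from parallel arrays, merge weights additively, and scale them per key or uniformly.
; CalculateEntropy measures a distribution's Shannon entropy in bits, normalising by the same SumWeights total that Pick uses.
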(fn Pick
  (params (Weights :type Map%20of%20Names%20to%20Reals))
  (if (<= (Utilities|Map|Length Weights) 0)
    (return "None" false)
    (else
      (bind _output_get (LocalVariables|SetLocal%20Weights Weights))
      (bind _keys (Utilities|Map|Keys _output_get))
      (bind _output_get_2 (LocalVariables|SetKeys _keys))
      (Utilities|Array|Shuffle _output_get_2)
      (LocalVariables|SetWeightAcc (* (CallFunction|SumWeights (LocalVariables|GetLocal%20Weights)) (Math|Random|RandomFloat)))
      ;[0.15 0.15 0.15 0.5] Real For Each Loop. (actually waits for each loop body to complete before doing the next one)
      (bind _output_get_3 (LocalVariables|SetCounter 0))
      (if (< _output_get_3 (Utilities|Array|Length _output_get_2)) :!label _label
        (bind _output_get_4 (LocalVariables|SetCurrentChoice (Utilities|Array|Get(acopy) _output_get_2 _output_get_3)))
        (if (<= (- (LocalVariables|GetWeightAcc) (.Value (Utilities|Map|Find (LocalVariables|GetLocal%20Weights) _output_get_4))) 0.0)
          _
          (else
            (LocalVariables|SetWeightAcc (- (LocalVariables|GetWeightAcc) (.Value (Utilities|Map|Find (LocalVariables|GetLocal%20Weights) _output_get_4))))
            (Math|Integer|IncrementInt _output_get_3
              (:%20%20
                (goto _label))))))
      (return (LocalVariables|GetCurrentChoice) true))))

(fn CalculateEntropy
  (params (Weights :type Map%20of%20Names%20to%20Reals))
  (LocalVariables|SetWeightAcc (CallFunction|SumWeights Weights))
  (LocalVariables|SetEntropyAcc 0.0)
  (bind _values (Utilities|Map|Values Weights))
  ;[0.15 0.15 0.15 0.5] Real For Each Loop. (actually waits for each loop body to complete before doing the next one)
  (bind _output_get (LocalVariables|SetCounter 0))
  (if (< _output_get (Utilities|Array|Length _values)) :!label _label
    (LocalVariables|SetEntropyAcc (- (LocalVariables|GetEntropyAcc) (* (/ (Utilities|Array|Get(acopy) _values _output_get) (LocalVariables|GetWeightAcc)) (Math|Float|Log (/ (Utilities|Array|Get(acopy) _values _output_get) (LocalVariables|GetWeightAcc)) 2.0))))
    (Math|Integer|IncrementInt _output_get
      (:%20%20
        (goto _label)))
    (else
      (return (LocalVariables|GetEntropyAcc)))))

(fn SumWeights
  (params (Weights :type Map%20of%20Names%20to%20Reals))
  (LocalVariables|SetWeightAcc 0.0)
  (bind _values (Utilities|Map|Values Weights))
  (for _array_element _values
    (LocalVariables|SetWeightAcc (+ _array_element (LocalVariables|GetWeightAcc))))
  (return (LocalVariables|GetWeightAcc)))

(fn AddWeights
  (params (Target :type Map%20of%20Names%20to%20Reals) (AddedWeights :type Map%20of%20Names%20to%20Reals))
  (bind _keys (Utilities|Map|Keys AddedWeights))
  (for _array_element _keys
    (if (.ReturnValue (Utilities|Map|Find Target _array_element))
      (Utilities|Map|Add Target _array_element (+ (.Value (Utilities|Map|Find Target _array_element)) (.Value (Utilities|Map|Find AddedWeights _array_element))))
      (else
        (Utilities|Map|Add Target _array_element (.Value (Utilities|Map|Find AddedWeights _array_element))))))
  (return))

(fn ScaleWeights
  (params (Weights :type Map%20of%20Names%20to%20Reals) (ScaledWeights :type Map%20of%20Names%20to%20Reals))
  (bind _keys (Utilities|Map|Keys ScaledWeights))
  (for _array_element _keys
    (if (.ReturnValue (Utilities|Map|Find Weights _array_element))
      (Utilities|Map|Add Weights _array_element (* (.Value (Utilities|Map|Find Weights _array_element)) (.Value (Utilities|Map|Find ScaledWeights _array_element))))))
  (return))

(fn ScaleWeightsUniform
  (params (Weights :type Map%20of%20Names%20to%20Reals) (ScalingFactor :type Float%20%28double-precision%29))
  (bind _keys (Utilities|Map|Keys Weights))
  (for _array_element _keys
    (Utilities|Map|Add Weights _array_element (* (.Value (Utilities|Map|Find Weights _array_element)) ScalingFactor)))
  (return))

(fn ToWeightedChoices
  (params (Names :type Array%20of%20Names) (Weights :type Array%20of%20Floats%20%28double-precision%29))
  (for _index (range 0 (- (Math|Integer|Min(Integer) (Utilities|Array|Length Names) (Utilities|Array|Length Weights)) 1))
    (Utilities|Map|Add (LocalVariables|GetLocalWeights) (Utilities|Array|Get(acopy) Names _index) (Utilities|Array|Get(acopy) Weights _index)))
  (return (LocalVariables|GetLocalWeights)))