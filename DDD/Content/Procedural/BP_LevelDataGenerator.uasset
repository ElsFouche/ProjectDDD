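; BP_LevelDataGenerator is an actor that procedurally generates maze-based level data when play begins.
; On BeginPlay it adds an AC_MazeGenerator component, then chains maze generation, level-info generation and parsing into PCG tile data.
; Each stage prints its output for debugging, and an unconnected loop prints index-to-position round-trip conversions as a test.
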(event EventBeginPlay
  (bind _dimensions (Variables|Default|GetDimensions))
  (bind _returnvalue (Game|AddComponentbyClass "/Game/Procedural/AC_MazeGenerator.AC_MazeGenerator_C"))
  (Variables|Default|SetChosenRoomGenerator _returnvalue)
  (bind _mazedata (Default|GenerateMaze _returnvalue _dimensions 0.5 0.5))
  (Development|PrintString (Utilities|String|Append "number of maze nodes: " (Utilities|String|ToString(Integer) (Utilities|Map|Length _mazedata))))
  (bind _leveldata (Default|MazeLevelInfoGenerator _returnvalue _mazedata _dimensions))
  (Development|PrintString (Utilities|String|Append "number of tiles after level info generation: " (Utilities|String|ToString(Integer) (Utilities|Map|Length (.TileInfo (Utilities|Struct|BreakF_LevelInfo _leveldata))))))
  (bind _pcgdata (Default|ParseLevelInfo _returnvalue _leveldata))
  (Development|PrintString (Utilities|String|Append "number of tiles after parsing: " (Utilities|String|ToString(Integer) (.Tiles (Utilities|Struct|BreakF_PCGData _pcgdata))))))

(event Collision|EventActorBeginOverlap
  (params (OtherActor :type Actor%20Object%20Reference)))

(event EventTick
  (params (DeltaSeconds :type Float%20%28single-precision%29)))

(fn ConstructionScript)