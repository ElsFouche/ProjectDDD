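; Procedural maze generator component that grows a randomly branching maze on a half-resolution grid with a cellular automaton.
; GenerateMaze cycles nodes through Disconnected, Seed, Invite and Connected using double-buffered Old/New states, storing parent directions and printing debug output.
; MazeLevelInfoGenerator converts nodes and parent links into air tiles amid solid tiles, over a solid floor.
; TurningFactor is unused, MazeCALogic duplicates the inline automaton, and GenerateMaze's level-building stage is unreachable WIP.
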(event EventBeginPlay
  (|CallParentFunction) ; This node is disabled and will not be called.\nDrag off pins to build functionality.
)

(event EventTick
  (params (DeltaSeconds :type Float%20%28single-precision%29))
  (|CallParentFunction DeltaSeconds) ; This node is disabled and will not be called.\nDrag off pins to build functionality.
)

(fn GenerateMaze
  (params (Dimensions :type Int%20Vector%20Structure) (BranchingFactor :type Float%20%28double-precision%29) (TurningFactor :type Float%20%28double-precision%29))
  (bind _returnvalue (Math|Float|Clamp(Float) BranchingFactor))
  (bind _2d (Utilities|ToIntVector2d Dimensions))
  (bind _f_mazenode (Utilities|Struct|MakeF_MazeNode "NewEnumerator0" "NewEnumerator0" "NewEnumerator0"))
  (bind _mazenodes (Variables|Default|GetMazeNodes))
  (bind _neighbors (Variables|Default|GetNeighbors))
  (bind _mazenodes_2 (Variables|Default|GetMazeNodes))
  (bind _neighbors_2 (Variables|Default|GetNeighbors))
  (bind _mazenodes_3 (Variables|Default|GetMazeNodes))
  (bind _neighbors_3 (Variables|Default|GetNeighbors))
  (bind (_outitem _outindex) (Utilities|Array|Random _neighbors_3))
  (bind (_outitem_2 _outindex_2) (Utilities|Array|Random _neighbors))
  (bind (_outitem_3 _outindex_3) (Utilities|Array|Random _neighbors_2))
  (bind _out (Utilities|-(2d) _2d (Utilities|Struct|MakeF_IntVector2d 1 1)))
  (bind _out_2 (Utilities|/(2d) _out (Utilities|Struct|MakeF_IntVector2d 2 2)))
  (bind _returnvalue_2 (!= _outindex_2 -1))
  (bind _returnvalue_3 (!= _outindex -1))
  (bind _returnvalue_4 (!= _outindex_3 -1))
  (bind (_x _y) (Utilities|Struct|BreakF_IntVector2d _out_2))
  (bind _out_3 (Utilities|-(2d) _out_2 (Utilities|Struct|MakeF_IntVector2d 1 1)))
  (bind _returnvalue_5 (select _returnvalue_4 _outitem_3 "NewEnumerator0"))
  (bind _returnvalue_6 (select _returnvalue_4 "NewEnumerator2" "NewEnumerator3"))
  (bind _f_mazenode_2 (Utilities|Struct|MakeF_MazeNode _returnvalue_6 _returnvalue_5 _returnvalue_5))
  (Variables|Default|SetDimensions Dimensions)
  (CallFunction|ClearLevelInfo)
  ;[0.15 0.15 0.15 0.5] Initialize All Maze Nodes as Disconnected
  (for _index (range 0 (.x _out_3))
    (for _index_2 (range 0 (.y _out_3))
      (Utilities|Map|Add (Variables|Default|GetMazeNodes) (Utilities|Struct|MakeF_IntVector2d _index _index_2) (Utilities|Struct|MakeF_HistoricalMazeNode _f_mazenode _f_mazenode))))
  ;[0.15 0.15 0.15 0.5 30] Choose one random node to be our seed node
  ;;[0.15 0.15 0.15 0.5] Get Disconnected Neighbors of Random Maze Node
  (bind _output_get (Variables|Default|SetStartingSeedPosition (Utilities|Struct|MakeF_IntVector2d (Math|Random|RandomInteger _x) (Math|Random|RandomInteger _y))))
  (bind _enumvalue (|ForEachE_Direction)
    (:LoopBody
      (if (and (Utilities|Enum|Equal(Enum) (.state (.old (.Value (Utilities|Map|Find (Variables|Default|GetMazeNodes) (Utilities|+(2d) _output_get (Utilities|ToUnitVector2d _enumvalue)))))) "NewEnumerator0") (.ReturnValue (Utilities|Map|Find (Variables|Default|GetMazeNodes) (Utilities|+(2d) _output_get (Utilities|ToUnitVector2d _enumvalue)))))
        (Utilities|Array|Add (Variables|Default|GetNeighbors) _enumvalue)))
    (:then
      ;;[0.15 0.15 0.15 0.5] If disconnected neighbors found, set state to invite and choose one to invite, otherwise, set to connected
      (Utilities|Map|Add (Variables|Default|GetMazeNodes) _output_get (Utilities|Struct|MakeF_HistoricalMazeNode _f_mazenode_2 _f_mazenode_2))
      ;;[0.15 0.15 0.15 0.5] Clean the Slate before the Cellular Automaton Starts
      (Variables|Default|SetisLiveSeeds false)
      (Variables|Default|SetisComplete false)
      (Utilities|Array|Clear (Variables|Default|GetNeighbors))
      (LocalVariables|SetDebugChecks 0)
      ;[0.15 0.15 0.15 0.5] Comment
      (Development|PrintString "Post Initialization:")
      (bind _keys (Utilities|Map|Keys _mazenodes_3))
      (for _array_element _keys
        (Development|PrintString (select (Utilities|Enum|NotEqual(Enum) (.state (.old (.Value (Utilities|Map|Find _mazenodes_3 _array_element)))) "NewEnumerator0") (Utilities|String|Append (Utilities|String|Append "X" (Utilities|String|ToString(Integer) (.x (Utilities|Struct|BreakF_IntVector2d _array_element))) " Y" (Utilities|String|ToString(Integer) (.y (Utilities|Struct|BreakF_IntVector2d _array_element))) " | " (Utilities|String|EnumtoString (.state (.old (.Value (Utilities|Map|Find _mazenodes_3 _array_element)))))) " Parent is at  X" (Utilities|String|ToString(Integer) (.x (Utilities|+(2d) (Utilities|ToUnitVector2d (.connectvector (.old (.Value (Utilities|Map|Find _mazenodes_3 _array_element))))) _array_element))) " Y" (Utilities|String|ToString(Integer) (.y (Utilities|+(2d) (Utilities|ToUnitVector2d (.connectvector (.old (.Value (Utilities|Map|Find _mazenodes_3 _array_element))))) _array_element)))) (Utilities|String|Append "X" (Utilities|String|ToString(Integer) (.x (Utilities|Struct|BreakF_IntVector2d _array_element))) " Y" (Utilities|String|ToString(Integer) (.y (Utilities|Struct|BreakF_IntVector2d _array_element))) " | " (Utilities|String|EnumtoString (.state (.old (.Value (Utilities|Map|Find _mazenodes_3 _array_element)))))))))
      (Development|PrintString "--------------")
      ;[0.15 0.15 0.15 0.5] CA Looper
      (while (not (Variables|Default|GetisComplete))
        ;[0.15 0.15 0.15 0.5 122] Maze Generation Cellular Automaton Loop
        ;;[0.15 0.15 0.15 0.5] iterate over all cells
        (bind _keys_2 (Utilities|Map|Keys (Variables|Default|GetMazeNodes)))
        (for _array_element_2 _keys_2
          (Utilities|Array|Clear (Variables|Default|GetNeighbors))
          (switch Utilities|FlowControl|Switch|SwitchonE_MazeNodeState (.State (Utilities|Struct|BreakF_MazeNode (.old (.Value (Utilities|Map|Find (Variables|Default|GetMazeNodes) _array_element_2)))))
            (:NewEnumerator0
              ;;[0.15 0.15 0.15 0.5 30] For Disconnected Cells
              ;;;[0.15 0.15 0.15 0.5] Get Inviting Neighbors
              (bind _enumvalue_2 (|ForEachE_Direction)
                (:LoopBody
                  (if (Math|Boolean|ANDBoolean (Utilities|Enum|Equal(Enum) (.state (.old (.Value (Utilities|Map|Find (Variables|Default|GetMazeNodes) (Utilities|+(2d) _array_element_2 (Utilities|ToUnitVector2d _enumvalue_2)))))) "NewEnumerator2") (Utilities|Enum|Equal(Enum) (.invitevector (.old (.Value (Utilities|Map|Find (Variables|Default|GetMazeNodes) (Utilities|+(2d) _array_element_2 (Utilities|ToUnitVector2d _enumvalue_2)))))) (Utilities|ReverseDirection _enumvalue_2)) (.ReturnValue (Utilities|Map|Find (Variables|Default|GetMazeNodes) (Utilities|+(2d) _array_element_2 (Utilities|ToUnitVector2d _enumvalue_2)))))
                    (Utilities|Array|Add (Variables|Default|GetNeighbors) _enumvalue_2)))
                (:then
                  ;;;[0.15 0.15 0.15 0.5] Pick a random inviting neighbor to connect to
                  (Utilities|Map|Add (Variables|Default|GetMazeNodes) _array_element_2 (Utilities|Struct|MakeF_HistoricalMazeNode (.old (.Value (Utilities|Map|Find (Variables|Default|GetMazeNodes) _array_element_2))) (Utilities|Struct|MakeF_MazeNode (select _returnvalue_3 "NewEnumerator1" (.State (Utilities|Struct|BreakF_MazeNode (.old (.Value (Utilities|Map|Find (Variables|Default|GetMazeNodes) _array_element_2)))))) (select _returnvalue_3 _outitem (.ConnectVector (Utilities|Struct|BreakF_MazeNode (.old (.Value (Utilities|Map|Find (Variables|Default|GetMazeNodes) _array_element_2)))))) (.InviteVector (Utilities|Struct|BreakF_MazeNode (.old (.Value (Utilities|Map|Find (Variables|Default|GetMazeNodes) _array_element_2))))))))
                  (Utilities|Array|Clear (Variables|Default|GetNeighbors)))))
            (:NewEnumerator1
              ;;[0.15 0.15 0.15 0.5 30] For Seed Cells
              ;;;[0.15 0.15 0.15 0.5] Get Disconnected Neighbors
              (bind _enumvalue_3 (|ForEachE_Direction)
                (:LoopBody
                  (if (and (Utilities|Enum|Equal(Enum) (.state (.old (.Value (Utilities|Map|Find (Variables|Default|GetMazeNodes) (Utilities|+(2d) _array_element_2 (Utilities|ToUnitVector2d _enumvalue_3)))))) "NewEnumerator0") (.ReturnValue (Utilities|Map|Find (Variables|Default|GetMazeNodes) (Utilities|+(2d) _array_element_2 (Utilities|ToUnitVector2d _enumvalue_3)))))
                    (Utilities|Array|Add (Variables|Default|GetNeighbors) _enumvalue_3)))
                (:then
                  ;;;[0.15 0.15 0.15 0.5] Choose random disconnected neighbor node to invite
                  (Utilities|Map|Add (Variables|Default|GetMazeNodes) _array_element_2 (Utilities|Struct|MakeF_HistoricalMazeNode (.old (.Value (Utilities|Map|Find (Variables|Default|GetMazeNodes) _array_element_2))) (Utilities|Struct|MakeF_MazeNode (select _returnvalue_2 "NewEnumerator2" "NewEnumerator3") (.ConnectVector (Utilities|Struct|BreakF_MazeNode (.old (.Value (Utilities|Map|Find (Variables|Default|GetMazeNodes) _array_element_2))))) (select _returnvalue_2 _outitem_2 (.InviteVector (Utilities|Struct|BreakF_MazeNode (.old (.Value (Utilities|Map|Find (Variables|Default|GetMazeNodes) _array_element_2)))))))))
                  (Utilities|Array|Clear (Variables|Default|GetNeighbors)))))
            (:NewEnumerator2
              ;;[0.15 0.15 0.15 0.5 30] For Invite Cells
              (Utilities|Map|Add (Variables|Default|GetMazeNodes) _array_element_2 (Utilities|Struct|MakeF_HistoricalMazeNode (.old (.Value (Utilities|Map|Find (Variables|Default|GetMazeNodes) _array_element_2))) (Utilities|Struct|MakeF_MazeNode (select (> _returnvalue (Math|Random|RandomFloatinRange 0.0 1.0)) "NewEnumerator1" "NewEnumerator3") (.ConnectVector (Utilities|Struct|BreakF_MazeNode (.old (.Value (Utilities|Map|Find (Variables|Default|GetMazeNodes) _array_element_2))))) (.InviteVector (Utilities|Struct|BreakF_MazeNode (.old (.Value (Utilities|Map|Find (Variables|Default|GetMazeNodes) _array_element_2))))))))
              (Utilities|Array|Clear (Variables|Default|GetNeighbors)))
            (:NewEnumerator3
              ;;[0.15 0.15 0.15 0.5 30] For Connected Seeds
              (if (Variables|Default|GetisLiveSeeds)
                ;;;[0.15 0.15 0.15 0.5] Possibly Convert to Seed if no current seeds, based on branching factor
                (Utilities|Map|Add (Variables|Default|GetMazeNodes) _array_element_2 (Utilities|Struct|MakeF_HistoricalMazeNode (.old (.Value (Utilities|Map|Find (Variables|Default|GetMazeNodes) _array_element_2))) (Utilities|Struct|MakeF_MazeNode (select (and (!= -1 (.OutIndex (Utilities|Array|Random (Variables|Default|GetNeighbors)))) (> _returnvalue (Math|Random|RandomFloatinRange 0.0 1.0))) "NewEnumerator1" (.State (Utilities|Struct|BreakF_MazeNode (.old (.Value (Utilities|Map|Find (Variables|Default|GetMazeNodes) _array_element_2)))))) (.ConnectVector (Utilities|Struct|BreakF_MazeNode (.old (.Value (Utilities|Map|Find (Variables|Default|GetMazeNodes) _array_element_2))))) (.InviteVector (Utilities|Struct|BreakF_MazeNode (.old (.Value (Utilities|Map|Find (Variables|Default|GetMazeNodes) _array_element_2))))))) :!label _label)
                (Utilities|Array|Clear (Variables|Default|GetNeighbors))
                (else
                  ;;;[0.15 0.15 0.15 0.5] Get Disconnected Neighbors
                  (bind _enumvalue_4 (|ForEachE_Direction)
                    (:LoopBody
                      (if (and (Utilities|Enum|Equal(Enum) (.state (.old (.Value (Utilities|Map|Find (Variables|Default|GetMazeNodes) (Utilities|+(2d) _array_element_2 (Utilities|ToUnitVector2d _enumvalue_4)))))) "NewEnumerator0") (.ReturnValue (Utilities|Map|Find (Variables|Default|GetMazeNodes) (Utilities|+(2d) _array_element_2 (Utilities|ToUnitVector2d _enumvalue_4)))))
                        (Utilities|Array|Add (Variables|Default|GetNeighbors) _enumvalue_4)))
                    (:then
                      (goto _label))))))))
        ;;[0.15 0.15 0.15 0.5] Reset and Check if Done
        (Math|Integer|IncrementInt (LocalVariables|GetDebugChecks)
          (:%20%20
            (Variables|Default|SetisLiveSeeds false)
            (Variables|Default|SetisComplete true)
            (bind _keys_3 (Utilities|Map|Keys _mazenodes))
            (for _array_element_3 _keys_3
              (if (and (not (Variables|Default|GetisLiveSeeds)) (Utilities|Enum|Equal(Enum) (.State (Utilities|Struct|BreakF_MazeNode (.new (.Value (Utilities|Map|Find _mazenodes _array_element_3))))) "NewEnumerator1"))
                (Variables|Default|SetisLiveSeeds true))
              (if (or (> (LocalVariables|GetDebugChecks) 50) (and (Variables|Default|GetisComplete) (Utilities|Enum|NotEqual(Enum) (.State (Utilities|Struct|BreakF_MazeNode (.new (.Value (Utilities|Map|Find _mazenodes _array_element_3))))) "NewEnumerator3")))
                (Variables|Default|SetisComplete false))
              (Utilities|Map|Add (Variables|Default|GetMazeNodes) _array_element_3 (Utilities|Struct|MakeF_HistoricalMazeNode (.new (.Value (Utilities|Map|Find _mazenodes _array_element_3))) (.new (.Value (Utilities|Map|Find _mazenodes _array_element_3))))))
            ;[0.15 0.15 0.15 0.5] Comment
            (Development|PrintString (Utilities|String|Append "Loop Number " (Utilities|String|ToString(Integer) (LocalVariables|GetDebugChecks))))
            (bind _keys_4 (Utilities|Map|Keys _mazenodes_2))
            (for _array_element_4 _keys_4
              (Development|PrintString (select (Utilities|Enum|NotEqual(Enum) (.state (.old (.Value (Utilities|Map|Find _mazenodes_2 _array_element_4)))) "NewEnumerator0") (Utilities|String|Append (Utilities|String|Append "X" (Utilities|String|ToString(Integer) (.x (Utilities|Struct|BreakF_IntVector2d _array_element_4))) " Y" (Utilities|String|ToString(Integer) (.y (Utilities|Struct|BreakF_IntVector2d _array_element_4))) " | " (Utilities|String|EnumtoString (.state (.old (.Value (Utilities|Map|Find _mazenodes_2 _array_element_4)))))) " Parent is at  X" (Utilities|String|ToString(Integer) (.x (Utilities|+(2d) (Utilities|ToUnitVector2d (.connectvector (.old (.Value (Utilities|Map|Find _mazenodes_2 _array_element_4))))) _array_element_4))) " Y" (Utilities|String|ToString(Integer) (.y (Utilities|+(2d) (Utilities|ToUnitVector2d (.connectvector (.old (.Value (Utilities|Map|Find _mazenodes_2 _array_element_4))))) _array_element_4)))) (Utilities|String|Append "X" (Utilities|String|ToString(Integer) (.x (Utilities|Struct|BreakF_IntVector2d _array_element_4))) " Y" (Utilities|String|ToString(Integer) (.y (Utilities|Struct|BreakF_IntVector2d _array_element_4))) " | " (Utilities|String|EnumtoString (.state (.old (.Value (Utilities|Map|Find _mazenodes_2 _array_element_4)))))))))
            (Development|PrintString "--------------"))))
      ;[0.15 0.15 0.15 0.5] Output finished maze node map
      (Utilities|Map|Clear (LocalVariables|GetMazeNodesOut))
      (bind _keys_5 (Utilities|Map|Keys (Variables|Default|GetMazeNodes)))
      (for _array_element_5 _keys_5
        (Utilities|Map|Add (LocalVariables|GetMazeNodesOut) _array_element_5 (.old (.Value (Utilities|Map|Find (Variables|Default|GetMazeNodes) _array_element_5)))))
      (return (LocalVariables|GetMazeNodesOut) true))))

(fn MazeCALogic
  (params (MazeNodes :type Map%20of%20F%20Int%20Vector%202d%20Structures%20to%20Structs) (Position :type F%20Int%20Vector%202d%20Structure) (Branching%20Factor :type Float%20%28double-precision%29) (TurningFactor :type Float%20%28double-precision%29))
  (bind _value (Utilities|Map|Find MazeNodes Position))
  (bind _neighbors (LocalVariables|GetNeighbors))
  (bind _neighbors_2 (LocalVariables|GetNeighbors))
  (bind (_state _connectvector _invitevector) (Utilities|Struct|BreakF_MazeNode (.old _value)))
  (bind (_state_2 _connectvector_2 _invitevector_2) (Utilities|Struct|BreakF_MazeNode (.old _value)))
  (bind (_state_3 _connectvector_3 _invitevector_3) (Utilities|Struct|BreakF_MazeNode (.old _value)))
  (bind (_state_4 _connectvector_4 _invitevector_4) (Utilities|Struct|BreakF_MazeNode (.old _value)))
  (bind (_outitem _outindex) (Utilities|Array|Random _neighbors_2))
  (bind (_outitem_2 _outindex_2) (Utilities|Array|Random _neighbors))
  (bind _returnvalue (!= _outindex_2 -1))
  (bind _returnvalue_2 (!= _outindex -1))
  (Utilities|Array|Clear (Variables|Default|GetNeighbors))
  (switch Utilities|FlowControl|Switch|SwitchonE_MazeNodeState (.State (Utilities|Struct|BreakF_MazeNode (.old _value)))
    (:NewEnumerator0
      ;[0.15 0.15 0.15 0.5 30] For Disconnected Cells
      ;;[0.15 0.15 0.15 0.5] Get Inviting Neighbors
      (bind _enumvalue (|ForEachE_Direction)
        (:LoopBody
          (if (Math|Boolean|ANDBoolean (Utilities|Enum|Equal(Enum) (.state (.old (.Value (Utilities|Map|Find (Variables|Default|GetMazeNodes) (Utilities|+(2d) Position (Utilities|ToUnitVector2d _enumvalue)))))) "NewEnumerator2") (Utilities|Enum|Equal(Enum) (.invitevector (.old (.Value (Utilities|Map|Find (Variables|Default|GetMazeNodes) (Utilities|+(2d) Position (Utilities|ToUnitVector2d _enumvalue)))))) (Utilities|ReverseDirection _enumvalue)) (.ReturnValue (Utilities|Map|Find (Variables|Default|GetMazeNodes) (Utilities|+(2d) Position (Utilities|ToUnitVector2d _enumvalue)))))
            (Utilities|Array|Add (LocalVariables|GetNeighbors) _enumvalue)))
        (:then
          ;;[0.15 0.15 0.15 0.5] Pick a random inviting neighbor to connect to
          (Utilities|Map|Add (Variables|Default|GetMazeNodes) Position (Utilities|Struct|MakeF_HistoricalMazeNode (.old _value) (Utilities|Struct|MakeF_MazeNode (select _returnvalue_2 "NewEnumerator1" _state_3) (select _returnvalue_2 _outitem _connectvector_3) _invitevector_3)))
          (Utilities|Array|Clear (LocalVariables|GetNeighbors)))))
    (:NewEnumerator1
      ;[0.15 0.15 0.15 0.5 30] For Seed Cells
      ;;[0.15 0.15 0.15 0.5] Get Disconnected Neighbors
      (bind _enumvalue_2 (|ForEachE_Direction)
        (:LoopBody
          (if (and (Utilities|Enum|Equal(Enum) (.state (.old (.Value (Utilities|Map|Find (Variables|Default|GetMazeNodes) (Utilities|+(2d) Position (Utilities|ToUnitVector2d _enumvalue_2)))))) "NewEnumerator0") (.ReturnValue (Utilities|Map|Find (Variables|Default|GetMazeNodes) (Utilities|+(2d) Position (Utilities|ToUnitVector2d _enumvalue_2)))))
            (Utilities|Array|Add (LocalVariables|GetNeighbors) _enumvalue_2)))
        (:then
          ;;[0.15 0.15 0.15 0.5] Choose random disconnected neighbor node to invite
          (Utilities|Map|Add (Variables|Default|GetMazeNodes) Position (Utilities|Struct|MakeF_HistoricalMazeNode (.old _value) (Utilities|Struct|MakeF_MazeNode (select _returnvalue "NewEnumerator2" "NewEnumerator3") _connectvector_2 (select _returnvalue _outitem_2 _invitevector_2))))
          (Utilities|Array|Clear (LocalVariables|GetNeighbors)))))
    (:NewEnumerator2
      ;[0.15 0.15 0.15 0.5 30] For Invite Cells
      (Utilities|Map|Add (Variables|Default|GetMazeNodes) Position (Utilities|Struct|MakeF_HistoricalMazeNode (.old _value) (Utilities|Struct|MakeF_MazeNode (select (> Branching%20Factor (Math|Random|RandomFloatinRange 0.0 1.0)) "NewEnumerator1" "NewEnumerator3") _connectvector_4 _invitevector_4)))
      (Utilities|Array|Clear (LocalVariables|GetNeighbors)))
    (:NewEnumerator3
      ;[0.15 0.15 0.15 0.5 30] For Connected Seeds
      (if (Variables|Default|GetisLiveSeeds)
        ;;[0.15 0.15 0.15 0.5] Possibly Convert to Seed if no current seeds, based on branching factor
        (Utilities|Map|Add (Variables|Default|GetMazeNodes) Position (Utilities|Struct|MakeF_HistoricalMazeNode (.old _value) (Utilities|Struct|MakeF_MazeNode (select (and (!= -1 (.OutIndex (Utilities|Array|Random (LocalVariables|GetNeighbors)))) (> Branching%20Factor (Math|Random|RandomFloatinRange 0.0 1.0))) "NewEnumerator1" _state) _connectvector _invitevector)) :!label _label)
        (Utilities|Array|Clear (LocalVariables|GetNeighbors))
        (else
          ;;[0.15 0.15 0.15 0.5] Get Disconnected Neighbors
          (bind _enumvalue_3 (|ForEachE_Direction)
            (:LoopBody
              (if (and (Utilities|Enum|Equal(Enum) (.state (.old (.Value (Utilities|Map|Find (Variables|Default|GetMazeNodes) (Utilities|+(2d) Position (Utilities|ToUnitVector2d _enumvalue_3)))))) "NewEnumerator0") (.ReturnValue (Utilities|Map|Find (Variables|Default|GetMazeNodes) (Utilities|+(2d) Position (Utilities|ToUnitVector2d _enumvalue_3)))))
                (Utilities|Array|Add (LocalVariables|GetNeighbors) _enumvalue_3)))
            (:then
              (goto _label))))))))

(fn MazeLevelInfoGenerator
  (params (MazeNodes :type Map%20of%20F%20Int%20Vector%202d%20Structures%20to%20Structs) (Dimensions :type Int%20Vector%20Structure))
  (for _index (range 0 (Utilities|GetLastIndex Dimensions))
    (Utilities|Array|Clear (LocalVariables|GetNeighbors))
    ;[0.15 0.15 0.15 0.5] If on first layer, Set to Solid
    (if (== (.Z (Utilities|Struct|BreakIntVector (.Position (Utilities|GetPositionfromIndex Dimensions _index)))) 0)
      (CallFunction|AddTile (.Position (Utilities|GetPositionfromIndex Dimensions _index)) "NewEnumerator1" "NewEnumerator0" "NewEnumerator0" (Utilities|Array|MakeArray "NewEnumerator1"))
      (else
        ;[0.15 0.15 0.15 0.5] Else If Maps to Maze Node, Set to Air
        (bind _ismazenodefound (Utilities|FindMazeNode (.Position (Utilities|GetPositionfromIndex Dimensions _index)) (Variables|Default|GetMazeNodes))
          (:Complete
            (if _ismazenodefound
              (CallFunction|AddTile (.Position (Utilities|GetPositionfromIndex Dimensions _index)) "NewEnumerator0" "NewEnumerator0" "NewEnumerator29" "NewEnumerator0")
              (else
                ;[0.15 0.15 0.15 0.5] Else if any adjacent space maps to a maze node and its parent vector points to our node, Set as Air
                (bind _array_element (Utilities|Array|ForEachLoopwithBreak (Utilities|Array|MakeArray "NewEnumerator0" "NewEnumerator1" "NewEnumerator2" "NewEnumerator3") :!label _label)
                  (:LoopBody
                    (bind (_mazenode _ismazenodefound_2) (Utilities|FindMazeNode (Utilities|+(3d) (.Position (Utilities|GetPositionfromIndex Dimensions _index)) (Utilities|ToIntVector (Utilities|ToUnitVector2d _array_element))) (Variables|Default|GetMazeNodes))
                      (:Complete
                        (if (and _ismazenodefound_2 (Utilities|Enum|Equal(Enum) (.connectvector _mazenode) (Utilities|ReverseDirection _array_element)))
                          (Utilities|Array|Add (Variables|Default|GetNeighbors) _array_element)
                          (goto _label Break)))))
                  (:Completed
                    (if (> (Utilities|Array|Length (LocalVariables|GetNeighbors)) 0)
                      (CallFunction|AddTile (.Position (Utilities|GetPositionfromIndex Dimensions _index)) "NewEnumerator0" "NewEnumerator0" "NewEnumerator29" "NewEnumerator0")
                      (else
                        ;[0.15 0.15 0.15 0.5] Else set to Solid
                        (CallFunction|AddTile (.Position (Utilities|GetPositionfromIndex Dimensions _index)) "NewEnumerator1" "NewEnumerator0" "NewEnumerator0" (Utilities|Array|MakeArray "NewEnumerator1")))))))))))))
  ;[0.15 0.15 0.15 0.5] When Done
  (return (Variables|Default|GetLevelInfo)))