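; Procedural level actor that generates a maze on BeginPlay and hands its tile data to a PCG component.
; GenerateLevel calls ACMazeGenerator.GenerateMaze, then unpacks the TileInfo structs into parallel arrays of position, yaw, terrain type and mesh path for PCG to read.
; Mesh soft object paths are built from tile shape enum names, and yaw comes from quarter-turn counts.
; PCG is notified after clearing and after repopulating; a failed generation only prints a message.
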(event EventBeginPlay
  (CallFunction|GenerateLevel (Variables|MazeInput|GetMazeDimensions) 0.5 1.0))

(fn ConstructionScript)

(fn GenerateLevel
  (params (MazeDimensions :type F%20Int%20Vector%202d%20Structure) (BranchingFactor :type Float%20%28double-precision%29) (TurningFactor :type Float%20%28double-precision%29))
  ;[0.15 0.15 0.15 0.5] Init: Delete old data and notify PCG of data change.
  (Utilities|Array|Clear (Variables|MazeOutput|GetTileInfo))
  (Utilities|Array|Clear (Variables|ExtractedTileData|GetTilePos))
  (Utilities|Array|Clear (Variables|ExtractedTileData|GetTileRot))
  (Utilities|Array|Clear (Variables|ExtractedTileData|GetTileType))
  (Utilities|Array|Clear (Variables|ExtractedTileData|GetTileShapeSOP))
  (Class|PCGComponent|NotifyPropertiesChangedfromBlueprint (Variables|Default|GetPCG))
  ;[0.15 0.15 0.15 0.5] Generate level. This section to be revised as more level types are created.
  (bind _output_get (Variables|MazeInput|SetMazeDimensions MazeDimensions))
  (bind (_tileinfo _issuccessful) (Default|GenerateMaze :self (Variables|Default|GetAC_MazeGenerator) :MazeNodeDimensions _output_get :BranchingFactor BranchingFactor :TurningFactor TurningFactor))
  (if _issuccessful
    (bind _output_get_2 (Variables|MazeOutput|SetTileInfo _tileinfo))
    ;[0.15 0.15 0.15 0.5] Set size of extracted data arrays to incoming data size
    (Utilities|Array|Resize (Variables|ExtractedTileData|GetTilePos) (Utilities|Array|Length _output_get_2))
    (Utilities|Array|Resize (Variables|ExtractedTileData|GetTileRot) (Utilities|Array|Length _output_get_2))
    (Utilities|Array|Resize (Variables|ExtractedTileData|GetTileType) (Utilities|Array|Length _output_get_2))
    (Utilities|Array|Resize (Variables|ExtractedTileData|GetTileShapeSOP) (Utilities|Array|Length _output_get_2))
    ;[0.15 0.15 0.15 0.5] Populate Arrays for PCG from TileInfo Struct
    (for (_array_element _array_index) _output_get_2
      (Utilities|Array|SetArrayElem (Variables|ExtractedTileData|GetTilePos) _array_index (Math|Conversions|ToVector(Float) (.position _array_element)))
      ;;[0.15 0.15 0.15 0.5] Construct mesh soft object path from tile name
      (Utilities|Array|SetArrayElem (Variables|ExtractedTileData|GetTileShapeSOP) _array_index (Utilities|MakeSoftObjectPath (Utilities|String|Append "/Game/Assets/StaticMeshes/Tiles/" (Utilities|String|Append "Tile_" (Utilities|String|EnumtoString (.tileshape _array_element))) "." (Utilities|String|Append "Tile_" (Utilities|String|EnumtoString (.tileshape _array_element))))))
      ;;[0.15 0.15 0.15 0.5] Derive angle from number of 90 degree turns
      (Utilities|Array|SetArrayElem (Variables|ExtractedTileData|GetTileRot) _array_index (Math|Rotator|MakeRotator 0.0 0.0 (Math|Conversions|ToFloat(Integer) (* (.rotation _array_element) 90))))
      (Utilities|Array|SetArrayElem (Variables|ExtractedTileData|GetTileType) _array_index (.terraintype _array_element)))
    ;[0.15 0.15 0.15 0.5] Notify PCG of updated data
    (Class|PCGComponent|NotifyPropertiesChangedfromBlueprint (Variables|Default|GetPCG))
    (else
      ;[0.15 0.15 0.15 0.5] Level Failed to Load
      (Development|PrintString "Level Failed to Load"))))