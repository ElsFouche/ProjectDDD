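; Procedural room generator that builds a maze level as tile data from its construction script.
; A cellular automaton grows the maze in double-buffered nodes through Disconnected, Seed, Invite and Connected states, with BranchingFactor weighting random state changes.
; The node grid then expands into a three-layer Tiles array with a solid floor, carving cells and links from invite directions.
; TurningFactor is unused, BuildTacticalCortex is empty, and GenerateTestLevel is an uncalled noise-heightmap stub.
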(event EventBeginPlay)

(event Collision|EventActorBeginOverlap
  (params (OtherActor :type Actor%20Object%20Reference)))

(event EventTick
  (params (DeltaSeconds :type Float%20%28single-precision%29)))

(fn ConstructionScript
  (CallFunction|GenerateMazeLevel)
  (CallFunction|BuildTacticalCortex))

(fn GenerateTestLevel
  (bind _dimensions (Variables|Default|GetDimensions))
  (bind _heightmap (LocalVariables|GetHeightMap))
  ;[0.15 0.15 0.15 0.5] Initialize Height Map With Noise
  (for _index (range 0 (- (* (.x _dimensions) (.y _dimensions)) 1))
    (Utilities|Array|SetArrayElem _heightmap _index (Math|Random|RandomInteger (.z _dimensions)) true))
  (bind _shuffled (CallFunction|GenerateShuffledOrdering (Utilities|Array|Length _heightmap)))
  (for _array_element _shuffled
    (CallFunction|Get2dNeighbors (Variables|Default|GetDimensions) _array_element false false)))

(fn AddTile
  (params (New%20Tile :type F%20Tile%20Info%20Structure))
  (Utilities|Array|SetArrayElem (Variables|Default|GetTiles) (.index (Utilities|GetIndexfromPosition (.Position (Utilities|Struct|BreakF_TileInfo New%20Tile)) (Variables|Default|GetDimensions))) New%20Tile true))

(fn GenerateMazeLevel
  (params (MazeDimensions :type F%20Int%20Vector%202d%20Structure) (Branching%20Factor :type Float%20%28double-precision%29) (Turning%20Factor :type Float%20%28double-precision%29))
  (bind (_x _y) (Utilities|Struct|BreakF_IntVector2d MazeDimensions))
  (bind _returnvalue (Math|Float|Clamp(Float) Branching%20Factor))
  (bind _out (Utilities|-(2d) MazeDimensions (Utilities|Struct|MakeF_IntVector2d 1 1)))
  (bind _out_2 (Utilities|*(2d) MazeDimensions (Utilities|Struct|MakeF_IntVector2d 2 2)))
  (bind _f_mazenode (Utilities|Struct|MakeF_MazeNode "NewEnumerator0" "NewEnumerator0" "NewEnumerator0"))
  (bind _mazenodes (LocalVariables|GetMazeNodes))
  (bind _neighbors (LocalVariables|GetNeighbors))
  (bind _neighbors_2 (LocalVariables|GetNeighbors))
  (bind (_outitem _outindex) (Utilities|Array|Random _neighbors_2))
  (bind (_outitem_2 _outindex_2) (Utilities|Array|Random _neighbors))
  (bind _out_3 (Utilities|+(2d) _out_2 (Utilities|Struct|MakeF_IntVector2d 1 1)))
  (bind _returnvalue_2 (!= _outindex_2 -1))
  (bind _returnvalue_3 (!= _outindex -1))
  ;[0.15 0.15 0.15 0.5] initialize CA
  (for _index (range 0 (.x _out))
    (for _index_2 (range 0 (.y _out))
      (Utilities|Map|Add (LocalVariables|GetMazeNodes) (Utilities|Struct|MakeF_IntVector2d _index _index_2) (Utilities|Struct|MakeF_HistoricalMazeNode _f_mazenode _f_mazenode)) ; state 0 means
    ))
  ;[0.15 0.15 0.15 0.5] set one point as a seed value
  (Utilities|Struct|SetmembersinF_MazeNode (.old (.Value (Utilities|Map|Find (LocalVariables|GetMazeNodes) (Utilities|Struct|MakeF_IntVector2d (Math|Random|RandomInteger _x) (Math|Random|RandomInteger _y))))) "NewEnumerator1")
  ;[0.15 0.15 0.15 0.5] CA Looper
  (bind _output_get (LocalVariables|SetisLiveSeeds true))
  (bind _output_get_2 (LocalVariables|SetisComplete false))
  (while (and _output_get (not _output_get_2))
    ;[0.15 0.15 0.15 0.5 122] Maze Generation Cellular Automaton Loop
    ;;[0.15 0.15 0.15 0.5] iterate over all cells
    (bind _keys (Utilities|Map|Keys (LocalVariables|GetMazeNodes)))
    (for _array_element _keys
      (switch Utilities|FlowControl|Switch|SwitchonE_MazeNodeState (.State (Utilities|Struct|BreakF_MazeNode (.old (.Value (Utilities|Map|Find (LocalVariables|GetMazeNodes) _array_element)))))
        (:NewEnumerator0
          ;;[0.15 0.15 0.15 0.5 30] For Disconnected Cells
          ;;;[0.15 0.15 0.15 0.5] Get Inviting Neighbors
          (bind _enumvalue (|ForEachE_Direction)
            (:LoopBody
              (if (Math|Boolean|ANDBoolean (Utilities|Enum|Equal(Enum) (.state (.old (.Value (Utilities|Map|Find (LocalVariables|GetMazeNodes) (Utilities|+(2d) _array_element (Utilities|ToIntVector2d _enumvalue)))))) "NewEnumerator2") (Utilities|Enum|Equal(Enum) (.invitevector (.old (.Value (Utilities|Map|Find (LocalVariables|GetMazeNodes) (Utilities|+(2d) _array_element (Utilities|ToIntVector2d _enumvalue)))))) (Utilities|ReverseDirection _enumvalue)) (.ReturnValue (Utilities|Map|Find (LocalVariables|GetMazeNodes) (Utilities|+(2d) _array_element (Utilities|ToIntVector2d _enumvalue)))))
                (Utilities|Array|Add (LocalVariables|GetNeighbors) _enumvalue)))
            (:then
              ;;;[0.15 0.15 0.15 0.5] Pick a random inviting neighbor to connect to
              (Utilities|Struct|SetmembersinF_MazeNode (.new (.Value (Utilities|Map|Find (LocalVariables|GetMazeNodes) _array_element))) (select _returnvalue_3 "NewEnumerator1" (.State (Utilities|Struct|BreakF_MazeNode (.old (.Value (Utilities|Map|Find (LocalVariables|GetMazeNodes) _array_element)))))) (select _returnvalue_3 _outitem (.ConnectVector (Utilities|Struct|BreakF_MazeNode (.old (.Value (Utilities|Map|Find (LocalVariables|GetMazeNodes) _array_element)))))) (.InviteVector (Utilities|Struct|BreakF_MazeNode (.old (.Value (Utilities|Map|Find (LocalVariables|GetMazeNodes) _array_element))))))
              (Utilities|Array|Clear (LocalVariables|GetNeighbors)))))
        (:NewEnumerator1
          ;;[0.15 0.15 0.15 0.5 30] For Seed Cells
          ;;;[0.15 0.15 0.15 0.5] Get Disconnected Neighbors
          (bind _enumvalue_2 (|ForEachE_Direction)
            (:LoopBody
              (if (and (Utilities|Enum|Equal(Enum) (.state (.old (.Value (Utilities|Map|Find (LocalVariables|GetMazeNodes) (Utilities|+(2d) _array_element (Utilities|ToIntVector2d _enumvalue_2)))))) "NewEnumerator0") (.ReturnValue (Utilities|Map|Find (LocalVariables|GetMazeNodes) (Utilities|+(2d) _array_element (Utilities|ToIntVector2d _enumvalue_2)))))
                (Utilities|Array|Add (LocalVariables|GetNeighbors) _enumvalue_2)))
            (:then
              ;;;[0.15 0.15 0.15 0.5] Choose random disconnected neighbor node to invite
              (Utilities|Struct|SetmembersinF_MazeNode (.new (.Value (Utilities|Map|Find (LocalVariables|GetMazeNodes) _array_element))) (select _returnvalue_2 "NewEnumerator2" "NewEnumerator3") (.ConnectVector (Utilities|Struct|BreakF_MazeNode (.old (.Value (Utilities|Map|Find (LocalVariables|GetMazeNodes) _array_element))))) (select _returnvalue_2 _outitem_2 (.InviteVector (Utilities|Struct|BreakF_MazeNode (.old (.Value (Utilities|Map|Find (LocalVariables|GetMazeNodes) _array_element)))))))
              (Utilities|Array|Clear (LocalVariables|GetNeighbors)))))
        (:NewEnumerator2
          ;;[0.15 0.15 0.15 0.5 30] For Invite Cells
          (Utilities|Struct|SetmembersinF_MazeNode (.new (.Value (Utilities|Map|Find (LocalVariables|GetMazeNodes) _array_element))) (select (> _returnvalue (Math|Random|RandomFloatinRange 0.0 1.0)) "NewEnumerator3" "NewEnumerator1") (.ConnectVector (Utilities|Struct|BreakF_MazeNode (.old (.Value (Utilities|Map|Find (LocalVariables|GetMazeNodes) _array_element))))) (.InviteVector (Utilities|Struct|BreakF_MazeNode (.old (.Value (Utilities|Map|Find (LocalVariables|GetMazeNodes) _array_element))))))
          (Utilities|Array|Clear (LocalVariables|GetNeighbors)))
        (:NewEnumerator3
          ;;[0.15 0.15 0.15 0.5 30] For Connected Seeds
          (if (LocalVariables|GetisLiveSeeds)
            ;;;[0.15 0.15 0.15 0.5] Possibly Convert to Seed if no current seeds, based on branching factor
            (Utilities|Struct|SetmembersinF_MazeNode (.new (.Value (Utilities|Map|Find (LocalVariables|GetMazeNodes) _array_element))) (select (and (!= -1 (.OutIndex (Utilities|Array|Random (LocalVariables|GetNeighbors)))) (> _returnvalue (Math|Random|RandomFloatinRange 0.0 1.0))) "NewEnumerator1" (.State (Utilities|Struct|BreakF_MazeNode (.old (.Value (Utilities|Map|Find (LocalVariables|GetMazeNodes) _array_element)))))) (.ConnectVector (Utilities|Struct|BreakF_MazeNode (.old (.Value (Utilities|Map|Find (LocalVariables|GetMazeNodes) _array_element))))) (.InviteVector (Utilities|Struct|BreakF_MazeNode (.old (.Value (Utilities|Map|Find (LocalVariables|GetMazeNodes) _array_element))))) :!label _label)
            (Utilities|Array|Clear (LocalVariables|GetNeighbors))
            (else
              ;;;[0.15 0.15 0.15 0.5] Get Disconnected Neighbors
              (bind _enumvalue_3 (|ForEachE_Direction)
                (:LoopBody
                  (if (and (Utilities|Enum|Equal(Enum) (.state (.old (.Value (Utilities|Map|Find (LocalVariables|GetMazeNodes) (Utilities|+(2d) _array_element (Utilities|ToIntVector2d _enumvalue_3)))))) "NewEnumerator0") (.ReturnValue (Utilities|Map|Find (LocalVariables|GetMazeNodes) (Utilities|+(2d) _array_element (Utilities|ToIntVector2d _enumvalue_3)))))
                    (Utilities|Array|Add (LocalVariables|GetNeighbors) _enumvalue_3)))
                (:then
                  (goto _label))))))))
    ;;[0.15 0.15 0.15 0.5] Reset and Check if Done
    (LocalVariables|SetisLiveSeeds false)
    (LocalVariables|SetisComplete true)
    (bind _keys_2 (Utilities|Map|Keys _mazenodes))
    (for _array_element_2 _keys_2
      (|SetBy-RefVar (.old (.Value (Utilities|Map|Find _mazenodes _array_element_2))) (.new (.Value (Utilities|Map|Find _mazenodes _array_element_2))))
      (if (and (not (LocalVariables|GetisLiveSeeds)) (Utilities|Enum|Equal(Enum) (.State (Utilities|Struct|BreakF_MazeNode (.old (.Value (Utilities|Map|Find _mazenodes _array_element_2))))) "NewEnumerator1"))
        (LocalVariables|SetisLiveSeeds true))
      (if (and (LocalVariables|GetisComplete) (Utilities|Enum|Equal(Enum) (.State (Utilities|Struct|BreakF_MazeNode (.old (.Value (Utilities|Map|Find _mazenodes _array_element_2))))) "NewEnumerator0"))
        (LocalVariables|SetisComplete false))))
  ;[0.15 0.15 0.15 0.5 30] Build The Level
  (bind _output_get_3 (Variables|Default|SetDimensions (Utilities|Struct|MakeIntVector (.x _out_3) (.y _out_3) 3)))
  (for _index_3 (range 0 (.x (Utilities|+(3d) _output_get_3 (Utilities|Struct|MakeIntVector -1 -1 -1))))
    (for _index_4 (range 0 (.y (Utilities|+(3d) _output_get_3 (Utilities|Struct|MakeIntVector -1 -1 -1))))
      (for _index_5 (range 0 (.z (Utilities|+(3d) _output_get_3 (Utilities|Struct|MakeIntVector -1 -1 -1))))
        ;;[0.15 0.15 0.15 0.5] Set as Solid if on first Layer
        (if (== (.Z (Utilities|Struct|BreakIntVector (Utilities|Struct|MakeIntVector _index_3 _index_4 _index_5))) 0)
          (Utilities|Array|Add (Variables|Default|GetTiles) (Utilities|Struct|MakeF_TileInfo (Utilities|*(3d) (Utilities|Struct|MakeIntVector _index_3 _index_4 _index_5) (Utilities|Struct|MakeIntVector 100 100 100)) "NewEnumerator0" 0 "NewEnumerator1"))
          (else
            ;;[0.15 0.15 0.15 0.5] Set as Empty if it maps to a Maze Node
            (if (.isMazeNodeFound (Utilities|FindMazeNode (Utilities|Struct|MakeIntVector _index_3 _index_4 _index_5) (LocalVariables|GetMazeNodes)))
              (Utilities|Array|Add (Variables|Default|GetTiles) (Utilities|Struct|MakeF_TileInfo (Utilities|*(3d) (Utilities|Struct|MakeIntVector _index_3 _index_4 _index_5) (Utilities|Struct|MakeIntVector 100 100 100)) "NewEnumerator29" 0 "NewEnumerator0"))
              (else
                ;;[0.15 0.15 0.15 0.5] Set as Empty if any neighbors map to maze nodes that point to it, set as Solid otherwise.
                (bind _enumvalue_4 (|ForEachE_Direction)
                  (:LoopBody
                    (if (and (Utilities|Enum|Equal(Enum) (.invitevector (.Maze%20Node (Utilities|FindMazeNode (Utilities|+(3d) (Utilities|ToIntVector (Utilities|ToIntVector2d _enumvalue_4)) (Utilities|Struct|MakeIntVector _index_3 _index_4 _index_5)) (LocalVariables|GetMazeNodes)))) (Utilities|ReverseDirection _enumvalue_4)) (.isMazeNodeFound (Utilities|FindMazeNode (Utilities|+(3d) (Utilities|ToIntVector (Utilities|ToIntVector2d _enumvalue_4)) (Utilities|Struct|MakeIntVector _index_3 _index_4 _index_5)) (LocalVariables|GetMazeNodes))))
                      (Utilities|Array|Add (LocalVariables|GetNeighbors) _enumvalue_4)))
                  (:then
                    (Utilities|Array|Add (Variables|Default|GetTiles) (select (!= (.OutIndex (Utilities|Array|Random (LocalVariables|GetNeighbors))) 0) (Utilities|Struct|MakeF_TileInfo (Utilities|*(3d) (Utilities|Struct|MakeIntVector _index_3 _index_4 _index_5) (Utilities|Struct|MakeIntVector 100 100 100)) "NewEnumerator29" 0 "NewEnumerator0") (Utilities|Struct|MakeF_TileInfo (Utilities|*(3d) (Utilities|Struct|MakeIntVector _index_3 _index_4 _index_5) (Utilities|Struct|MakeIntVector 100 100 100)) "NewEnumerator0" 0 "NewEnumerator1")))))))))))))

(fn BuildTacticalCortex)