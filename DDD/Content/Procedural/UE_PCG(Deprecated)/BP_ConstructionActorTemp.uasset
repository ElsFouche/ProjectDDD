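; Temporary construction actor, in a deprecated PCG folder, that generates a maze room on BeginPlay.
; ACMazeGenerator builds the maze from MazeDimensions, which also size a box, and parses it into TacticalCortex and tile transform, mesh, texture and prop arrays.
; The PCG component is notified to consume those arrays.
; Batching, progress reporting and old-mesh cleanup are disconnected, the completion callback does nothing, and GenerateRoom is a stub beside the older GenerateLevelOLD.
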(event OnPCGGraphGeneratedExternal(PCG_Component)
  (params (PCGComponent :type PCG%20Component%20Object%20Reference))
  ;[0.15 0.15 0.15 0.5] Every 10 data entries: update PCG, break new meshes' link to PCG, and clear arrays.
  ;;[0.15 0.15 0.15 0.5] PCG generation complete, was it requested?
  (if (Variables|Batching|GetGenerationRequested)
    _))

(event EventBeginPlay
  (CallFunction|GenerateRoomStart self false (Variables|MazeInput|GetMazeDimensions)))

(event EventEndPlay
  (params (EndPlayReason :type EEndPlayReason%20Enum :default "Destroyed"))
  (Components|Activation|SetActive (Variables|Components|GetPCG_Component) false false))

(event EventGenerateRoomStart
  (params (RequestedBy :type Object%20Object%20Reference%20%28by%20ref%29) (RoomType :type Boolean) (RoomDimensions :type Int%20Vector%20Structure))
  (bind _ac_mazegenerator (Variables|Default|GetAC_MazeGenerator))
  ;[0.15 0.15 0.15 0.5] Clear arrays of parsed data and notify PCG of emptied arrays
  (Variables|Batching|SetGenerationRequested true)
  (CallFunction|ClearArrays)
  ;[0.15 0.15 0.15 0.5] Generate level. This section to be revised as more level types are created.
  (bind _output_get (Variables|MazeInput|SetMazeDimensions RoomDimensions))
  (bind _issuccessful (Default|GenerateMaze _ac_mazegenerator _output_get 0.0 0.0))
  (if _issuccessful
    (bind (_pcgdata _tacticalcortex) (Default|ParseLevelInfo _ac_mazegenerator))
    (Variables|TileData|SetTacticalCortex _tacticalcortex)
    (Variables|TileData|SetTilePos (.position _pcgdata))
    (Variables|TileData|SetTileRot (.rotation _pcgdata))
    (Variables|TileData|SetTileMesh (.tilemesh _pcgdata))
    (Variables|TileData|SetTopTexture (.toptexture _pcgdata))
    (Variables|TileData|SetNorthTexture (.northtexture _pcgdata))
    (Variables|TileData|SetEastTexture (.easttexture _pcgdata))
    (Variables|TileData|SetSouthTexture (.southtexture _pcgdata))
    (Variables|TileData|SetWestTexture (.westtexture _pcgdata))
    (Variables|TileData|SetProps (.props _pcgdata))
    (Class|PCGComponent|NotifyPropertiesChangedfromBlueprint (Variables|Components|GetPCG_Component))
    (else
      ;[0.15 0.15 0.15 0.5] Level Failed to Load
      (Development|PrintString "Level Failed to Load"))))

(fn ConstructionScript
  (bind _mazedimensions (Variables|MazeInput|GetMazeDimensions))
  (Components|Box|SetBoxExtent (Variables|Default|GetBox) (Math|Vector|MakeVector (Math|Conversions|ToFloat(Integer) (.x _mazedimensions)) (Math|Conversions|ToFloat(Integer) (.y _mazedimensions)) (Math|Conversions|ToFloat(Integer) (.z _mazedimensions))) true))

(fn GenerateLevelOLD
  (params (MazeDimensions :type Int%20Vector%20Structure) (BranchingFactor :type Float%20%28double-precision%29) (TurningFactor :type Float%20%28double-precision%29))
  (bind _ac_mazegenerator (Variables|Default|GetAC_MazeGenerator))
  (CallFunction|ClearArrays)
  (Class|PCGComponent|NotifyPropertiesChangedfromBlueprint (Variables|Components|GetPCG_Component))
  (bind _output_get (Variables|MazeInput|SetMazeDimensions MazeDimensions))
  ;[0.15 0.15 0.15 0.5] Generate level. This section to be revised as more level types are created.
  (bind _issuccessful (Default|GenerateMaze _ac_mazegenerator _output_get BranchingFactor TurningFactor))
  (if _issuccessful
    (bind (_pcgdata _tacticalcortex) (Default|ParseLevelInfo _ac_mazegenerator))
    (Variables|TileData|SetTacticalCortex _tacticalcortex)
    (for _index (range 0 (- (.tiles _pcgdata) 1))
      (Utilities|Array|Add (Variables|TileData|GetTilePos) (Utilities|Array|Get(acopy) (.position _pcgdata) _index))
      (Utilities|Array|Add (Variables|TileData|GetTileRot) (Utilities|Array|Get(acopy) (.rotation _pcgdata) _index))
      (Utilities|Array|Add (Variables|TileData|GetTileMesh) (Utilities|Array|Get(acopy) (.tilemesh _pcgdata) _index))
      (Utilities|Array|Add (Variables|TileData|GetTopTexture) (Utilities|Array|Get(acopy) (.toptexture _pcgdata) _index))
      (Utilities|Array|Add (Variables|TileData|GetNorthTexture) (Utilities|Array|Get(acopy) (.northtexture _pcgdata) _index))
      (Utilities|Array|Add (Variables|TileData|GetEastTexture) (Utilities|Array|Get(acopy) (.easttexture _pcgdata) _index))
      (Utilities|Array|Add (Variables|TileData|GetSouthTexture) (Utilities|Array|Get(acopy) (.southtexture _pcgdata) _index))
      (Utilities|Array|Add (Variables|TileData|GetWestTexture) (Utilities|Array|Get(acopy) (.westtexture _pcgdata) _index))
      (Utilities|Array|Add (Variables|TileData|GetProps) (Utilities|Array|Get(acopy) (.props _pcgdata) _index))
      ;[0.15 0.15 0.15 0.5] Every 10 data entries: update PCG, break new meshes' link to PCG, and clear arrays.
      (if (== (/ (Math|Integer|%(Integer) _index 10) 9) 1)
        ;;[0.15 0.15 0.15 0.5] Notify PCG of updated data
        (Class|PCGComponent|NotifyPropertiesChangedfromBlueprint (Variables|Components|GetPCG_Component))
        ;;[0.15 0.15 0.15 0.5] Detach meshes from PCG
        (Class|PCGComponent|ClearPCGLink (Variables|Components|GetPCG_Component) 0)))
    (else
      ;[0.15 0.15 0.15 0.5] Level Failed to Load
      (Development|PrintString "Level Failed to Load"))))

(fn ClearArrays
  (Utilities|Array|Clear (Variables|TileData|GetTilePos))
  (Utilities|Array|Clear (Variables|TileData|GetTileRot))
  (Utilities|Array|Clear (Variables|TileData|GetTileMesh))
  (Utilities|Array|Clear (Variables|TileData|GetTopTexture))
  (Utilities|Array|Clear (Variables|TileData|GetNorthTexture))
  (Utilities|Array|Clear (Variables|TileData|GetEastTexture))
  (Utilities|Array|Clear (Variables|TileData|GetSouthTexture))
  (Utilities|Array|Clear (Variables|TileData|GetWestTexture))
  (Utilities|Array|Clear (Variables|TileData|GetProps)))

(fn GenerateRoom
  (params (RoomType :type Boolean) (RoomDimensions :type Int%20Vector%20Structure))
  (return false 0.0))