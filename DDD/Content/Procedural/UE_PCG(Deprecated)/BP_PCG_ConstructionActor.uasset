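; Deprecated PCG construction actor that builds a maze level at BeginPlay and stores its TacticalCortex.
; ACMazeGenerator output is copied into per-tile transform, mesh, texture and prop arrays in batches, each pushed to PCG by a property-change notification.
; Each PCG completion callback clears the link and arrays, reports progress to the requester and loops to the next batch.
; EndPlay cleans up PCG to avoid a crash; comments flag ClearPCGLink as bugged.
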(event OnPCGGraphGeneratedExternal(PCG_Component)
  (params (PCGComponent :type PCG%20Component%20Object%20Reference))
  (bind _pcg_component (Variables|Components|GetPCG_Component))
  (bind _pcg_component_2 (Variables|Components|GetPCG_Component))
  (bind _batchsize (Variables|Batching|GetBatchSize))
  (bind _batchcount (Variables|Batching|GetBatchCount))
  (bind _returnvalue (* _batchcount _batchsize))
  ;[0.15 0.15 0.15 0.5] Batch process array information into sets of 10 prior to updating PCG with new information.
  ;;[0.15 0.15 0.15 0.5] Every 10 data entries: update PCG, break new meshes' link to PCG, and clear arrays.
  ;;;[0.15 0.15 0.15 0.5] PCG generation complete, was it requested?
  (if (Variables|Batching|GetGenerationRequested)
    ;;;[0.15 0.15 0.15 0.5] Wait for PCG to finalize
    (Utilities|FlowControl|DelayUntilNextTick)
    (Utilities|IsValid _pcg_component
      (:Is%20Valid
        (Class|PCGComponent|ClearPCGLink _pcg_component 0)
        (Utilities|FlowControl|DelayUntilNextTick)
        ;;;[0.15 0.15 0.15 0.5] If so, ready arrays for next batch
        (CallFunction|ClearArrays)
        ;;[0.15 0.15 0.15 0.5] Notify requester of progress and retrigger data batching
        (Class|BPIRoomConstruction|GenerateRoomProgress(Message) (stale EventGenerateRoomStart RequestedBy) false (Math|Float|SafeDivide (Math|Conversions|ToFloat(Integer) (stale _index)) (Math|Conversions|ToFloat(Integer) (.tiles (stale EventGenerateRoomStart _pcgdata)))))
        (if (<= (stale EventGenerateRoomStart _output_get_2) (/ (.tiles (stale EventGenerateRoomStart _pcgdata)) (Variables|Batching|GetBatchSize)))
          (for _index (range _returnvalue (+ _returnvalue _batchsize))
            (if (Utilities|Array|IsValidIndex (.position (stale EventGenerateRoomStart _pcgdata)) _index)
              (Utilities|Array|Add (Variables|TileData|GetTilePos) (Utilities|Array|Get(acopy) (.position (stale EventGenerateRoomStart _pcgdata)) _index)))
            (if (Utilities|Array|IsValidIndex (.rotation (stale EventGenerateRoomStart _pcgdata)) _index)
              (Utilities|Array|Add (Variables|TileData|GetTileRot) (Utilities|Array|Get(acopy) (.rotation (stale EventGenerateRoomStart _pcgdata)) _index)))
            (if (Utilities|Array|IsValidIndex (.tilemesh (stale EventGenerateRoomStart _pcgdata)) _index)
              (Utilities|Array|Add (Variables|TileData|GetTileMesh) (Utilities|Array|Get(acopy) (.tilemesh (stale EventGenerateRoomStart _pcgdata)) _index)))
            (if (Utilities|Array|IsValidIndex (.toptexture (stale EventGenerateRoomStart _pcgdata)) _index)
              (Utilities|Array|Add (Variables|TileData|GetTopTexture) (Utilities|Array|Get(acopy) (.toptexture (stale EventGenerateRoomStart _pcgdata)) _index)))
            (if (Utilities|Array|IsValidIndex (.northtexture (stale EventGenerateRoomStart _pcgdata)) _index)
              (Utilities|Array|Add (Variables|TileData|GetNorthTexture) (Utilities|Array|Get(acopy) (.northtexture (stale EventGenerateRoomStart _pcgdata)) _index)))
            (if (Utilities|Array|IsValidIndex (.easttexture (stale EventGenerateRoomStart _pcgdata)) _index)
              (Utilities|Array|Add (Variables|TileData|GetEastTexture) (Utilities|Array|Get(acopy) (.easttexture (stale EventGenerateRoomStart _pcgdata)) _index)))
            (if (Utilities|Array|IsValidIndex (.southtexture (stale EventGenerateRoomStart _pcgdata)) _index)
              (Utilities|Array|Add (Variables|TileData|GetSouthTexture) (Utilities|Array|Get(acopy) (.southtexture (stale EventGenerateRoomStart _pcgdata)) _index)))
            (if (Utilities|Array|IsValidIndex (.westtexture (stale EventGenerateRoomStart _pcgdata)) _index)
              (Utilities|Array|Add (Variables|TileData|GetWestTexture) (Utilities|Array|Get(acopy) (.westtexture (stale EventGenerateRoomStart _pcgdata)) _index)))
            (if (Utilities|Array|IsValidIndex (.props (stale EventGenerateRoomStart _pcgdata)) _index)
              (Utilities|Array|Add (Variables|TileData|GetProps) (Utilities|Array|Get(acopy) (.props (stale EventGenerateRoomStart _pcgdata)) _index)))
            ;;[0.15 0.15 0.15 0.5] Checks if the batch of data has finished loading into the arrays
            (bind _result (Math|Integer|IncrementInt (Variables|Batching|GetBatchPosition))
              (:%20%20
                (if (> _result (Variables|Batching|GetBatchSize))
                  (goto _label In2)))))
          (Utilities|DowhenBoth :!label _label
            (:Out
              (Variables|Batching|SetBatchPosition 0)
              (Math|Integer|IncrementInt (Variables|Batching|GetBatchCount)
                (:%20%20
                  ;;;[0.15 0.15 0.15 0.5] Notify PCG of updated data
                  (Utilities|IsValid _pcg_component_2
                    (:Is%20Valid
                      (Class|PCGComponent|NotifyPropertiesChangedfromBlueprint _pcg_component_2))
                    (:Is%20Not%20Valid
                      (CallFunction|Debug "PCG Component: " "Component Invalid")))))))
          (else
            ;;[0.15 0.15 0.15 0.5] Notify requester of completed generation.
            (Class|BPIRoomConstruction|GenerateRoomProgress(Message) (stale EventGenerateRoomStart RequestedBy) true 1e+02)
            (Variables|Batching|SetGenerationRequested false)))))))

(event EventBeginPlay
  (CallFunction|GenerateRoomStart self false (Variables|MazeInput|GetMazeDimensions)))

(event EventEndPlay
  (params (EndPlayReason :type EEndPlayReason%20Enum :default "Destroyed"))
  (bind _pcg_component (Variables|Components|GetPCG_Component))
  ;[0.15 0.15 0.15 0.5] Deactivate PCG on end play to prevent a crash
  (Utilities|IsValid _pcg_component
    (:Is%20Valid
      (Class|PCGComponent|Cleanup _pcg_component true true)
      (Components|Activation|Deactivate _pcg_component))))

(event EventGenerateRoomStart
  (params (RequestedBy :type Object%20Object%20Reference%20%28by%20ref%29) (RoomType :type Boolean) (RoomDimensions :type Int%20Vector%20Structure))
  (bind _ac_mazegenerator (Variables|Default|GetAC_MazeGenerator))
  (bind _pcg_component (Variables|Components|GetPCG_Component))
  (bind _pcg_component_2 (Variables|Components|GetPCG_Component))
  (bind _batchsize (Variables|Batching|GetBatchSize))
  ;[0.15 0.15 0.15 0.5] Clear arrays of parsed data and clean up PCG
  (Variables|Batching|SetGenerationRequested true)
  (CallFunction|ClearArrays)
  (Utilities|IsValid _pcg_component_2
    (:Is%20Valid
      (Class|PCGComponent|Cleanup _pcg_component_2 true true)
      ;[0.15 0.15 0.15 0.5] Generate level. This section to be revised as more level types are created.
      (bind _output_get (Variables|MazeInput|SetMazeDimensions RoomDimensions))
      (Utilities|IsValid _ac_mazegenerator
        (:Is%20Valid
          (bind _issuccessful (Default|GenerateMaze _ac_mazegenerator _output_get 0.0 0.0))
          (if _issuccessful
            (bind (_pcgdata _tacticalcortex) (Default|ParseLevelInfo _ac_mazegenerator))
            ;[0.15 0.15 0.15 0.5] Initialize tactical cortex for the generated data
            (Variables|TileData|SetTacticalCortex _tacticalcortex)
            ;[0.15 0.15 0.15 0.5] Batch process array information into sets of 10 prior to updating PCG with new information.
            ;;[0.15 0.15 0.15 0.5] Initialize batch processing variables
            (bind _output_get_2 (Variables|Batching|SetBatchCount 0))
            (if (<= _output_get_2 (/ (.tiles _pcgdata) (Variables|Batching|GetBatchSize)))
              (for _index (range (* (Variables|Batching|GetBatchCount) _batchsize) (+ (* (Variables|Batching|GetBatchCount) _batchsize) _batchsize))
                (if (Utilities|Array|IsValidIndex (.position _pcgdata) _index)
                  (Utilities|Array|Add (Variables|TileData|GetTilePos) (Utilities|Array|Get(acopy) (.position _pcgdata) _index)))
                (if (Utilities|Array|IsValidIndex (.rotation _pcgdata) _index)
                  (Utilities|Array|Add (Variables|TileData|GetTileRot) (Utilities|Array|Get(acopy) (.rotation _pcgdata) _index)))
                (if (Utilities|Array|IsValidIndex (.tilemesh _pcgdata) _index)
                  (Utilities|Array|Add (Variables|TileData|GetTileMesh) (Utilities|Array|Get(acopy) (.tilemesh _pcgdata) _index)))
                (if (Utilities|Array|IsValidIndex (.toptexture _pcgdata) _index)
                  (Utilities|Array|Add (Variables|TileData|GetTopTexture) (Utilities|Array|Get(acopy) (.toptexture _pcgdata) _index)))
                (if (Utilities|Array|IsValidIndex (.northtexture _pcgdata) _index)
                  (Utilities|Array|Add (Variables|TileData|GetNorthTexture) (Utilities|Array|Get(acopy) (.northtexture _pcgdata) _index)))
                (if (Utilities|Array|IsValidIndex (.easttexture _pcgdata) _index)
                  (Utilities|Array|Add (Variables|TileData|GetEastTexture) (Utilities|Array|Get(acopy) (.easttexture _pcgdata) _index)))
                (if (Utilities|Array|IsValidIndex (.southtexture _pcgdata) _index)
                  (Utilities|Array|Add (Variables|TileData|GetSouthTexture) (Utilities|Array|Get(acopy) (.southtexture _pcgdata) _index)))
                (if (Utilities|Array|IsValidIndex (.westtexture _pcgdata) _index)
                  (Utilities|Array|Add (Variables|TileData|GetWestTexture) (Utilities|Array|Get(acopy) (.westtexture _pcgdata) _index)))
                (if (Utilities|Array|IsValidIndex (.props _pcgdata) _index)
                  (Utilities|Array|Add (Variables|TileData|GetProps) (Utilities|Array|Get(acopy) (.props _pcgdata) _index)))
                ;;[0.15 0.15 0.15 0.5] Checks if the batch of data has finished loading into the arrays
                (bind _result (Math|Integer|IncrementInt (Variables|Batching|GetBatchPosition))
                  (:%20%20
                    (if (> _result (Variables|Batching|GetBatchSize))
                      (goto _label In2)))))
              (Utilities|DowhenBoth :!label _label
                (:Out
                  (Variables|Batching|SetBatchPosition 0)
                  (Math|Integer|IncrementInt (Variables|Batching|GetBatchCount)
                    (:%20%20
                      ;;[0.15 0.15 0.15 0.5] Every 10 data entries: update PCG, break new meshes' link to PCG, and clear arrays.
                      ;;;[0.15 0.15 0.15 0.5] Notify PCG of updated data
                      (Utilities|IsValid _pcg_component
                        (:Is%20Valid
                          (Class|PCGComponent|NotifyPropertiesChangedfromBlueprint _pcg_component))
                        (:Is%20Not%20Valid
                          (CallFunction|Debug "PCG Component: " "Component Invalid")))))))
              (else
                ;;[0.15 0.15 0.15 0.5] Notify requester of completed generation.
                (Class|BPIRoomConstruction|GenerateRoomProgress(Message) RequestedBy true 1e+02)
                (Variables|Batching|SetGenerationRequested false)))
            (else
              ;;[1 0.8202 0 0.5] Level Failed to Load
              (Development|PrintString "Level Failed to Load"))))
        (:Is%20Not%20Valid
          (CallFunction|Debug "AC Maze Generator:  " "Component Invalid"))))
    (:Is%20Not%20Valid
      (CallFunction|Debug "PCG Component:  " "Component Invalid"))))

(fn ConstructionScript
  (bind _mazedimensions (Variables|MazeInput|GetMazeDimensions))
  (Components|Box|SetBoxExtent (Variables|Default|GetBox) (Math|Vector|MakeVector (Math|Conversions|ToFloat(Integer) (.x _mazedimensions)) (Math|Conversions|ToFloat(Integer) (.y _mazedimensions)) (Math|Conversions|ToFloat(Integer) (.z _mazedimensions))) true))

(fn GenerateLevelOLD
  (params (MazeDimensions :type Int%20Vector%20Structure) (BranchingFactor :type Float%20%28double-precision%29) (TurningFactor :type Float%20%28double-precision%29))
  (bind _ac_mazegenerator (Variables|Default|GetAC_MazeGenerator))
  (CallFunction|ClearArrays)
  (Class|PCGComponent|NotifyPropertiesChangedfromBlueprint (Variables|Components|GetPCG_Component))
  (bind _output_get (Variables|MazeInput|SetMazeDimensions MazeDimensions))
  ;[0.15 0.15 0.15 0.5] Generate level. This section to be revised as more level types are created.
  (bind _issuccessful (Default|GenerateMaze _ac_mazegenerator _output_get BranchingFactor TurningFactor))
  (if _issuccessful
    (bind (_pcgdata _tacticalcortex) (Default|ParseLevelInfo _ac_mazegenerator))
    (Variables|TileData|SetTacticalCortex _tacticalcortex)
    (for _index (range 0 (- (.tiles _pcgdata) 1))
      (Utilities|Array|Add (Variables|TileData|GetTilePos) (Utilities|Array|Get(acopy) (.position _pcgdata) _index))
      (Utilities|Array|Add (Variables|TileData|GetTileRot) (Utilities|Array|Get(acopy) (.rotation _pcgdata) _index))
      (Utilities|Array|Add (Variables|TileData|GetTileMesh) (Utilities|Array|Get(acopy) (.tilemesh _pcgdata) _index))
      (Utilities|Array|Add (Variables|TileData|GetTopTexture) (Utilities|Array|Get(acopy) (.toptexture _pcgdata) _index))
      (Utilities|Array|Add (Variables|TileData|GetNorthTexture) (Utilities|Array|Get(acopy) (.northtexture _pcgdata) _index))
      (Utilities|Array|Add (Variables|TileData|GetEastTexture) (Utilities|Array|Get(acopy) (.easttexture _pcgdata) _index))
      (Utilities|Array|Add (Variables|TileData|GetSouthTexture) (Utilities|Array|Get(acopy) (.southtexture _pcgdata) _index))
      (Utilities|Array|Add (Variables|TileData|GetWestTexture) (Utilities|Array|Get(acopy) (.westtexture _pcgdata) _index))
      (Utilities|Array|Add (Variables|TileData|GetProps) (Utilities|Array|Get(acopy) (.props _pcgdata) _index))
      ;[0.15 0.15 0.15 0.5] Every 10 data entries: update PCG, break new meshes' link to PCG, and clear arrays.
      (if (== (/ (Math|Integer|%(Integer) _index 10) 9) 1)
        ;;[0.15 0.15 0.15 0.5] Notify PCG of updated data
        (Class|PCGComponent|NotifyPropertiesChangedfromBlueprint (Variables|Components|GetPCG_Component))
        ;;[0.15 0.15 0.15 0.5] Detach meshes from PCG
        (Class|PCGComponent|ClearPCGLink (Variables|Components|GetPCG_Component) 0)))
    (else
      ;[0.15 0.15 0.15 0.5] Level Failed to Load
      (Development|PrintString "Level Failed to Load"))))

(fn ClearArrays
  (Utilities|Array|Clear (Variables|TileData|GetTilePos))
  (Utilities|Array|Clear (Variables|TileData|GetTileRot))
  (Utilities|Array|Clear (Variables|TileData|GetTileMesh))
  (Utilities|Array|Clear (Variables|TileData|GetTopTexture))
  (Utilities|Array|Clear (Variables|TileData|GetNorthTexture))
  (Utilities|Array|Clear (Variables|TileData|GetEastTexture))
  (Utilities|Array|Clear (Variables|TileData|GetSouthTexture))
  (Utilities|Array|Clear (Variables|TileData|GetWestTexture))
  (Utilities|Array|Clear (Variables|TileData|GetProps)))

(fn Debug
  (params (Message1 :type String) (Message2 :type String))
  (Development|PrintString (Utilities|String|Append Message1 Message2) true true "(R=0.619792,G=0.605024,B=0.000000,A=1.000000)" 5.0))

(fn GenerateMaze
  (return))

(fn GenerateRoom
  (params (RoomType :type Boolean) (RoomDimensions :type Int%20Vector%20Structure))
  (return false 0.0))