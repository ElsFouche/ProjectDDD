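; Procedural construction actor that builds a room from level data produced by an obstacle course generator component, starting itself on BeginPlay.
; Returned tile data is stored and its tactical cortex is passed to the game state.
; Tiles are processed in batches a tick apart, creating one HISM per unique mesh in a map and adding instances, with progress reported to the requester.
; Texture and prop arrays are batched but not yet applied.
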(event Custom|BatchProcessData
  (params (CurrentBatch :type Integer))
  (bind _batchsize (Variables|Batching|GetBatchSize))
  (bind _hism_map (Variables|Components|GetHISM_Map))
  ;[0.15 0.15 0.15 0.5] Batch Processing Loop
  (Utilities|FlowControl|Sequence
    (:then_0
      (bind _subarray (Utilities|BatchProcessArray CurrentBatch _batchsize (Variables|TileData|GetTilePos))
        (:__
          _)))
    (:then_1
      (bind _subarray_2 (Utilities|BatchProcessArray CurrentBatch _batchsize (Variables|TileData|GetTileRot))
        (:__
          _)))
    (:then_2
      (bind _subarray_3 (Utilities|BatchProcessArray CurrentBatch _batchsize (Variables|TileData|GetTileMesh))
        (:__
          _)))
    (:then_3
      (bind _subarray_4 (Utilities|BatchProcessArray CurrentBatch _batchsize (Variables|TileData|GetTopTexture))
        (:__
          _)))
    (:then_4
      (bind _subarray_5 (Utilities|BatchProcessArray CurrentBatch _batchsize (Variables|TileData|GetNorthTexture))
        (:__
          _)))
    (:then_5
      (bind _subarray_6 (Utilities|BatchProcessArray CurrentBatch _batchsize (Variables|TileData|GetEastTexture))
        (:__
          _)))
    (:then_6
      (bind _subarray_7 (Utilities|BatchProcessArray CurrentBatch _batchsize (Variables|TileData|GetSouthTexture))
        (:__
          _)))
    (:then_7
      (bind _subarray_8 (Utilities|BatchProcessArray CurrentBatch _batchsize (Variables|TileData|GetWestTexture))
        (:__
          _)))
    (:then_8
      (bind _subarray_9 (Utilities|BatchProcessArray CurrentBatch _batchsize (Variables|TileData|GetProps))
        (:__
          _))))
  (Utilities|DowhenN 9 ; Pulses must match number of inputs for execution to continue.
    (:Done
      ;;[0.15 0.15 0.15 0.5] HISM Ops Loop
      (for _index (range 0 (Variables|Batching|GetBatchSize))
        ;;;[0.15 0.15 0.15 0.5] Add HISM slot per unique new mesh
        (if (Utilities|Array|IsValidIndex _subarray_3 _index)
          (if (Utilities|Map|Contains _hism_map (Utilities|Array|Get(acopy) _subarray_3 _index))
            _
            (else
              (bind _returnvalue (AddComponent|AddHierarchicalInstancedStaticMeshComponent false))
              (Utilities|Map|Add _hism_map (Utilities|Array|Get(acopy) _subarray_3 _index) _returnvalue)
              (if (== 0 (Utilities|ResolveSoftReference (Utilities|Array|Get(acopy) _subarray_3 _index)))
                (bind _returnvalue_2 (Utilities|LoadAssetBlocking (Utilities|Array|Get(acopy) _subarray_3 _index)))
                (bind _asstatic_mesh (Utilities|Casting|CastToStaticMesh _returnvalue_2)
                  (:then
                    (Components|StaticMesh|SetStaticMesh _returnvalue _asstatic_mesh))
                  (:CastFailed
                    _))
                (else
                  (Components|StaticMesh|SetStaticMesh _returnvalue (Utilities|ResolveSoftReference (Utilities|Array|Get(acopy) _subarray_3 _index))))))))
        ;;;[0.15 0.15 0.15 0.5] Populate HISM with instances
        (if (and (.ReturnValue (Utilities|Map|Find (Variables|Components|GetHISM_Map) (Utilities|Array|Get(acopy) _subarray_3 _index))) (Utilities|Array|IsValidIndex _subarray _index))
          (Batching|AddInsttoHISM (.Value (Utilities|Map|Find (Variables|Components|GetHISM_Map) (Utilities|Array|Get(acopy) _subarray_3 _index))) (Utilities|Array|Get(acopy) _subarray _index) (Math|Rotator|SelectRotator (Utilities|Array|Get(acopy) _subarray_2 _index) "0, 0, 0" (Utilities|Array|IsValidIndex _subarray_2 _index)) 0 0.0)
          ;;;[0.15 0.15 0.15 0.5] -Actually- wait for loop completion
          (Utilities|DowhenN (Utilities|Array|Length _subarray_3)
            (:Done
              ;;[0.15 0.15 0.15 0.5] Notify when batch finished
              (CallFunction|BatchComplete (Utilities|Array|MakeArray (Utilities|Array|Length _subarray) (Utilities|Array|Length _subarray_2) (Utilities|Array|Length _subarray_3) (Utilities|Array|Length _subarray_4) (Utilities|Array|Length _subarray_5) (Utilities|Array|Length _subarray_6) (Utilities|Array|Length _subarray_7) (Utilities|Array|Length _subarray_8) (Utilities|Array|Length _subarray_9))))))))))

(event Custom|BatchComplete
  (params (SubArrLengths :type Array%20of%20Integers))
  (bind _totaltiles (Variables|Batching|GetTotalTiles))
  (bind _batchsize (Variables|Batching|GetBatchSize))
  (bind _numbatches (Utilities|GetBatchCount _totaltiles _batchsize))
  ;[0 0.15 0.1405 0.5] Batch Complete
  (bind _result (Math|Integer|IncrementInt (Variables|Batching|GetBatchCount))
    (:%20%20
      ;;[0.03806 0.3177 0.2999 0.5] Notify requester of progress
      (Class|BPIRoomConstruction|GenerateRoomProgress(Message) (Variables|MazeInput|GetGenerationRequestedBy) false (Math|Float|SafeDivide (Math|Conversions|ToFloat(Integer) _result) (Math|Conversions|ToFloat(Integer) _numbatches)))
      (Utilities|FlowControl|DelayUntilNextTick)
      ;[0 0.15 0.1405 0.5] Initialize batch counter, run while there are batches left to process.
      (if (<= (stale EventLevelDataComplete _output_get_2) _numbatches)
        (CallFunction|BatchProcessData (stale EventLevelDataComplete _output_get_2))
        (else
          ;;[0.15 0.15 0.15 0.5] Notify requester of completed generation.
          (Class|BPIRoomConstruction|GenerateRoomProgress(Message) (Variables|MazeInput|GetGenerationRequestedBy) true 1e+02))))))

(event Custom|ClearAllData
  (bind _hism_map (Variables|Components|GetHISM_Map))
  ;[0.15 0.03121 0.03419 0.5] Hard reset all stored data in this actor. CAUTION: This should never be called while an area is currently being generated!
  (bind _keys (Utilities|Map|Keys _hism_map))
  (for _array_element _keys
    (if (.ReturnValue (Utilities|Map|Find _hism_map _array_element))
      (Components|InstancedStaticMesh|ClearInstances (.Value (Utilities|Map|Find _hism_map _array_element)))))
  (Utilities|Map|Clear _hism_map)
  (Batching|ClearArrays))

(event EventBeginPlay
  (bind _self self)
  (Class|AutomationBlueprintFunctionLibrary|AutomationWaitforLoading)
  (Default|GenerateRoomStart _self _self false (Variables|MazeInput|GetMazeDimensions)))

(event EventEndPlay
  (params (EndPlayReason :type EEndPlayReason%20Enum :default "Destroyed")))

(event EventTacticalCortexUpdated
  (params (CompleteTacticalCortex :type BP%20Tactical%20Cortex%20Object%20Reference%20%28by%20ref%29))
  (Variables|TileData|SetTacticalCortex CompleteTacticalCortex))

(event EventGenerateRoomStart
  (params (RequestedBy :type Object%20Object%20Reference%20%28by%20ref%29) (RoomType :type Boolean) (RoomDimensions :type Int%20Vector%20Structure))
  (bind _hism_map (Variables|Components|GetHISM_Map))
  (Variables|MazeInput|SetGenerationRequestedBy RequestedBy)
  (Variables|MazeInput|SetMazeDimensions RoomDimensions)
  ;[0.15 0.15 0.15 0.5] Clear meshes
  (bind _keys (Utilities|Map|Keys _hism_map))
  (for _array_element _keys
    (if (.ReturnValue (Utilities|Map|Find _hism_map _array_element))
      (Components|InstancedStaticMesh|ClearInstances (.Value (Utilities|Map|Find _hism_map _array_element)))))
  (Utilities|Map|Clear _hism_map)
  ;[0.15 0.15 0.15 0.5] Level Data Generation: To Be expanded as more level types are added.
  (bind _returnvalue (AddComponent|AddACObstacleCourseGenerator))
  (bind _output_get (Variables|Default|SetCurrentRoomGenerator _returnvalue))
  (Class|BPIRoomConstruction|GenerateRoomStart(Message) _output_get self false (Variables|MazeInput|GetMazeDimensions)))

(event EventLevelDataComplete
  (params (PCGData :type F%20PCG%20Data%20Structure) (TacticalCortex :type BP%20Tactical%20Cortex%20Object%20Reference))
  (bind (_tiles _position _rotation _tilemesh _toptexture _northtexture _easttexture _southtexture _westtexture _props) (Utilities|Struct|BreakF_PCGData PCGData))
  (Variables|Batching|SetTotalTiles _tiles)
  (Variables|TileData|SetTilePos _position)
  (Variables|TileData|SetTileRot _rotation)
  (Variables|TileData|SetTileMesh _tilemesh)
  (Variables|TileData|SetTopTexture _toptexture)
  (Variables|TileData|SetNorthTexture _northtexture)
  (Variables|TileData|SetEastTexture _easttexture)
  (Variables|TileData|SetSouthTexture _southtexture)
  (Variables|TileData|SetWestTexture _westtexture)
  (Variables|TileData|SetProps _props)
  (bind _output_get (Variables|TileData|SetTacticalCortex TacticalCortex))
  ;[0 0.15 0.1405 0.5] Notify game state of new tactical cortex.
  (Class|BPITacticalCortex|AddtoTacticalCortex(Message) (Game|GetGameState) _output_get)
  ;[0 0.15 0.1405 0.5] Initialize batch counter, run while there are batches left to process.
  (bind _output_get_2 (Variables|Batching|SetBatchCount 0))
  (if (<= _output_get_2 (Utilities|GetBatchCount (Variables|Batching|GetTotalTiles) (Variables|Batching|GetBatchSize)))
    (CallFunction|BatchProcessData _output_get_2)
    (else
      ;;[0.15 0.15 0.15 0.5] Notify requester of completed generation.
      (Class|BPIRoomConstruction|GenerateRoomProgress(Message) (Variables|MazeInput|GetGenerationRequestedBy) true 1e+02))))

(fn ConstructionScript)

(fn ClearArrays
  (Utilities|Array|Clear (Variables|TileData|GetTilePos))
  (Utilities|Array|Clear (Variables|TileData|GetTileRot))
  (Utilities|Array|Clear (Variables|TileData|GetTileMesh))
  (Utilities|Array|Clear (Variables|TileData|GetTopTexture))
  (Utilities|Array|Clear (Variables|TileData|GetNorthTexture))
  (Utilities|Array|Clear (Variables|TileData|GetEastTexture))
  (Utilities|Array|Clear (Variables|TileData|GetSouthTexture))
  (Utilities|Array|Clear (Variables|TileData|GetWestTexture))
  (Utilities|Array|Clear (Variables|TileData|GetProps))
  (return))

(fn Debug
  (params (Message1 :type String) (Message2 :type String))
  (Development|PrintString (Utilities|String|Append Message1 Message2) true true "(R=0.619792,G=0.605024,B=0.000000,A=1.000000)" 5.0))

(fn AddInsttoHISM
  (params (InHISM_Ref :type Hierarchical%20Instanced%20Static%20Mesh%20Component%20Object%20Reference%20%28by%20ref%29) (NewSM_Pos :type Vector) (NewSM_Rot :type Rotator) (CustomDataIndex :type Integer) (CustomDataValue :type Float%20%28double-precision%29))
  (bind _returnvalue (Components|InstancedStaticMesh|AddInstance InHISM_Ref (Math|Transform|MakeTransform NewSM_Pos NewSM_Rot) false))
  ;[0.7969 0.7638 0.00935 0.5] Uncertain if this is working properly at the moment
  (bind _returnvalue_2 (Components|InstancedStaticMesh|SetCustomDataValue InHISM_Ref _returnvalue CustomDataIndex CustomDataValue false))
  (return _returnvalue_2))

(fn GenerateRoom
  (params (RoomType :type Boolean) (RoomDimensions :type Int%20Vector%20Structure))
  (return false 0.0))

(fn GetTacticalCortex
  (return 0))