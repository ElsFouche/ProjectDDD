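; Template component for procedural room generators that builds tile-based level info and converts it for PCG.
; AddTile stores tiles by grid position, grows the level dimensions and spreads up to five textures across the tile faces.
; ParseLevelInfo flattens the tile map into parallel PCG arrays, resolving meshes through DT_TileShapeInfo with a fallback row, and returns them with a newly constructed, unpopulated BP_TacticalCortex.
; GenerateMaze is a stub that always reports failure.
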(event EventBeginPlay)

(event EventTick
  (params (DeltaSeconds :type Float%20%28single-precision%29)))

(fn AddTile
  (params (Position :type Int%20Vector%20Structure) (TerrainType :type E_TerrainTypes%20Enum :default "NewEnumerator0") (Rotation :type E_Direction%20Enum :default "NewEnumerator0") (TileShape :type E_TileShapes%20Enum :default "NewEnumerator29") (Textures :type Array%20of%20E_TextureTypes%20Enums :default "NewEnumerator0"))
  (bind (_x _y _z) (Utilities|Struct|BreakIntVector Position))
  (bind _returnvalue (Utilities|Array|Length Textures))
  (bind _output (Utilities|Array|Get(acopy) Textures))
  (bind _output_2 (Utilities|Array|Get(acopy) Textures 1))
  (bind _output_3 (Utilities|Array|Get(acopy) Textures 3))
  (bind _output_4 (Utilities|Array|Get(acopy) Textures 2))
  (LocalVariables|SetNewDimensions (Utilities|Struct|MakeIntVector (Utilities|Greatest _x (.X (Utilities|Struct|BreakIntVector (.dimensions (Variables|Default|GetLevelInfo))))) (Utilities|Greatest _y (.Y (Utilities|Struct|BreakIntVector (.dimensions (Variables|Default|GetLevelInfo))))) (Utilities|Greatest _z (.Z (Utilities|Struct|BreakIntVector (.dimensions (Variables|Default|GetLevelInfo)))))))
  (bind _output_get (LocalVariables|SetOldTileInfo (.tileinfo (Variables|Default|GetLevelInfo))))
  (bind _output_get_2 (LocalVariables|SetNewTileInfo _output_get))
  (Utilities|Map|Add _output_get_2 Position (Utilities|Select :Index (Math|Integer|SelectInt 5 _returnvalue (>= _returnvalue 5)) :Option%200 (Utilities|Struct|MakeF_TileInfo TerrainType Rotation TileShape) :Option%201 (Utilities|Struct|MakeF_TileInfo TerrainType Rotation TileShape _output _output _output _output _output) :Option%202 (Utilities|Struct|MakeF_TileInfo TerrainType Rotation TileShape _output _output_2 _output_2 _output_2 _output_2) :Option%203 (Utilities|Struct|MakeF_TileInfo TerrainType Rotation TileShape _output _output_2 _output_4 _output_2 _output_4) :Option%204 (Utilities|Struct|MakeF_TileInfo TerrainType Rotation TileShape _output _output_2 _output_3 _output_4 _output_3) :Option%205 (Utilities|Struct|MakeF_TileInfo TerrainType Rotation TileShape _output _output_2 _output_4 _output_3 (Utilities|Array|Get(acopy) Textures 4))))
  (Variables|Default|SetLevelInfo (Utilities|Struct|MakeF_LevelInfo (LocalVariables|GetNewTileInfo) (LocalVariables|GetNewDimensions) (.props (Variables|Default|GetLevelInfo)) (.entrances (Variables|Default|GetLevelInfo))))
  (return))

(fn ClearLevelInfo
  (Variables|Default|SetLevelInfo (Utilities|Struct|MakeF_LevelInfo (Utilities|Map|MakeMap) (Utilities|Struct|MakeIntVector 0 0 0) (Utilities|Array|MakeArray) (Utilities|Array|MakeArray)))
  (return))

(fn ParseLevelInfo
  (params (LevelInfo :type F%20Level%20Info%20Structure))
  (bind (_tileinfo _dimensions _props) (Utilities|Struct|BreakF_LevelInfo LevelInfo))
  (bind _pcgtilemeshes (LocalVariables|GetPCGTileMeshes))
  (bind _pcgprops (LocalVariables|GetPCGProps))
  (bind _returnvalue (Game|ConstructObjectfromClass "/Game/Units/AI/BP_TacticalCortex.BP_TacticalCortex_C"))
  (LocalVariables|SetCortexOut _returnvalue)
  (bind _keys (Utilities|Map|Keys _tileinfo))
  (Utilities|Array|Clear _pcgprops)
  (Utilities|Array|AppendArray _pcgprops _props)
  (Utilities|Array|Resize (LocalVariables|GetPCGPositions) (Utilities|Array|Length _keys))
  (Utilities|Array|Resize (LocalVariables|GetPCGRotations) (Utilities|Array|Length _keys))
  (Utilities|Array|Resize (LocalVariables|GetPCGTileMeshes) (Utilities|Array|Length _keys))
  (Utilities|Array|Resize (LocalVariables|GetPCGTopTextures) (Utilities|Array|Length _keys))
  (Utilities|Array|Resize (LocalVariables|GetPCGNorthTextures) (Utilities|Array|Length _keys))
  (Utilities|Array|Resize (LocalVariables|GetPCGEastTextures) (Utilities|Array|Length _keys))
  (Utilities|Array|Resize (LocalVariables|GetPCGSouthTextures) (Utilities|Array|Length _keys))
  (Utilities|Array|Resize (LocalVariables|GetPCGWestTextures) (Utilities|Array|Length _keys))
  (for (_array_element _array_index) _keys
    (Utilities|Array|SetArrayElem (LocalVariables|GetPCGPositions) _array_index (* (Math|Conversions|ToVector(Float) _array_element) "100.000000,100.000000,100.000000"))
    (Utilities|Array|SetArrayElem (LocalVariables|GetPCGRotations) _array_index (Math|Rotator|MakeRotator 0.0 0.0 (Math|Conversions|ToFloat(Integer) (* (Math|Conversions|ToInteger(Byte) (.rotation (.Value (Utilities|Map|Find _tileinfo _array_element)))) 90))))
    (bind _returnvalue_2 (Utilities|GetDataTableRow "/Game/Procedural/Data/DT_TileShapeInfo.DT_TileShapeInfo" (Utilities|String|StringToName (Utilities|String|EnumtoString (.tileshape (.Value (Utilities|Map|Find _tileinfo _array_element))))))
      (:then
        (Utilities|Array|SetArrayElem _pcgtilemeshes _array_index (.tilemeshsop _returnvalue_2)))
      (:RowNotFound
        (bind _returnvalue_3 (Utilities|GetDataTableRow "/Game/Procedural/Data/DT_TileShapeInfo.DT_TileShapeInfo" "----")
          (:then
            (Utilities|Array|SetArrayElem _pcgtilemeshes _array_index (.tilemeshsop _returnvalue_3))))))
    (Utilities|Array|SetArrayElem (LocalVariables|GetPCGTopTextures) _array_index (.toptexture (.Value (Utilities|Map|Find _tileinfo _array_element))))
    (Utilities|Array|SetArrayElem (LocalVariables|GetPCGNorthTextures) _array_index (.northtexture (.Value (Utilities|Map|Find _tileinfo _array_element))))
    (Utilities|Array|SetArrayElem (LocalVariables|GetPCGEastTextures) _array_index (.easttexture (.Value (Utilities|Map|Find _tileinfo _array_element))))
    (Utilities|Array|SetArrayElem (LocalVariables|GetPCGSouthTextures) _array_index (.southtexture (.Value (Utilities|Map|Find _tileinfo _array_element))))
    (Utilities|Array|SetArrayElem (LocalVariables|GetPCGWestTextures) _array_index (.westtexture (.Value (Utilities|Map|Find _tileinfo _array_element)))))
  (LocalVariables|SetPCGOut (Utilities|Struct|MakeF_PCGData (Utilities|Array|Length _keys) (LocalVariables|GetPCGPositions) (LocalVariables|GetPCGRotations) (LocalVariables|GetPCGTileMeshes) (LocalVariables|GetPCGTopTextures) (LocalVariables|GetPCGNorthTextures) (LocalVariables|GetPCGEastTextures) (LocalVariables|GetPCGSouthTextures) (LocalVariables|GetPCGWestTextures) (LocalVariables|GetPCGProps)))
  (return (LocalVariables|GetPCGOut) (LocalVariables|GetCortexOut)))

(fn GenerateMaze
  (params (Dimensions :type Int%20Vector%20Structure) (BranchingFactor :type Float%20%28double-precision%29) (TurningFactor :type Float%20%28double-precision%29))
  (return 0 false))