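; Base grid-tactics unit: a camera-billboarded flipbook sprite with RPG stats, damage/healing and a downed state.
; FindPath or supplied points feed a move loop that walks tile edge to center; jump and fall moves are unfinished, and BeginPlay starts a temporary test loop.
; Animation states set four directional Knight flipbooks, picked by facing minus camera quadrant, preserving playback position.
; Data tables drive class stats and level-up growth.
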(event Custom|MoveToLocation
  (params (Destination :type Int%20Vector%20Structure))
  (bind _rootcomponent (Variables|Transformation|GetRootComponent))
  (bind _ac_gridnavigation (Variables|Default|GetAC_GridNavigation))
  ;[0.1003 0.533 0.6875 0.5] Move Events
  ;;[0.2581 0.6667 0.8125 0.5] Retrieve path to desired location.
  (bind _snappedpoint (Default|PointSnaptoGrid _ac_gridnavigation (Transformation|GetActorLocation)))
  (bind _outpathpoints (Default|FindPath _ac_gridnavigation _snappedpoint Destination (Utilities|Struct|BreakF_UnitStats (Variables|Stats|GetCurrStats))))
  (Variables|Movement|SetMovePath _outpathpoints)
  ;[0.1003 0.533 0.6875 0.5] For each point in the path attempt to move to the correct location if there are sufficient moves remaining.
  ;;[0.2581 0.6667 0.8125 0.5] Only perform movements from one trigger at a time.
  (bind _counter (Utilities|FlowControl|DoN 1)
    (:Exit
      (if (>= _counter 1) ; TODO: Notify caller of failed movement
        (Variables|Movement|SetMainMoveLoopIndex 0)
        ;;[0.2581 0.6667 0.8125 0.5] Main movement loop
        (bind (_arrayelement _arrayindex) (Utilities|ForEachLoopReal (Variables|Movement|GetMovePath))
          (:LoopBody
            (bind _output_get (Variables|Movement|SetPathPoint _arrayelement))
            (Variables|Movement|SetMainMoveLoopIndex _arrayindex)
            ;;[0.2581 0.6667 0.8125 0.5] Only perform a movement if the unit has sufficient movement remaining.
            (if (<= (Utilities|Struct|BreakF_MoveData _output_get) (Variables|Stats|GetMovementRemaining)) ; TODO: Notify caller of failed movement
              _
              (else
                (CallFunction|ResetMovement)))
            (switch Utilities|FlowControl|Switch|SwitchonE_MoveTypes (Utilities|Struct|BreakF_MoveData (Variables|Movement|GetPathPoint))
              (:NewEnumerator0
                ;;[0.2581 0.6667 0.8125 0.5] Walking
                ;;;[0.469 0.822 0.9479 0.5] Move to the edge of the current tile
                (bind _output_get_2 (Variables|Movement|SetUnitFacing (.MoveDirection (Utilities|Struct|BreakF_MoveData (Variables|Movement|GetPathPoint)))))
                (bind _nearedgeposition (Movement|CalculatePositionNearEdge (Transformation|GetActorLocation) _output_get_2 (.StartEdgeHeight (Utilities|Struct|BreakF_MoveData (Variables|Movement|GetPathPoint))) (Variables|/Game/Blueprints/ActorComponents/AC_GridNavigation.AC_GridNavigation_C|GetGridSize (Variables|Default|GetAC_GridNavigation)) 1.0))
                (CallFunction|AnimUpdate "NewEnumerator1")
                (Components|MoveComponentTo _rootcomponent _nearedgeposition "0, 0, 0" false false (* (Utilities|Struct|BreakF_MoveData (Variables|Movement|GetPathPoint)) 0.2) false)
                ;;;[0.469 0.822 0.9479 0.5] Move to the center of the destination tile and iterate to the next cycle of the loop.
                (Components|MoveComponentTo _rootcomponent (Math|Conversions|ToVector(Float) (Utilities|Struct|BreakF_MoveData (Variables|Movement|GetPathPoint))) "0, 0, 0" false false (* (Utilities|Struct|BreakF_MoveData (Variables|Movement|GetPathPoint)) 0.2) false)
                (CallFunction|ContinueMoving))
              (:NewEnumerator1
                ;;[0.2581 0.6667 0.8125 0.5] Calculate the current tile's almost-edge position.
                (CallFunction|AnimUpdate "NewEnumerator2" :!label _label)
                (bind _nearedgeposition_2 (Movement|CalculatePositionNearEdge (Transformation|GetActorLocation) (Utilities|Struct|BreakF_MoveData (Variables|Movement|GetPathPoint)) 0 (Variables|/Game/Blueprints/ActorComponents/AC_GridNavigation.AC_GridNavigation_C|GetGridSize (Variables|Default|GetAC_GridNavigation)) 0.6))
                (Variables|Movement|SetAlmostEdgeCurrTile _nearedgeposition_2)
                (if (Utilities|Array|IsValidIndex (Variables|Movement|GetMovePath) (+ (Variables|Movement|GetMainMoveLoopIndex) 1))
                  (if (Utilities|Enum|Equal(Enum) (Utilities|Struct|BreakF_MoveData (Variables|Movement|GetPathPoint)) (Utilities|ReverseDirection (Utilities|Struct|BreakF_MoveData (Utilities|Array|Get(acopy) (Variables|Movement|GetMovePath) (+ (Variables|Movement|GetMainMoveLoopIndex) 1)))))
                    (Variables|Movement|SetAlmostEdgeDestTile "0, 0, 0")
                    (else
                      (Variables|Movement|SetAlmostEdgeDestTile "0, 0, 0" :!label _label_2)))
                  (else
                    (goto _label_2))))
              (:NewEnumerator2
                (goto _label))
              (:NewEnumerator3
                (goto _label))
              (:NewEnumerator4
                (goto _label))))
          (:Completed
            (CallFunction|ResetMovement) ; Movement completed
            (CallFunction|TempMoveLoop)))))))

(event Custom|StartOfTurn
  ;[0.07682 0.09855 0.3073 0.5] Turn Start
)

(event Custom|MoveThroughPoints
  (params (Path :type Array%20of%20F%20Move%20Data%20Structures))
  (bind _rootcomponent (Variables|Transformation|GetRootComponent))
  ;[0.1003 0.533 0.6875 0.5] Move Events
  (Variables|Movement|SetMovePath Path)
  ;[0.1003 0.533 0.6875 0.5] For each point in the path attempt to move to the correct location if there are sufficient moves remaining.
  ;;[0.2581 0.6667 0.8125 0.5] Only perform movements from one trigger at a time.
  (bind _counter (Utilities|FlowControl|DoN 1)
    (:Exit
      (if (>= _counter 1) ; TODO: Notify caller of failed movement
        (Variables|Movement|SetMainMoveLoopIndex 0)
        ;;[0.2581 0.6667 0.8125 0.5] Main movement loop
        (bind (_arrayelement _arrayindex) (Utilities|ForEachLoopReal (Variables|Movement|GetMovePath))
          (:LoopBody
            (bind _output_get (Variables|Movement|SetPathPoint _arrayelement))
            (Variables|Movement|SetMainMoveLoopIndex _arrayindex)
            ;;[0.2581 0.6667 0.8125 0.5] Only perform a movement if the unit has sufficient movement remaining.
            (if (<= (Utilities|Struct|BreakF_MoveData _output_get) (Variables|Stats|GetMovementRemaining)) ; TODO: Notify caller of failed movement
              _
              (else
                (CallFunction|ResetMovement)))
            (switch Utilities|FlowControl|Switch|SwitchonE_MoveTypes (Utilities|Struct|BreakF_MoveData (Variables|Movement|GetPathPoint))
              (:NewEnumerator0
                ;;[0.2581 0.6667 0.8125 0.5] Walking
                ;;;[0.469 0.822 0.9479 0.5] Move to the edge of the current tile
                (bind _output_get_2 (Variables|Movement|SetUnitFacing (.MoveDirection (Utilities|Struct|BreakF_MoveData (Variables|Movement|GetPathPoint)))))
                (bind _nearedgeposition (Movement|CalculatePositionNearEdge (Transformation|GetActorLocation) _output_get_2 (.StartEdgeHeight (Utilities|Struct|BreakF_MoveData (Variables|Movement|GetPathPoint))) (Variables|/Game/Blueprints/ActorComponents/AC_GridNavigation.AC_GridNavigation_C|GetGridSize (Variables|Default|GetAC_GridNavigation)) 1.0))
                (CallFunction|AnimUpdate "NewEnumerator1")
                (Components|MoveComponentTo _rootcomponent _nearedgeposition "0, 0, 0" false false (* (Utilities|Struct|BreakF_MoveData (Variables|Movement|GetPathPoint)) 0.2) false)
                ;;;[0.469 0.822 0.9479 0.5] Move to the center of the destination tile and iterate to the next cycle of the loop.
                (Components|MoveComponentTo _rootcomponent (Math|Conversions|ToVector(Float) (Utilities|Struct|BreakF_MoveData (Variables|Movement|GetPathPoint))) "0, 0, 0" false false (* (Utilities|Struct|BreakF_MoveData (Variables|Movement|GetPathPoint)) 0.2) false)
                (CallFunction|ContinueMoving))
              (:NewEnumerator1
                ;;[0.2581 0.6667 0.8125 0.5] Calculate the current tile's almost-edge position.
                (CallFunction|AnimUpdate "NewEnumerator2" :!label _label)
                (bind _nearedgeposition_2 (Movement|CalculatePositionNearEdge (Transformation|GetActorLocation) (Utilities|Struct|BreakF_MoveData (Variables|Movement|GetPathPoint)) 0 (Variables|/Game/Blueprints/ActorComponents/AC_GridNavigation.AC_GridNavigation_C|GetGridSize (Variables|Default|GetAC_GridNavigation)) 0.6))
                (Variables|Movement|SetAlmostEdgeCurrTile _nearedgeposition_2)
                (if (Utilities|Array|IsValidIndex (Variables|Movement|GetMovePath) (+ (Variables|Movement|GetMainMoveLoopIndex) 1))
                  (if (Utilities|Enum|Equal(Enum) (Utilities|Struct|BreakF_MoveData (Variables|Movement|GetPathPoint)) (Utilities|ReverseDirection (Utilities|Struct|BreakF_MoveData (Utilities|Array|Get(acopy) (Variables|Movement|GetMovePath) (+ (Variables|Movement|GetMainMoveLoopIndex) 1)))))
                    (Variables|Movement|SetAlmostEdgeDestTile "0, 0, 0")
                    (else
                      (Variables|Movement|SetAlmostEdgeDestTile "0, 0, 0" :!label _label_2)))
                  (else
                    (goto _label_2))))
              (:NewEnumerator2
                (goto _label))
              (:NewEnumerator3
                (goto _label))
              (:NewEnumerator4
                (goto _label))))
          (:Completed
            (CallFunction|ResetMovement) ; Movement completed
            (CallFunction|TempMoveLoop)))))))

(event Custom|ResetMovement
  (bind _rootcomponent (Variables|Transformation|GetRootComponent))
  (bind _movepath (Variables|Movement|GetMovePath))
  ;[0.1003 0.533 0.6875 0.5] For each point in the path attempt to move to the correct location if there are sufficient moves remaining.
  ;;[0.2581 0.6667 0.8125 0.5] Reset movement loop when move failed or completed
  (CallFunction|AnimUpdate "NewEnumerator0")
  ;;[0.2581 0.6667 0.8125 0.5] Only perform movements from one trigger at a time.
  (Utilities|FlowControl|DoN 1) ; enters at Reset
)

(event Custom|ContinueMoving
  (bind _rootcomponent (Variables|Transformation|GetRootComponent))
  (bind _movepath (Variables|Movement|GetMovePath))
  ;[0.1003 0.533 0.6875 0.5] For each point in the path attempt to move to the correct location if there are sufficient moves remaining.
  ;;[0.2581 0.6667 0.8125 0.5] Main movement loop
  (Utilities|ForEachLoopReal (Variables|Movement|GetMovePath)) ; enters at Continue
)

(event Custom|AnimUpdate
  (params (NewAnimState :type E_MoveAnims%20Enum :default "NewEnumerator0"))
  ;[0.15 0.15 0.15 0.5] Animation State Machine
  (if (not (Utilities|Enum|Equal(Enum) NewAnimState (Variables|Animation|GetCurrentAnimationState)))
    (bind _output_get (Variables|Animation|SetCurrentAnimationState NewAnimState))
    (switch Utilities|FlowControl|Switch|SwitchonE_MoveAnims _output_get
      (:NewEnumerator0
        (Utilities|FlowControl|Sequence
          (:then_0
            (Variables|Animation|SetCurrAnimNW "/Game/_Local/2DAnimTesting/Idle/Knight_Idle_NW.Knight_Idle_NW"))
          (:then_1
            (Variables|Animation|SetCurrAnimNE "/Game/_Local/2DAnimTesting/Idle/Knight_Idle_NE.Knight_Idle_NE"))
          (:then_2
            (Variables|Animation|SetCurrAnimSW "/Game/_Local/2DAnimTesting/Idle/Knight_Idle_SW.Knight_Idle_SW"))
          (:then_3
            (Variables|Animation|SetCurrAnimSE "/Game/_Local/2DAnimTesting/Idle/Knight_Idle_SE.Knight_Idle_SE")))
        (Utilities|DowhenN 4
          (:Done
            (CallFunction|AnimSwitchbyViewDirection (Variables|Animation|GetCameraRotationIndex)))))
      (:NewEnumerator1
        (Utilities|FlowControl|Sequence
          (:then_0
            (Variables|Animation|SetCurrAnimNW "/Game/_Local/2DAnimTesting/Walk/Knight_Walk_NW.Knight_Walk_NW"))
          (:then_1
            (Variables|Animation|SetCurrAnimNE "/Game/_Local/2DAnimTesting/Walk/Knight_Walk_NE.Knight_Walk_NE"))
          (:then_2
            (Variables|Animation|SetCurrAnimSW "/Game/_Local/2DAnimTesting/Walk/Knight_Walk_SW.Knight_Walk_SW"))
          (:then_3
            (Variables|Animation|SetCurrAnimSE "/Game/_Local/2DAnimTesting/Walk/Knight_Walk_SE.Knight_Walk_SE")))
        (Utilities|DowhenN 4
          (:Done
            (CallFunction|AnimSwitchbyViewDirection (Variables|Animation|GetCameraRotationIndex)))))
      (:NewEnumerator2
        (Utilities|FlowControl|Sequence :!label _label
          (:then_0
            (Variables|Animation|SetCurrAnimNW "/Game/_Local/2DAnimTesting/Jump/Knight_Jump_NW.Knight_Jump_NW"))
          (:then_1
            (Variables|Animation|SetCurrAnimNE "/Game/_Local/2DAnimTesting/Jump/Knight_Jump_NE.Knight_Jump_NE"))
          (:then_2
            (Variables|Animation|SetCurrAnimSE "/Game/_Local/2DAnimTesting/Jump/Knight_Jump_SE.Knight_Jump_SE"))
          (:then_3
            (Variables|Animation|SetCurrAnimSW "/Game/_Local/2DAnimTesting/Jump/Knight_Jump_SW.Knight_Jump_SW")))
        (Utilities|DowhenN 4
          (:Done
            (CallFunction|AnimSwitchbyViewDirection (Variables|Animation|GetCameraRotationIndex)))))
      (:NewEnumerator3
        (goto _label))
      (:NewEnumerator4
        (goto _label)))
    (else
      (CallFunction|AnimSwitchbyViewDirection (Variables|Animation|GetCameraRotationIndex)))))

(event Custom|AnimSwitchByViewDirection
  (params (CameraRotationOffset :type Integer))
  (bind _sprite (Variables|Default|GetSprite))
  ;[0.15 0.15 0.15 0.5] Animation State Machine
  ;;[0.15 0.15 0.15 0.5] Switch animation based on camera angle
  (bind _output_get (Variables|Animation|SetPlaybackPosition (Components|Timeline|GetPlaybackPosition _sprite)))
  (bind _returnvalue (Sprite|SetFlipbook _sprite (Utilities|Select :Index (Utilities|Int% (- (Math|Conversions|ToInteger(Byte) (Variables|Movement|GetUnitFacing)) CameraRotationOffset) 4) :Option%200 (Variables|Animation|GetCurrAnimNE) :Option%201 (Variables|Animation|GetCurrAnimSE) :Option%202 (Variables|Animation|GetCurrAnimSW) :Option%203 (Variables|Animation|GetCurrAnimNW))))
  (if _returnvalue
    (Components|Timeline|SetPlaybackPosition _sprite _output_get false)))

(event Custom|StartOfRound
  ;[0.07682 0.09855 0.3073 0.5] Round Start
  (Variables|Stats|SetMovementRemaining (Utilities|Struct|BreakF_UnitStats (Variables|Stats|GetCurrStats))))

(event Custom|TempMoveLoop
  (CallFunction|MoveThroughPoints (Utilities|Array|MakeArray (Utilities|Struct|MakeF_MoveData (Utilities|Struct|MakeIntVector -150 -50 0) 1 "NewEnumerator0" "NewEnumerator1") (Utilities|Struct|MakeF_MoveData (Utilities|Struct|MakeIntVector -150 -150 0) 1 "NewEnumerator0" "NewEnumerator2") (Utilities|Struct|MakeF_MoveData (Utilities|Struct|MakeIntVector -50 -150 0) 1 "NewEnumerator0" "NewEnumerator3") (Utilities|Struct|MakeF_MoveData (Utilities|Struct|MakeIntVector 50 -150 0) 1 "NewEnumerator0" "NewEnumerator3") (Utilities|Struct|MakeF_MoveData (Utilities|Struct|MakeIntVector 50 -50 0) 1) (Utilities|Struct|MakeF_MoveData (Utilities|Struct|MakeIntVector -50 -50 0) 1 "NewEnumerator0" "NewEnumerator1"))))

(event EventBeginPlay
  ;[0.09459 0.401 0.06841] Begin Play
  (Variables|Stats|SetMovementRemaining (Utilities|Struct|BreakF_UnitStats (Variables|Stats|GetCurrStats)))
  (Variables|Components|SetActiveCamera (Game|GetPlayerCameraManager 0))
  (Pawn|Components|CharacterMovement|SetMovementMode (Variables|Character|GetCharacterMovement) "MOVE_Custom" 0)
  (Utilities|FlowControl|Delay 2.0)
  (Utilities|FlowControl|DoOnce false
    (:Completed
      (CallFunction|MoveThroughPoints (Utilities|Array|MakeArray (Utilities|Struct|MakeF_MoveData (Utilities|Struct|MakeIntVector -150 -50 0) 1 "NewEnumerator0" "NewEnumerator1") (Utilities|Struct|MakeF_MoveData (Utilities|Struct|MakeIntVector -150 -150 0) 1 "NewEnumerator0" "NewEnumerator2") (Utilities|Struct|MakeF_MoveData (Utilities|Struct|MakeIntVector -50 -150 0) 1 "NewEnumerator0" "NewEnumerator3") (Utilities|Struct|MakeF_MoveData (Utilities|Struct|MakeIntVector 50 -150 0) 1 "NewEnumerator0" "NewEnumerator3") (Utilities|Struct|MakeF_MoveData (Utilities|Struct|MakeIntVector 50 -50 0) 1) (Utilities|Struct|MakeF_MoveData (Utilities|Struct|MakeIntVector -50 -50 0) 1 "NewEnumerator0" "NewEnumerator1"))))))

(event EventTick
  (params (DeltaSeconds :type Float%20%28single-precision%29))
  (bind _activecamera (Variables|Components|GetActiveCamera))
  (bind _returnvalue (Camera|GetCameraRotation _activecamera))
  (bind _returnvalue_2 (Camera|GetCameraRotation _activecamera))
  (bind (_roll _pitch _yaw) (Math|Rotator|BreakRotator _returnvalue_2))
  (bind _returnvalue_3 (+ (.yaw _returnvalue) 3.6e+02))
  (bind _returnvalue_4 (Math|Float|%(Float) _returnvalue_3 3.6e+02))
  (bind _returnvalue_5 (Math|Float|Truncate _returnvalue_4))
  (bind _returnvalue_6 (/ _returnvalue_5 90))
  ;[0.112 0.1198 0.07757 0.5] Tick Events
  (Utilities|IsValid _activecamera
    (:Is%20Valid
      ;;[0.2157 0.2549 0.1922 0.502] Billboard to Camera
      (Transformation|SetWorldRotation (Variables|Default|GetSprite) (Math|Rotator|MakeRotator _pitch 0.0 (+ _yaw 9e+01)) false false)
      ;;[0.2157 0.2549 0.1922 0.502] Only update animations when the camera changes
      (if (!= (Variables|Animation|GetCameraRotationIndex) _returnvalue_6)
        (bind _output_get (Variables|Animation|SetCameraRotationIndex _returnvalue_6))
        (CallFunction|AnimSwitchbyViewDirection _output_get)))))

(event EventHarmUnit
  (params (HealthDmg :type Float%20%28double-precision%29) (FocusDmg :type Float%20%28double-precision%29) (MoraleDmg :type Integer))
  ;[0.08333 0.03003 0.07706 0.5] From BPI_UnitCombat
  (Combat|ReceiveDmgorHeals (* HealthDmg -1.0) (* FocusDmg -1.0) (* MoraleDmg -1)))

(event EventHealUnit
  (params (HealthHealed :type Float%20%28double-precision%29) (FocusHealed :type Float%20%28double-precision%29) (MoraleHealed :type Integer))
  ;[0.08333 0.03003 0.07706 0.5] From BPI_UnitCombat
  (Combat|ReceiveDmgorHeals HealthHealed FocusHealed MoraleHealed))

(fn ConstructionScript)

(fn NewUnitOfType
  (params (NewUnitType :type E_UnitType%20Enum :default "NewEnumerator0"))
  (bind _output_get (Variables|Stats|SetUnitType NewUnitType))
  ;[0.15 0.15 0.15 0.5] Is unit a non-generic unit?
  (bind _returnvalue (Utilities|GetDataTableRow "/Game/Units/Data/DT_RawUnitStats.DT_RawUnitStats" (Utilities|String|StringToName (Utilities|String|EnumtoString _output_get)))
    (:then
      (Variables|Stats|SetBaseStats _returnvalue))
    (:RowNotFound
      ;[0.15 0.15 0.15 0.5] Is unit a generic unit?
      (bind _returnvalue_2 (Utilities|GetDataTableRow "/Game/Units/Data/DT_RawUnitStats.DT_RawUnitStats" "Generic")
        (:then
          (Variables|Stats|SetBaseStats _returnvalue_2)))))
  ;[0.15 0.15 0.15 0.5] Grant unit their first level in their class.
  (Progression|LevelUp true))

(fn NewUnitRandom
  (params (RandTypeMin :type E_UnitType%20Enum :default "NewEnumerator0") (RandTypeMax :type E_UnitType%20Enum :default "NewEnumerator0"))
  (bind _returnvalue (Math|Conversions|ToInteger(Byte) RandTypeMin))
  (bind _returnvalue_2 (Math|Conversions|ToInteger(Byte) RandTypeMax))
  ;[0.15 0.15 0.15 0.5] A new unit has no unit type e.g. class. Randomly assign it a class. The maximum value of the random function will be limited to the number of specific beginner jobs in later versions.
  (bind _output_get (Variables|Stats|SetUnitType (Utilities|Enum|ByteToEnumE_UnitType (Math|Conversions|ToByte(Integer) (Math|Integer|SelectInt (- (Math|Random|RandomIntegerinRange 0 (|GetNumEnumEntries)) 1) (Math|Random|RandomIntegerinRange _returnvalue _returnvalue_2) (== _returnvalue _returnvalue_2))))))
  ;[0.15 0.15 0.15 0.5] Is unit a non-generic unit?
  (bind _returnvalue_3 (Utilities|GetDataTableRow "/Game/Units/Data/DT_RawUnitStats.DT_RawUnitStats" (Utilities|String|StringToName (Utilities|String|EnumtoString _output_get)))
    (:then
      (Variables|Stats|SetBaseStats _returnvalue_3))
    (:RowNotFound
      ;[0.15 0.15 0.15 0.5] Is unit a generic unit?
      (bind _returnvalue_4 (Utilities|GetDataTableRow "/Game/Units/Data/DT_RawUnitStats.DT_RawUnitStats" "Generic")
        (:then
          (Variables|Stats|SetBaseStats _returnvalue_4)))))
  ;[0.15 0.15 0.15 0.5] Grant unit their first level in their class.
  (Progression|LevelUp true))

(fn LevelUp
  (params (IsQuietLevelup? :type Boolean))
  ;[0.15 0.15 0.15 0.5] Increment Level
  (bind _result (Math|Integer|IncrementInt (Utilities|Struct|BreakF_UnitStats (Variables|Stats|GetBaseStats)))
    (:%20%20
      (Utilities|Struct|SetmembersinF_UnitStats (Variables|Stats|GetBaseStats) _result)
      ;[0.15 0.15 0.15 0.5] Improve the unit's base stats from level-and-rpg-class-based growth data and raw unit stats.
      (bind _modifiedstats (StatHelpers|CalculateGrowth (Variables|Stats|GetBaseStats) (Variables|Stats|GetUnitType)))
      ;[0.15 0.15 0.15 0.5] If this is the unit's first level gained, do not calculate how damaged it is.
      (if (== (.Level (Utilities|Struct|BreakF_UnitStats _modifiedstats)) 1)
        _
        (else
          ;[0.15 0.15 0.15 0.5] Store the unit's current health & focus state as a percentage
          (LocalVariables|SetPercentHealth (Math|Float|SafeDivide (.Health (Utilities|Struct|BreakF_UnitStats (Variables|Stats|GetCurrStats))) (.Health (Utilities|Struct|BreakF_UnitStats (Variables|Stats|GetModdedStats)))))
          (LocalVariables|SetPercentFocus (Math|Float|SafeDivide (.Focus (Utilities|Struct|BreakF_UnitStats (Variables|Stats|GetCurrStats))) (.Focus (Utilities|Struct|BreakF_UnitStats (Variables|Stats|GetModdedStats)))))))
      ;[0.15 0.15 0.15 0.5] Modify base stats based on the units rpg class
      (bind _output_get (Variables|Stats|SetBaseStats _modifiedstats))
      (bind _modifiedstats_2 (StatHelpers|CalculateClassStats _output_get (Variables|Stats|GetUnitType)))
      ;[0.15 0.15 0.15 0.5] Update the unit's stats based on rpg class
      (bind _output_get_2 (Variables|Stats|SetModdedStats _modifiedstats_2))
      (bind _output_get_3 (Variables|Stats|SetCurrStats _output_get_2))
      ;[0.15 0.15 0.15 0.5] Reset the unit's health and focus to its relative state prior to level up
      (Utilities|Struct|SetmembersinF_UnitStats _output_get_3 (* (.Health (Utilities|Struct|BreakF_UnitStats _output_get_3)) (LocalVariables|GetPercentHealth)) (* (.Focus (Utilities|Struct|BreakF_UnitStats _output_get_3)) (LocalVariables|GetPercentFocus))))))

(fn CalculateGrowth
  (params (StatsToModify :type F%20Unit%20Stats%20Structure) (UnitType :type E_UnitType%20Enum :default "NewEnumerator0"))
  (bind (_level _health _focus _morale _physatk _physdef _magatk _magdef _move _jump _speed) (Utilities|Struct|BreakF_UnitStats StatsToModify))
  ;[0.15 0.15 0.15 0.5] Based on level, get the growth value. Don't exceed the max number of levels that have explicit growth values.
  (bind _outrownames (DataTable|GetDataTableRowNames "/Game/Units/Data/DT_RawGrowthValues.DT_RawGrowthValues"))
  (bind _returnvalue (Utilities|GetDataTableRow "/Game/Units/Data/DT_RawGrowthValues.DT_RawGrowthValues" (Utilities|String|StringToName (Utilities|String|ToString(Integer) (Math|Integer|Min(Integer) (Utilities|Array|Length _outrownames) (Utilities|Struct|BreakF_UnitStats StatsToModify)))))
    (:then
      ;[0.15 0.15 0.15 0.5] Extra Stats = Raw Growth Value * Growth Multiplier
      (bind _returnvalue_2 (Utilities|GetDataTableRow "/Game/Units/Data/DT_GrowthMultipliers.DT_GrowthMultipliers" (Utilities|String|StringToName (Utilities|String|EnumtoString UnitType)))
        (:then
          (return (Utilities|Struct|MakeF_UnitStats _level (+ _health (* (.Health (Utilities|Struct|BreakF_UnitStats _returnvalue_2)) (.Health (Utilities|Struct|BreakF_UnitStats _returnvalue)))) (+ _focus (* (.Focus (Utilities|Struct|BreakF_UnitStats _returnvalue_2)) (.Focus (Utilities|Struct|BreakF_UnitStats _returnvalue)))) _morale (+ _physatk (* (.PhysAtk (Utilities|Struct|BreakF_UnitStats _returnvalue_2)) (.PhysAtk (Utilities|Struct|BreakF_UnitStats _returnvalue)))) (+ _physdef (* (.PhysDef (Utilities|Struct|BreakF_UnitStats _returnvalue_2)) (.PhysDef (Utilities|Struct|BreakF_UnitStats _returnvalue)))) (+ _magatk (* (.MagAtk (Utilities|Struct|BreakF_UnitStats _returnvalue_2)) (.MagAtk (Utilities|Struct|BreakF_UnitStats _returnvalue)))) (+ _magdef (* (.MagDef (Utilities|Struct|BreakF_UnitStats _returnvalue_2)) (.MagDef (Utilities|Struct|BreakF_UnitStats _returnvalue)))) _move _jump _speed)))))))

(fn ReceiveDmgorHeals
  (params (Health :type Float%20%28double-precision%29) (Focus :type Float%20%28double-precision%29) (Morale :type Integer))
  (bind _returnvalue (Math|Float|MakeLiteralFloat 1.0))
  (bind _currstats (Variables|Stats|GetCurrStats))
  (bind _moddedstats (Variables|Stats|GetModdedStats))
  (bind (_health _focus) (Utilities|Struct|BreakF_UnitStats _moddedstats))
  (bind (_health_2 _focus_2 _morale) (Utilities|Struct|BreakF_UnitStats _currstats))
  (bind _returnvalue_2 (+ _health_2 Health))
  (bind _returnvalue_3 (Math|Float|Clamp(Float) _returnvalue_2 0.0 _health))
  (bind _returnvalue_4 (Math|Float|Truncate _returnvalue_2))
  (bind _returnvalue_5 (== _returnvalue_4 0))
  (bind _returnvalue_6 (Math|Float|SelectFloat _returnvalue _returnvalue_3 _returnvalue_5))
  (Utilities|Struct|SetmembersinF_UnitStats _currstats _returnvalue_6 (Math|Float|Clamp(Float) (+ _focus_2 Focus) 0.0 _focus) (Math|Integer|Clamp(Integer) (+ _morale Morale) 0 100))
  (if (Math|Float|NearlyEqual(Float) _returnvalue_6 0.0 0.01)
    (Combat|ReceiveStatusEffect "NewEnumerator0")))

(fn ReceiveStatusEffect
  (params (EffectToAdd :type E_StatusEffects%20Enum :default "NewEnumerator0"))
  (switch Utilities|FlowControl|Switch|SwitchonE_StatusEffects EffectToAdd
    (:NewEnumerator0
      ;[0.15 0.15 0.15 0.5] UNIT DOWNED LOGIC
      (Utilities|Array|AddUnique (Variables|Stats|GetStatusEffects) "NewEnumerator0")
      (Utilities|Struct|SetmembersinF_UnitStats (Variables|Stats|GetCurrStats) 0.0))))

(fn CalculateClassStats
  (params (StatsToModify :type F%20Unit%20Stats%20Structure) (UnitClass :type E_UnitType%20Enum :default "NewEnumerator0"))
  (bind (_level _health _focus _morale _physatk _physdef _magatk _magdef _move _jump _speed) (Utilities|Struct|BreakF_UnitStats StatsToModify))
  (bind _returnvalue (Utilities|GetDataTableRow "/Game/Units/Data/DT_StatMultipliers.DT_StatMultipliers" (Utilities|String|StringToName (Utilities|String|EnumtoString UnitClass)))
    (:then
      (return (Utilities|Struct|MakeF_UnitStats _level (* _health (.Health (Utilities|Struct|BreakF_UnitStats _returnvalue))) (* _focus (.Focus (Utilities|Struct|BreakF_UnitStats _returnvalue))) _morale (* _physatk (.PhysAtk (Utilities|Struct|BreakF_UnitStats _returnvalue))) (* _physdef (.PhysDef (Utilities|Struct|BreakF_UnitStats _returnvalue))) (* _magatk (.MagAtk (Utilities|Struct|BreakF_UnitStats _returnvalue))) (* _magdef (.MagDef (Utilities|Struct|BreakF_UnitStats _returnvalue))) (+ _move (.Move (Utilities|Struct|BreakF_UnitStats _returnvalue))) (+ _jump (.Jump (Utilities|Struct|BreakF_UnitStats _returnvalue))) (+ _speed (.Speed (Utilities|Struct|BreakF_UnitStats _returnvalue))))))
    (:RowNotFound
      (Development|PrintString "Row not found in DT_StatMultipliers - ensure Unit Type exactly matches the row name!"))))

(fn ModifyBaseStat
  (params (InStat :type Integer) (InModifier :type Integer) (IsPercent? :type Boolean))
  (if IsPercent?
    (LocalVariables|SetTempModifiedStat (Math|Float|Round (* (Math|Conversions|ToFloat(Integer) InStat) (/ (Math|Conversions|ToFloat(Integer) InModifier) 100))))
    (else
      (LocalVariables|SetTempModifiedStat (+ InStat InModifier))))
  (return (LocalVariables|GetTempModifiedStat)))

(fn CalculatePositionNearEdge
  (params (TileCenter :type Vector) (TravelDirection :type E_Direction%20Enum :default "NewEnumerator0") (TileEdgeHeight :type Integer) (GridSize :type Int%20Vector%20Structure) (PercentTowardsEdge :type Float%20%28double-precision%29))
  (bind _vector (Utilities|ToUnitVector2d TravelDirection))
  (bind ____ (Utilities|Divide(IntVector) GridSize (Utilities|Struct|MakeIntVector 2 2 2)))
  (bind ___ (Utilities|ToIntVector _vector))
  (bind _____2 (Utilities|Multiply(IntVector) ___ ____))
  (bind _returnvalue (+ TileCenter _____2))
  (return (+ (* (- (Math|Vector|MakeVector (.x _returnvalue) (.y _returnvalue) (Math|Conversions|ToFloat(Integer) TileEdgeHeight)) TileCenter) PercentTowardsEdge) TileCenter)))