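; BP_TacticalNode is a tactical grid node in the unit AI, holding a position, player and edge heights, and a list of pickups.
; AddPickup and RemovePickup maintain the pickup list.
; PrintTacticalNodeData is a debug helper that builds an on-screen string from optional position and height sections.
; Its Contents option is an empty branch, so pickups are never printed.
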(fn AddPickup
  (params (Pickup :type Actor%20Object%20Reference))
  (bind _returnvalue (Utilities|Array|Add (Variables|TacticalContents|GetPickups) Pickup))
  (return _returnvalue))

(fn RemovePickup
  (params (Pickup :type Actor%20Object%20Reference))
  (bind _pickups (Variables|TacticalContents|GetPickups))
  (Utilities|Array|RemoveIndex _pickups (Utilities|Array|FindItem _pickups Pickup)))

(fn PrintTacticalNodeData
  (params (Position :type Boolean) (Heights :type Boolean) (Contents :type Boolean))
  (if Position
    (bind _output_get (LocalVariables|SetprintString (Utilities|String|Append (LocalVariables|GetprintString) "X: " (Utilities|String|ToString(Integer) (.x (Variables|TacticalContents|GetPosition))) " Y: " (Utilities|String|ToString(Integer) (.y (Variables|TacticalContents|GetPosition))) " Z: " (Utilities|String|ToString(Integer) (.z (Variables|TacticalContents|GetPosition)))))))
  (if Heights
    (bind _output_get_2 (LocalVariables|SetprintString (Utilities|String|Append _output_get " | Heights: P: " (Utilities|String|ToString(Integer) (Variables|TacticalElevationOffsets|GetPlayerHeight)) " N: " (Utilities|String|ToString(Integer) (Variables|TacticalElevationOffsets|GetNorthEdgeHeight)) " E: " (Utilities|String|ToString(Integer) (Variables|TacticalElevationOffsets|GetEastEdgeHeight)) " S: " (Utilities|String|ToString(Integer) (Variables|TacticalElevationOffsets|GetSouthEdgeHeight)) " W: " (Utilities|String|ToString(Integer) (Variables|TacticalElevationOffsets|GetWestEdgeHeight))))))
  (if Contents
    _
    (else
      _))
  (Development|PrintString 0 _output_get_2 true true "(R=0.000000,G=0.660000,B=1.000000,A=1.000000)" 6e+01)
  (return))