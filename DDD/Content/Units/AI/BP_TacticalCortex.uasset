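; Tactical grid brain that stores standable tile nodes and computes possible unit jump moves.
; AddNewNode builds nodes from the tile-shape data table, keyed by XY column and then height for multi-level lookup.
; FindMoves scans each direction for unoccupied nodes within jump cost, using edge heights and accumulating a hazard score for long falls.
; Longer jumps solve a parabolic arc and require clear half-height air points along it.
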(fn AddNode
  (params (NewNode :type F%20Tactical%20Node%20Structure))
  (bind _position (Utilities|Struct|BreakF_TacticalNode NewNode))
  (bind _navigablepoints (Variables|Default|GetNavigablePoints))
  (bind (_value _returnvalue) (Utilities|Map|Find _navigablepoints (Utilities|Struct|MakeF_IntVector2d (.x _position) (.y _position))))
  (if _returnvalue
    (Utilities|Map|Add (Utilities|Struct|BreakF_TacticalArray _value) (.z _position) NewNode)
    (else
      (Utilities|Map|Add _navigablepoints (Utilities|Struct|MakeF_IntVector2d (.x _position) (.y _position)) (Utilities|Struct|MakeF_TacticalArray (Utilities|Map|MakeMap (.z _position) NewNode))))))

(fn PrintNodes
  (bind _navigablepoints (Variables|Default|GetNavigablePoints))
  (bind _keys (Utilities|Map|Keys _navigablepoints))
  (for _array_element _keys
    (bind _keys_2 (Utilities|Map|Keys (Utilities|Struct|BreakF_TacticalArray (.Value (Utilities|Map|Find _navigablepoints _array_element)))))
    (for _array_element_2 _keys_2
      _)))

(fn AddNewNode
  (params (Position :type Int%20Vector%20Structure) (TileShape :type E_TileShapes%20Enum :default "NewEnumerator29") (TerrainType :type E_TerrainTypes%20Enum :default "NewEnumerator0"))
  (bind _returnvalue (Utilities|GetDataTableRow "/Game/Procedural/Data/DT_TileShapeInfo.DT_TileShapeInfo" (Utilities|String|StringToName (Utilities|String|EnumtoString TileShape)))
    (:then
      (if (.isstandable _returnvalue)
        (CallFunction|AddNode (Utilities|Struct|MakeF_TacticalNode Position TerrainType 0 0 (.characterheight _returnvalue) (.edgeheightnorth _returnvalue) (.edgeheighteast _returnvalue) (.edgeheightsouth _returnvalue) (.edgeheightwest _returnvalue))))
      (return))
    (:RowNotFound
      (Development|PrintString 0 "tile shape info not found"))))

(fn FindNodes
  (params (Position :type F%20Int%20Vector%202d%20Structure))
  (bind _navigablepoints (Variables|Default|GetNavigablePoints))
  (bind (_value _returnvalue) (Utilities|Map|Find _navigablepoints Position))
  (bind _values (Utilities|Map|Values (Utilities|Struct|BreakF_TacticalArray _value)))
  (return (select _returnvalue _values (Utilities|Array|MakeArray))))

(fn GetNode
  (params (Position :type Int%20Vector%20Structure))
  (bind _navigablepoints (Variables|Default|GetNavigablePoints))
  (bind (_value _returnvalue) (Utilities|Map|Find _navigablepoints (Utilities|Struct|MakeF_IntVector2d (.x Position) (.y Position))))
  (bind (_value_2 _returnvalue_2) (Utilities|Map|Find (.nodes _value) (.z Position)))
  (return _value_2 (and _returnvalue_2 _returnvalue)))

(fn FindMoves
  (params (Starting%20Position :type Int%20Vector%20Structure) (JumpDistance :type Integer) (FallDistance :type Integer))
  (bind ___ (Utilities|ToTilePosition Starting%20Position))
  (bind _returnvalue (/ JumpDistance 100))
  (bind _returnvalue_2 (+ _returnvalue 1))
  (LocalVariables|SetJump_Distance _returnvalue_2)
  (bind _output_get (LocalVariables|SetStartTileCoordinates ___))
  (bind _foundnode (CallFunction|GetNode _output_get))
  (LocalVariables|SetStartNode _foundnode)
  (bind _enumvalue (|ForEachE_Direction)
    (:LoopBody
      (bind _output_get_2 (LocalVariables|SetCurrentDirection _enumvalue))
      (for _index (range 1 _returnvalue_2)
        (LocalVariables|SetMoveDistance _index)
        (bind _tacticalnodes (CallFunction|FindNodes (Utilities|+(2d) (Utilities|*(2d) (Utilities|Struct|MakeF_IntVector2d _index _index) (Utilities|ToUnitVector2d _output_get_2)) (Utilities|ToIntVector2d ___))))
        (for _array_element _tacticalnodes
          (bind _output_get_3 (LocalVariables|SetDesinationNode _array_element))
          ;[0.15 0.15 0.15 0.5] Check if destination is occupied. If unit is opposing, break. If unit is allied, mark not final as true.
          (LocalVariables|SetDestinationTileCoordinates (Utilities|ToTilePosition (.Position (Utilities|Struct|BreakF_TacticalNode _output_get_3))))
          (if (not (Utilities|IsValid (.Unit (Utilities|Struct|BreakF_TacticalNode _output_get_3))))
            ;[0.15 0.15 0.15 0.5] Check if destination is close enough to jump to
            (if (<= (+ (Math|Integer|Max(Integer) (Utilities|GetEdgeHeightGain (LocalVariables|GetCurrentDirection) (LocalVariables|GetStartNode) (LocalVariables|GetDesinationNode))) (* (LocalVariables|GetMoveDistance) 100)) JumpDistance)
              (LocalVariables|SetHazardAccumulator (+ (LocalVariables|GetHazardAccumulator) (select (< (+ (Utilities|GetEdgeHeightGain (LocalVariables|GetCurrentDirection) (LocalVariables|GetStartNode) (LocalVariables|GetDesinationNode)) FallDistance) 0) 50 0)))
              ;[0.15 0.15 0.15 0.5] Check if path to destination is clear
              ;;[0.15 0.15 0.15 0.5] add move if distance is 1
              (if (== (LocalVariables|GetMoveDistance) 1)
                ;[0.15 0.15 0.15 0.5] add possible move
                (Utilities|Array|Add (LocalVariables|GetPossible%20Moves) (Utilities|Struct|MakeF_MoveData (.Position (Utilities|Struct|BreakF_TacticalNode (LocalVariables|GetDesinationNode))) (LocalVariables|GetHazardAccumulator) (LocalVariables|GetMoveDistance)) :!label _label)
                (else
                  ;;[0.15 0.15 0.15 0.5] find parabolic jump arc between points
                  (bind (_a_b_c _issolved) (Utilities|CalculateParabolicJumpArc (Utilities|ToIntVector2d(byDirection) (Utilities|GetBottomAirTile (LocalVariables|GetStartTileCoordinates)) (LocalVariables|GetCurrentDirection)) (Utilities|ToIntVector2d(byDirection) (Utilities|GetBottomAirTile (LocalVariables|GetDestinationTileCoordinates)) (LocalVariables|GetCurrentDirection)) (Math|Conversions|ToFloat(Integer) (LocalVariables|GetJump_Distance))))
                  (if _issolved
                    (LocalVariables|SetValidJump true)
                    ;;[0.15 0.15 0.15 0.5] for each tile between them horizontally, use the coefficients from above to find the paths height at that x,y coordinate,
                    (for _index_2 (range 0 (LocalVariables|GetMoveDistance))
                      ;;;[0 0.571 0 0.5] Tweak this to jump through narrower gaps
                      (for _index_3 (range 1 4)
                        (if (not (Utilities|Array|ContainsItem (Variables|Default|GetAirPoints) (Utilities|Struct|MakeIntVector (.X (Utilities|Struct|BreakIntVector (Utilities|+(3d) (Utilities|GetBottomAirTile (LocalVariables|GetStartTileCoordinates)) (Utilities|Scale(3d) (Utilities|ToIntVector (Utilities|ToUnitVector2d (LocalVariables|GetCurrentDirection))) (Math|Conversions|ToFloat(Integer) _index_2))))) (.Y (Utilities|Struct|BreakIntVector (Utilities|+(3d) (Utilities|GetBottomAirTile (LocalVariables|GetStartTileCoordinates)) (Utilities|Scale(3d) (Utilities|ToIntVector (Utilities|ToUnitVector2d (LocalVariables|GetCurrentDirection))) (Math|Conversions|ToFloat(Integer) _index_2))))) (+ (+ (Math|Float|Truncate (.Z (Math|Vector|BreakVector _a_b_c))) (* (Math|Float|Truncate (.X (Math|Vector|BreakVector _a_b_c))) (+ (.x (Utilities|*(3d) (Utilities|+(3d) (Utilities|GetBottomAirTile (LocalVariables|GetStartTileCoordinates)) (Utilities|Scale(3d) (Utilities|ToIntVector (Utilities|ToUnitVector2d (LocalVariables|GetCurrentDirection))) (Math|Conversions|ToFloat(Integer) _index_2))) (Utilities|ToIntVector (Utilities|ToUnitVector2d (LocalVariables|GetCurrentDirection))))) (.y (Utilities|*(3d) (Utilities|+(3d) (Utilities|GetBottomAirTile (LocalVariables|GetStartTileCoordinates)) (Utilities|Scale(3d) (Utilities|ToIntVector (Utilities|ToUnitVector2d (LocalVariables|GetCurrentDirection))) (Math|Conversions|ToFloat(Integer) _index_2))) (Utilities|ToIntVector (Utilities|ToUnitVector2d (LocalVariables|GetCurrentDirection))))) (.z (Utilities|*(3d) (Utilities|+(3d) (Utilities|GetBottomAirTile (LocalVariables|GetStartTileCoordinates)) (Utilities|Scale(3d) (Utilities|ToIntVector (Utilities|ToUnitVector2d (LocalVariables|GetCurrentDirection))) (Math|Conversions|ToFloat(Integer) _index_2))) (Utilities|ToIntVector (Utilities|ToUnitVector2d (LocalVariables|GetCurrentDirection))))) _index_2) (+ (.x (Utilities|*(3d) (Utilities|+(3d) (Utilities|GetBottomAirTile (LocalVariables|GetStartTileCoordinates)) (Utilities|Scale(3d) (Utilities|ToIntVector (Utilities|ToUnitVector2d (LocalVariables|GetCurrentDirection))) (Math|Conversions|ToFloat(Integer) _index_2))) (Utilities|ToIntVector (Utilities|ToUnitVector2d (LocalVariables|GetCurrentDirection))))) (.y (Utilities|*(3d) (Utilities|+(3d) (Utilities|GetBottomAirTile (LocalVariables|GetStartTileCoordinates)) (Utilities|Scale(3d) (Utilities|ToIntVector (Utilities|ToUnitVector2d (LocalVariables|GetCurrentDirection))) (Math|Conversions|ToFloat(Integer) _index_2))) (Utilities|ToIntVector (Utilities|ToUnitVector2d (LocalVariables|GetCurrentDirection))))) (.z (Utilities|*(3d) (Utilities|+(3d) (Utilities|GetBottomAirTile (LocalVariables|GetStartTileCoordinates)) (Utilities|Scale(3d) (Utilities|ToIntVector (Utilities|ToUnitVector2d (LocalVariables|GetCurrentDirection))) (Math|Conversions|ToFloat(Integer) _index_2))) (Utilities|ToIntVector (Utilities|ToUnitVector2d (LocalVariables|GetCurrentDirection))))) _index_2)) (* (Math|Float|Truncate (.Y (Math|Vector|BreakVector _a_b_c))) (+ (.x (Utilities|*(3d) (Utilities|+(3d) (Utilities|GetBottomAirTile (LocalVariables|GetStartTileCoordinates)) (Utilities|Scale(3d) (Utilities|ToIntVector (Utilities|ToUnitVector2d (LocalVariables|GetCurrentDirection))) (Math|Conversions|ToFloat(Integer) _index_2))) (Utilities|ToIntVector (Utilities|ToUnitVector2d (LocalVariables|GetCurrentDirection))))) (.y (Utilities|*(3d) (Utilities|+(3d) (Utilities|GetBottomAirTile (LocalVariables|GetStartTileCoordinates)) (Utilities|Scale(3d) (Utilities|ToIntVector (Utilities|ToUnitVector2d (LocalVariables|GetCurrentDirection))) (Math|Conversions|ToFloat(Integer) _index_2))) (Utilities|ToIntVector (Utilities|ToUnitVector2d (LocalVariables|GetCurrentDirection))))) (.z (Utilities|*(3d) (Utilities|+(3d) (Utilities|GetBottomAirTile (LocalVariables|GetStartTileCoordinates)) (Utilities|Scale(3d) (Utilities|ToIntVector (Utilities|ToUnitVector2d (LocalVariables|GetCurrentDirection))) (Math|Conversions|ToFloat(Integer) _index_2))) (Utilities|ToIntVector (Utilities|ToUnitVector2d (LocalVariables|GetCurrentDirection))))) _index_2))) _index_3))))
                          (LocalVariables|SetValidJump false))))
                    (if (LocalVariables|GetValidJump)
                      (goto _label))))))))))
    (:then
      (return (LocalVariables|GetPossible%20Moves)))))